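; Cave entrance trigger that toggles the visibility of a set of actors when the player passes through it.
; A box overlap by BP_PlayerCharacter drives a FlipFlop, alternately hiding and showing both actors tagged "SetHidden" and those in the ActorsToHide array.
; Both branches leave collision enabled on the ActorsToHide entries, and the state follows overlap count rather than crossing direction.
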(event OnComponentBeginOverlap(Box)
  (params (OverlappedComponent :type Primitive%20Component%20Object%20Reference) (OtherActor :type Actor%20Object%20Reference) (OtherComp :type Primitive%20Component%20Object%20Reference) (OtherBodyIndex :type Integer) (bFromSweep :type Boolean) (SweepResult :type Hit%20Result%20Structure%20%28by%20ref%29))
  (bind _actorstohide (Variables|LL|GetActorsToHide))
  (Utilities|Casting|CastToBP_PlayerCharacter OtherActor)
  (Utilities|FlowControl|FlipFlop
    (:A
      (Utilities|FlowControl|Sequence
        (:then_0
          (bind _outactors (Actor|GetAllActorswithTag "SetHidden"))
          (for _array_element _outactors
            (Rendering|SetActorHiddenInGame _array_element true)))
        (:then_1
          (for _array_element_2 _actorstohide
            (Rendering|SetActorHiddenInGame _array_element_2 true)
            (Collision|SetActorEnableCollision _array_element_2 true)))))
    (:B
      (Utilities|FlowControl|Sequence
        (:then_0
          (for _array_element_3 _actorstohide
            (Rendering|SetActorHiddenInGame _array_element_3 false)
            (Collision|SetActorEnableCollision _array_element_3 true)))
        (:then_1
          (bind _outactors_2 (Actor|GetAllActorswithTag "SetHidden"))
          (for _array_element_4 _outactors_2
            (Rendering|SetActorHiddenInGame _array_element_4 false)))))))

(event EventBeginPlay)

(event Collision|EventActorBeginOverlap
  (params (OtherActor :type Actor%20Object%20Reference)))

(event EventTick
  (params (DeltaSeconds :type Float%20%28single-precision%29)))

(fn ConstructionScript)