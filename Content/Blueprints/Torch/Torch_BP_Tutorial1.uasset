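; Tutorial torch Blueprint that the player can approach and light, leading into a tutorial dialog.
; Its overlap sphere registers itself as the player character's LanterOrb and shows a grab-lamp prompt widget, clearing both when the player leaves.
; TurnOn plays the IntensityOrb timeline to drive TorchLight intensity, then shows the second tutorial dialog widget after a short delay.
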(event OnComponentBeginOverlap(Sphere)
  (params (OverlappedComponent :type Primitive%20Component%20Object%20Reference) (OtherActor :type Actor%20Object%20Reference) (OtherComp :type Primitive%20Component%20Object%20Reference) (OtherBodyIndex :type Integer) (bFromSweep :type Boolean) (SweepResult :type Hit%20Result%20Structure%20%28by%20ref%29))
  (bind _asbp_player_character_tutorial (Utilities|Casting|CastToBP_Player_Character_Tutorial_1 OtherActor))
  (Variables|/Game/Blueprints/CharacterPlayer/BP_Player_Character_Tutorial_1.BP_Player_Character_Tutorial_1_C|SetLanterOrb _asbp_player_character_tutorial self)
  (bind _returnvalue (UserInterface|CreateWidget "/Game/UIX/Tutorial_1/WBP_GrabLamp.WBP_GrabLamp_C" (Game|GetPlayerController 0)))
  (Variables|Default|SetHUD_Instrucciones_temp _returnvalue)
  (UserInterface|Viewport|AddtoViewport _returnvalue 0))

(event OnComponentEndOverlap(Sphere)
  (params (OverlappedComponent :type Primitive%20Component%20Object%20Reference) (OtherActor :type Actor%20Object%20Reference) (OtherComp :type Primitive%20Component%20Object%20Reference) (OtherBodyIndex :type Integer))
  (bind _asbp_player_character_tutorial (Utilities|Casting|CastToBP_Player_Character_Tutorial_1 OtherActor))
  (Variables|/Game/Blueprints/CharacterPlayer/BP_Player_Character_Tutorial_1.BP_Player_Character_Tutorial_1_C|SetLanterOrb _asbp_player_character_tutorial 0)
  (bind _hud_instrucciones_temp (Variables|Default|GetHUD_Instrucciones_temp)
    (:then
      (Widget|RemovefromParent _hud_instrucciones_temp))
    (:else)))

(event Custom|TurnOn
  (bind _delta (Timeline|IntensityOrb PlayFromStart)
    (:Update
      (Rendering|Components|Light|SetIntensity (Variables|Default|GetTorchLight) _delta))
    (:Finished
      (Utilities|FlowControl|Delay 1.0)
      (bind _returnvalue (UserInterface|CreateWidget "/Game/UIX/Tutorial_1/WBP_Tutorial_01_Dialog2.WBP_Tutorial_01_Dialog2_C"))
      (UserInterface|Viewport|AddtoViewport _returnvalue 0))))

(event EventBeginPlay)

(event Collision|EventActorBeginOverlap
  (params (OtherActor :type Actor%20Object%20Reference)))

(fn ConstructionScript)