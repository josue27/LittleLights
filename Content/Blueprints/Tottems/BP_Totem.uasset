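; Totem objective Blueprint that the player discovers and completes by delivering missing pieces, extending a parent class.
; Discovery lights the base via a dynamic material, shows a widget, fires particles toward undelivered fragments, then activates each and spawns a beast.
; Delivered pieces fly from above the player into their hidden slots by timeline, and the last triggers TotemCompletion.
; BeaconCompleted expands a decal, shakes the camera and raises directional light.
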(event Custom|BeaconCompleted_Debug
  ;[0.1 0.15 0.2] Beacon Completed
  (Class|LLGameplayInterface|BeaconCompleted))

(event Custom|SpawnDecal
  ;[0.1 0.15 0.2] Spawn Decal
  (Variables|Default|GetEndDecalEffect
    (:then)
    (:else
      (bind _returnvalue (Game|SpawnActorfromClass "/Script/Engine.DecalActor" (Transformation|GetActorTransform) "AlwaysSpawn" "MultiplyWithRoot" 0 0))
      (bind _output_get (Variables|Default|SetEndDecalEffect _returnvalue))
      (Rendering|Components|Decal|SetDecalMaterial (Variables|/Script/Engine.DecalActor|GetDecal _output_get) "/Game/Material/M_TotemEndCircle_Decal_Inst.M_TotemEndCircle_Decal_Inst"))))

(event EventBeginPlay
  (Utilities|FlowControl|Sequence
    (:then_0
      ;[0.1 0.15 0.2] Hide totem pices that are in place
      (CallFunction|HideTotemPieces))
    (:then_1
      (Rendering|SetVisibility (Variables|Default|GetDecalDiscover) false false))
    (:then_2
      (bind _directionallight (Variables|Default|GetDirectionalLight)
        (:then
          (Rendering|Components|Light|SetIntensity (Variables|/Script/Engine.Light|GetLightComponent _directionallight) 0.0))
        (:else)))
    (:then_3
      (bind _tottembasemat (Variables|Default|GetTottemBaseMAT)
        (:then
          (Rendering|Material|SetScalarParameterValue _tottembasemat "EmissionIntensity" 0.0 :!class /Script/Engine.MaterialInstanceDynamic))
        (:else)))))

(event Collision|EventActorBeginOverlap
  (params (OtherActor :type Actor%20Object%20Reference)))

(event EventTick
  (params (DeltaSeconds :type Float%20%28single-precision%29)))

(event EventBeaconCompleted
  (bind _decaldiscover (Variables|Default|GetDecalDiscover))
  ;[0.1 0.15 0.2] Beacon Completed
  (|CallParentFunction)
  (Development|PrintString "Beacon Completed BP ")
  (Utilities|FlowControl|Delay 0.8)
  (Development|PrintString "Totem:Totem Completed")
  (Rendering|SetVisibility _decaldiscover true false)
  (Utilities|FlowControl|Sequence
    (:then_0
      (bind _delta (Timeline|ScaleDecalDelta PlayFromStart)
        (:Update
          (Transformation|SetWorldScale3D _decaldiscover (Math|Vector|Lerp(Vector) "1.000000,1.000000,1.000000" "50.000000,50.000000,50.000000" _delta)))))
    (:then_1
      (Camera|PlayWorldCameraShake "/Game/Blueprints/FX/TotemCompleted_ShakeCam.TotemCompleted_ShakeCam_C" (Transformation|GetActorLocation) 0.0 1e+03))
    (:then_2
      (Variables|Default|GetDirectionalLight
        (:then
          (bind _deltat (Timeline|IntensityDirectionLight Play)
            (:Update
              (Rendering|Components|Light|SetIntensity (Variables|/Script/Engine.Light|GetLightComponent (Variables|Default|GetDirectionalLight)) (Math|Float|Lerp 0.0 2e+01 _deltat)))))
        (:else)))
    (:then_3
      (Actor|GetActorOfClass "/Script/Engine.PostProcessVolume"))))

(event EventMovePieceAnim
  (params (PiecesToMoveInfo :type Map%20of%20TottemPieceType%20Enums%20to%20Structs :default "PieceA"))
  ;[1 1 1] Move piece animation logic(called in C++)
  (|CallParentFunction PiecesToMoveInfo)
  (bind _output_get (Variables|Default|SetPieces%20to%20Move%20Info PiecesToMoveInfo))
  (bind _enumvalue (|ForEachTottemPieceType)
    (:LoopBody
      (if (.ReturnValue (Utilities|Map|Find _output_get _enumvalue))
        (bind (_totempiecea_a _finalloc) (CallFunction|GetTotemPiecebyType _enumvalue))
        (Rendering|SetVisibility _totempiecea_a true true)
        (Math|Integer|DecrementInt (Variables|Default|GetPiecesToDeliver)
          (:%20%20
            (bind _player (Variables|Default|GetPlayer)
              (:then
                (Variables|Default|SetOriginalPos (Math|Vector|MakeVector (.x (Transformation|GetActorLocation _player)) (.y (Transformation|GetActorLocation _player)) (+ (.z (Transformation|GetActorLocation _player)) 1e+02)))
                (bind _alpha (Timeline|PieceMovement Play)
                  (:Update
                    (Transformation|SetWorldLocation _totempiecea_a (Math|Vector|Lerp(Vector) (Variables|Default|GetOriginalPos) _finalloc _alpha) false false))
                  (:Finished
                    (Class|LLTottem|MovePieceAnimEnded)
                    (if (== (Variables|Default|GetPiecesToDeliver) 0)
                      (Class|LLTottem|TotemCompletion)))))
              (:else))))))))

(event EventInteract
  (params (InstigatorPawn :type Pawn%20Object%20Reference))
  (|CallParentFunction InstigatorPawn))

(event EventTotemDiscoveredEvent
  (bind _returnvalue (Transformation|GetActorLocation))
  (bind _returnvalue_2 (Math|Vector|MakeVector 0.0 0.0 2e+02))
  (bind _totempieces (Variables|Default|GetTotemPieces))
  (bind _returnvalue_3 (+ _returnvalue_2 _returnvalue))
  ;[1 1 1] When player discovers the totem
  (|CallParentFunction)
  (bind _tottembasemat (Variables|Default|GetTottemBaseMAT)
    (:then
      (bind _newtrack_0 (Timeline|DeltaIntenistyBase Play)
        (:Update
          (Rendering|Material|SetScalarParameterValue _tottembasemat "EmissionIntensity" (Math|Float|Lerp 0.0 3.0 _newtrack_0) :!class /Script/Engine.MaterialInstanceDynamic))
        (:Finished
          (bind _returnvalue_4 (UserInterface|CreateWidget "/Game/UIX/PlayerHUDs/WBP_TotemDiscovered.WBP_TotemDiscovered_C" (Game|GetPlayerController 0)))
          (UserInterface|Viewport|AddtoViewport _returnvalue_4 0)
          ;[0.1 0.15 0.2] We Spawn a Particle system that travels to each totem fragment locaction
          (Utilities|FlowControl|Sequence
            (:then_0
              (for _array_element _totempieces
                (if (not (.Delivered (Utilities|Struct|BreakTottemPieceState _array_element)))
                  (Effects|SpawnEmitteratLocation "/Game/VFX/P_Priest_Shield.P_Priest_Shield" (+ _returnvalue_3 (* (Math|Vector|Normalize (- _returnvalue_3 (Transformation|GetActorLocation (.TotemPice (Utilities|Struct|BreakTottemPieceState _array_element))))) 1e+01)) (Math|Rotator|FindLookatRotation _returnvalue_3 (Transformation|GetActorLocation (.TotemPice (Utilities|Struct|BreakTottemPieceState _array_element))))))))
            (:then_1
              (Utilities|FlowControl|Delay 3.0)
              (for _array_element_2 _totempieces
                (if (not (.Delivered (Utilities|Struct|BreakTottemPieceState _array_element_2)))
                  (bind _asbp_totem_fragment (Utilities|Casting|CastToBP_Totem_Fragment (.TotemPice (Utilities|Struct|BreakTottemPieceState _array_element_2))))
                  (Default|Activate _asbp_totem_fragment true)
                  (bind _asbp_ll_game_mode_tl_4 (Utilities|Casting|CastToBP_LL_GameMode_TL_4 (Game|GetGameMode)))
                  (Class|LLGameModeBase|SpawnBeast _asbp_ll_game_mode_tl_4))))))))
    (:else)))

(event Input|KeyboardEvents|M
  (params (Key :type Key%20Structure :default "None")))

(fn ConstructionScript
  (bind _totembase (Variables|Default|GetTotemBase))
  (Utilities|FlowControl|Sequence
    (:then_0
      (bind _returnvalue (Rendering|Material|CreateDynamicMaterialInstance _totembase 0 "/Game/Materials/Base/MI_BaseBottom.MI_BaseBottom" "None" :!class /Script/Engine.PrimitiveComponent))
      (bind _output_get (Variables|Default|SetTottemBaseMAT _returnvalue))
      (Rendering|Material|SetMaterial _totembase 0 _output_get))
    (:then_1
      (for _array_element (Variables|Default|GetTotemPieces)
        (Rendering|Debug|DrawDebugLine (Transformation|GetActorLocation) (Transformation|GetActorLocation (.TotemPice (Utilities|Struct|BreakTottemPieceState _array_element))) "(R=1.000000,G=0.854518,B=0.000000,A=1.000000)" 0.0 2.0)))))

(fn GetTotemPiecebyType
  (params (Type :type TottemPieceType%20Enum :default "PieceA"))
  (bind _totempiecea_c (Variables|Default|GetTotemPieceA_C))
  (bind _totempiecea_d (Variables|Default|GetTotemPieceA_D))
  (bind _totempiecea_e (Variables|Default|GetTotemPieceA_E))
  (bind _totempiecea_a (Variables|Default|GetTotemPieceA_A))
  (bind _totempiecea_b (Variables|Default|GetTotemPieceA_B))
  (Utilities|FlowControl|Sequence
    (:then_0
      (switch Utilities|FlowControl|Switch|SwitchonTottemPieceType Type
        (:PieceA
          (LocalVariables|SetPieceSelected _totempiecea_a)
          (LocalVariables|SetLocSelected (Transformation|GetWorldLocation _totempiecea_a)))
        (:PieceB
          (LocalVariables|SetPieceSelected _totempiecea_b)
          (LocalVariables|SetLocSelected (Transformation|GetWorldLocation _totempiecea_b)))
        (:PieceC
          (LocalVariables|SetPieceSelected _totempiecea_c)
          (LocalVariables|SetLocSelected (Transformation|GetWorldLocation _totempiecea_c)))
        (:PieceD
          (LocalVariables|SetPieceSelected _totempiecea_d)
          (LocalVariables|SetLocSelected (Transformation|GetWorldLocation _totempiecea_d)))
        (:PieceE
          (LocalVariables|SetPieceSelected _totempiecea_e)
          (LocalVariables|SetLocSelected (Transformation|GetWorldLocation _totempiecea_e)))))
    (:then_1
      (return (LocalVariables|GetPieceSelected) (LocalVariables|GetLocSelected)))))

(fn HideTotemPieces
  (for _array_element (Variables|Default|GetTotemPieces)
    (if (not (.Delivered (Utilities|Struct|BreakTottemPieceState _array_element)))
      (Math|Integer|IncrementInt (Variables|Default|GetPiecesToDeliver)
        (:%20%20
          (switch Utilities|FlowControl|Switch|SwitchonTottemPieceType (.PieceType (Utilities|Struct|BreakTottemPieceState _array_element))
            (:PieceA
              (Rendering|SetVisibility (Variables|Default|GetTotemPieceA_A) false true))
            (:PieceB
              (Rendering|SetVisibility (Variables|Default|GetTotemPieceA_B) false true))
            (:PieceC
              (Rendering|SetVisibility (Variables|Default|GetTotemPieceA_C) false true))
            (:PieceD
              (Rendering|SetVisibility (Variables|Default|GetTotemPieceA_D) false true))
            (:PieceE
              (Rendering|SetVisibility (Variables|Default|GetTotemPieceA_E) false true))))))))