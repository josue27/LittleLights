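; BP_MainTottem_Test is a totem beacon that starts dark and lights up when TurnOnTottem is called.
; Activation runs once, notifies the Level Manager, and plays a timeline driving the point light, optional directional light and a fog Material Parameter Collection radius.
; When the timeline finishes, it unlocks the exit door.
; Player fragment-delivery logic is present but disconnected.
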(event Custom|TurnOnBeacon
  (bind _pointlight (Variables|Default|GetPointLight))
  (bind _level_manager (Variables|Default|GetLevel%20Manager))
  (bind _directionallight (Variables|Default|GetDirectionalLight))
  ;[1 1 1] Turning Beacon On
  (if (not (Variables|Default|GetBeaconActivated))
    (Variables|Default|SetBeaconActivated true)
    (Utilities|IsValid _level_manager
      (:Is%20Valid
        (Default|CallBeaconActivated _level_manager)
        (bind (_direction _lightintensity _radius _fogradiusexp _directionallightintensity) (Timeline|LigthtingOn PlayFromStart)
          (:Update
            (Rendering|Components|Light|SetIntensity _pointlight (* _lightintensity 1e+03))
            (Rendering|Lighting|SetAttenuationRadius _pointlight (* _radius 1e+03))
            (Rendering|Material|SetScalarParameterValue "/Game/Material/MC_Fog_Parametros.MC_Fog_Parametros" "RadiusExponential" _fogradiusexp :!class /Script/Engine.KismetMaterialLibrary)
            (Utilities|IsValid _directionallight
              (:Is%20Valid
                (Rendering|Components|Light|SetIntensity (Variables|/Script/Engine.Light|GetLightComponent _directionallight) _directionallightintensity))))
          (:Finished
            (bind (_newparam _valid) (CallFunction|GetExitDoor))
            (if _valid
              (Variables|/Script/LittleLights.DoorBase|SetbDoorUnlocked _newparam true)))))
      (:Is%20Not%20Valid
        (Development|PrintString "NO Level Manager ")))))

(event EventBeginPlay
  (bind _pointlight (Variables|Default|GetPointLight))
  (bind _directionallight (Variables|Default|GetDirectionalLight))
  (|CallParentFunction)
  (Rendering|Components|Light|SetIntensity _pointlight 0.0)
  (Rendering|Lighting|SetAttenuationRadius _pointlight 0.0)
  (bind (_bvalid _levelmanager) (CallFunction|GetLevelManager))
  (if _bvalid
    (Variables|Default|SetLevel%20Manager _levelmanager)
    (Utilities|IsValid _directionallight
      (:Is%20Valid
        (Rendering|Components|Light|SetIntensity (Variables|/Script/Engine.Light|GetLightComponent _directionallight) 0.0)))))

(event Collision|EventActorBeginOverlap
  (params (OtherActor :type Actor%20Object%20Reference))
  (|CallParentFunction OtherActor) ; This node is disabled and will not be called.\nDrag off pins to build functionality.
)

(event EventTick
  (params (DeltaSeconds :type Float%20%28single-precision%29))
  (|CallParentFunction DeltaSeconds) ; This node is disabled and will not be called.\nDrag off pins to build functionality.
)

(fn ConstructionScript
  (|CallParentFunction))

(fn TurnonTottem
  (|CallParentFunction)
  (CallFunction|TurnonBeacon))