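; Totem fragment actor that lights its mesh's emissive material shortly after play begins and can animate into a totem.
; InsertToTottem picks a random reachable point near the player, then after a delay shows mesh and light and lerps the actor to the target via timeline.
; Deactivate calls the parent and disables the sphere.
; Player pickup logic exists but is disconnected, leaving the overlap event empty; a debug path print remains.
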(event OnComponentBeginOverlap(Sphere)
  (params (OverlappedComponent :type Primitive%20Component%20Object%20Reference) (OtherActor :type Actor%20Object%20Reference) (OtherComp :type Primitive%20Component%20Object%20Reference) (OtherBodyIndex :type Integer) (bFromSweep :type Boolean) (SweepResult :type Hit%20Result%20Structure%20%28by%20ref%29)))

(event Custom|InsertSequence
  (params (WithDelay :type Float%20%28single-precision%29))
  (Utilities|FlowControl|Delay WithDelay)
  (CallFunction|Activate true)
  (bind _delta (Timeline|DeltaPosition PlayFromStart)
    (:Update
      (Transformation|SetActorLocation (Math|Vector|Lerp(Vector) (Variables|Default|GetPosInitAnimation) (Variables|Default|GetPosFinalAnimation) _delta) false false))))

(event EventBeginPlay
  (Utilities|FlowControl|Delay 2.0)
  (CallFunction|Turnon)
  (CallFunction|GetStaticMesh))

(event Collision|EventActorBeginOverlap
  (params (OtherActor :type Actor%20Object%20Reference)))

(event EventTick
  (params (DeltaSeconds :type Float%20%28single-precision%29)))

(event EventDeactivate
  (|CallParentFunction)
  (Collision|SetCollisionResponsetoAllChannels (Variables|Default|GetSphere) "ECR_Ignore")
  (Components|Activation|SetActive (Variables|Default|GetSphere) false false))

(fn ConstructionScript
  (bind _mesh (Variables|Default|GetMesh))
  (Utilities|IsValid _mesh
    (:Is%20Valid
      (Components|StaticMesh|SetStaticMesh (Variables|Default|GetStaticMesh) _mesh))
    (:Is%20Not%20Valid
      _))
  (bind _returnvalue (Rendering|Material|CreateDynamicMaterialInstance (Variables|Default|GetStaticMesh) 0 (Variables|Default|GetSource%20Material) "None" :!class /Script/Engine.PrimitiveComponent))
  (Variables|Default|SetDinamicaMAt _returnvalue))

(fn Turnon
  (Rendering|Material|SetScalarParameterValue (Variables|Default|GetDinamicaMAt) (Variables|Default|GetEmission%20Parameter%20Name) 1.0 :!class /Script/Engine.MaterialInstanceDynamic))

(fn Activate
  (params (activate :type Boolean))
  (Rendering|SetVisibility (Variables|Default|GetStaticMesh) activate false))

(fn GetName
  (return (Utilities|String|StringToName (Utilities|GetDisplayName (Variables|Default|GetStaticMesh)))))

(fn InserttoTottem
  (params (FinalPos :type Vector) (DelayOf :type Float%20%28single-precision%29))
  (Variables|Default|SetPosInitAnimation (.RandomLocation (AI|Navigation|GetRandomReachablePointinRadius (Transformation|GetActorLocation (Game|Player|GetPlayerPawn 0)) 2e+02 0 0)))
  (Variables|Default|SetPosFinalAnimation FinalPos)
  (CallFunction|InsertSequence DelayOf))

(fn GetStaticMesh
  (Development|PrintString (Class|KismetSystemLibrary|GetPathName (Variables|Default|GetStaticMesh))))