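; Collectible totem fragment that can be shown or hidden until the player takes it.
; BeVisible plays or reverses timelines that drive Mask and IntensityVertex on a dynamic material created at construction, and adjusts collision.
; Interact marks it taken and disables sphere collision only while visible.
; InsertToTottem only stores animation endpoints from a random reachable point near the player to the given position; Activate toggles mesh, light and collision.
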(event Custom|BeVisible
  (params (Visible :type Boolean))
  (bind _dinamicamat (Variables|Default|GetDinamicaMAt))
  (bind _dinamicamat_2 (Variables|Default|GetDinamicaMAt))
  (if (not (Variables|Default|GetbTaken))
    (if Visible
      ;[1 1 1] Change to Visible
      (Collision|SetCollisionResponsetoAllChannels (Variables|Default|GetSphereCollider) "ECR_Block")
      (Utilities|FlowControl|Sequence
        (:then_0
          (Rendering|Material|SetScalarParameterValue (Variables|Default|GetDinamicaMAt) "Mask" (Variables|Default|GetMask_Initial_PV) :!class /Script/Engine.MaterialInstanceDynamic)
          (Utilities|FlowControl|Delay 1.0)
          (Variables|Default|SetbIsVisible true)
          (bind _delta (Timeline|Timeline_0 PlayFromStart)
            (:Update
              (Rendering|Material|SetScalarParameterValue _dinamicamat "Mask" (Math|Float|Lerp (Variables|Default|GetMask_Initial_PV) 1.0 _delta) :!class /Script/Engine.MaterialInstanceDynamic)
              (Rendering|Material|SetScalarParameterValue _dinamicamat "IntensityVertex" (Math|Float|Lerp 2e+01 0.0 _delta) :!class /Script/Engine.MaterialInstanceDynamic))))
        (:then_1
          ;[1 1 1] Change to Invisible
          (bind _delta_2 (Timeline|Timeline_1 Stop)
            (:Update
              (Rendering|Material|SetScalarParameterValue _dinamicamat_2 "Mask" (Math|Float|Lerp (Variables|Default|GetMask_Initial_PV) 1.0 _delta_2) :!class /Script/Engine.MaterialInstanceDynamic)
              (Rendering|Material|SetScalarParameterValue _dinamicamat_2 "IntensityVertex" (Math|Float|Lerp 2e+01 0.0 _delta_2) :!class /Script/Engine.MaterialInstanceDynamic))
            (:Finished
              (Collision|SetCollisionResponsetoAllChannels (Variables|Default|GetMeshComponent) "ECR_Ignore")
              (Collision|SetCollisionResponsetoChannel (Variables|Default|GetSphereCollider) "ECC_Pawn" "ECR_Overlap")))))
      (else
        (Variables|Default|SetbIsVisible false)
        (Utilities|FlowControl|Sequence
          (:then_0
            (Timeline|Timeline_0 Stop))
          (:then_1
            (Timeline|Timeline_1 ReverseFromEnd)))))))

(event EventBeginPlay)

(event Collision|EventActorBeginOverlap
  (params (OtherActor :type Actor%20Object%20Reference)))

(event EventTick
  (params (DeltaSeconds :type Float%20%28single-precision%29)))

(event EventDeactivate
  (|CallParentFunction))

(event EventInteract
  (params (InstigatorPawn :type Pawn%20Object%20Reference))
  (bind _spherecollider (Variables|Default|GetSphereCollider))
  (|CallParentFunction InstigatorPawn)
  (if (Variables|Default|GetbIsVisible)
    (Variables|Default|SetbTaken true)
    (Collision|SetCollisionResponsetoAllChannels _spherecollider "ECR_Ignore")
    (Collision|SetCollisionEnabled _spherecollider "NoCollision")))

(fn ConstructionScript
  (bind _mesh (Variables|Default|GetMesh))
  (Utilities|IsValid _mesh
    (:Is%20Valid
      (Components|StaticMesh|SetStaticMesh (Variables|Default|GetMeshComponent) _mesh))
    (:Is%20Not%20Valid
      _))
  (bind _returnvalue (Rendering|Material|CreateDynamicMaterialInstance (Variables|Default|GetMeshComponent) 0 (Variables|Default|GetSource%20Material) "None" :!class /Script/Engine.PrimitiveComponent))
  (bind _output_get (Variables|Default|SetDinamicaMAt _returnvalue))
  (bind _returnvalue_2 (Rendering|Material|GetScalarParameterValue _output_get "Mask" :!class /Script/Engine.MaterialInstanceDynamic))
  (Variables|Default|SetMask_Initial_PV _returnvalue_2))

(fn Turnon
  (Rendering|Material|SetScalarParameterValue (Variables|Default|GetDinamicaMAt) (Variables|Default|GetEmission%20Parameter%20Name) 1.0 :!class /Script/Engine.MaterialInstanceDynamic))

(fn GetStaticMesh
  (Development|PrintString (Class|KismetSystemLibrary|GetPathName (Variables|Default|GetMeshComponent))))

(fn NewFunction0)

(fn InserttoTottem
  (params (FinalPos :type Vector) (DelayOf :type Float%20%28double-precision%29))
  (Variables|Default|SetPosInitAnimation (.RandomLocation (AI|Navigation|GetRandomReachablePointinRadius (Transformation|GetActorLocation (Game|Player|GetPlayerPawn 0)) 2e+02 0 0)))
  (Variables|Default|SetPosFinalAnimation FinalPos))

(fn Activate
  (params (activate :type Boolean))
  (bind _spherecollider (Variables|Default|GetSphereCollider))
  (Rendering|SetVisibility (Variables|Default|GetPointLight) activate false)
  (if activate
    (Collision|SetCollisionEnabled _spherecollider "QueryOnly")
    (else
      (Collision|SetCollisionEnabled _spherecollider "NoCollision"))))