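; Base totem actor that collects the fragments a player carries and turns on once it has received them all.
; On capsule overlap, it matches the player's fragments against its piece list, attaches each match at its stored offset and removes it from the player.
; Each fragment animates its own insertion with a staggered delay, and completion spawns a Niagara effect.
; The construction script derives the required count and piece names from that list.
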(event OnComponentBeginOverlap(Capsule)
  (params (OverlappedComponent :type Primitive%20Component%20Object%20Reference) (OtherActor :type Actor%20Object%20Reference) (OtherComp :type Primitive%20Component%20Object%20Reference) (OtherBodyIndex :type Integer) (bFromSweep :type Boolean) (SweepResult :type Hit%20Result%20Structure%20%28by%20ref%29))
  (bind _asbp_player_character (Utilities|Casting|CastToBP_PlayerCharacter OtherActor))
  (Variables|Default|SetAs%20BP%20Personaje%20Jugador _asbp_player_character)
  (for (_array_element _array_index) (Variables|/Game/Blueprints/CharacterPlayer/BP_PlayerCharacter.BP_PlayerCharacter_C|GetTottemFragments (Variables|Default|GetAs%20BP%20Personaje%20Jugador))
    (Development|PrintString (Utilities|GetDisplayName _array_element))
    (for (_array_element_2 _array_index_2) (Variables|Default|GetTottemsPieces_DB)
      (if (== _array_element (.TottemPiece (Utilities|Struct|BreakTottemPieceSettings _array_element_2)))
        (Development|PrintString "Player has a correct Piece")
        (bind _asbp_tottem_fragment (Utilities|Casting|CastToBP_TottemFragment (.TottemPiece (Utilities|Struct|BreakTottemPieceSettings _array_element_2))))
        (Utilities|IsValid _asbp_tottem_fragment
          (:Is%20Valid
            (Transformation|AttachActorToActor _asbp_tottem_fragment self "None" "KeepRelative" "KeepRelative" "KeepRelative" true)
            (Transformation|SetActorTransform _asbp_tottem_fragment (Math|Transform|MakeTransform (+ (Transformation|GetActorLocation) (+ (.Location (Math|Transform|BreakTransform (.MeshPostion (Utilities|Struct|BreakTottemPieceSettings _array_element_2)))) (Variables|Default|GetOffsetPiecesLocation))) (.Rotation (Math|Transform|BreakTransform (.MeshPostion (Utilities|Struct|BreakTottemPieceSettings _array_element_2)))) "1,1,1"))
            (bind _output_get (Variables|Default|SetAcumulatedDelay (+ (Variables|Default|GetAcumulatedDelay) 1.0)))
            ;[1 1 1] Is Piece is in charge of animating it's insertion
            (Default|InserttoTottem _asbp_tottem_fragment (+ (Transformation|GetActorLocation) (+ (.Location (Math|Transform|BreakTransform (.MeshPostion (Utilities|Struct|BreakTottemPieceSettings _array_element_2)))) (Variables|Default|GetOffsetPiecesLocation))) _output_get)
            (Variables|/Script/LittleLights.Tottem_Piece|SetbDelivered _asbp_tottem_fragment true)
            (bind _structout (Utilities|Struct|SetmembersinTottemPieceSettings _array_element_2 (.MeshPostion (Utilities|Struct|BreakTottemPieceSettings _array_element_2))))
            (Utilities|Array|SetArrayElem (Variables|Default|GetTottemsPieces_DB) _array_index_2 _structout)
            (Utilities|Array|RemoveIndex (Variables|/Game/Blueprints/CharacterPlayer/BP_PlayerCharacter.BP_PlayerCharacter_C|GetTottemFragments (Variables|Default|GetAs%20BP%20Personaje%20Jugador)) _array_index)
            (Default|RestToottemPiece (Variables|Default|GetAs%20BP%20Personaje%20Jugador) 1)
            ;[1 1 1] If the fragments have been completed
            (bind _result (Math|Integer|IncrementInt (Variables|Default|GetFragmentsRecieved))
              (:%20%20
                (if (>= _result (Variables|Default|GetFragmentsRequired))
                  (Utilities|FlowControl|Delay (Variables|Default|GetAcumulatedDelay))
                  (CallFunction|TurnonTottem))))))))
    (Variables|Default|SetAcumulatedDelay 0.0)))

(event OnComponentEndOverlap(Capsule)
  (params (OverlappedComponent :type Primitive%20Component%20Object%20Reference) (OtherActor :type Actor%20Object%20Reference) (OtherComp :type Primitive%20Component%20Object%20Reference) (OtherBodyIndex :type Integer))
  (if (== OtherActor (Variables|Default|GetAs%20BP%20Personaje%20Jugador))
    (Variables|Default|SetAs%20BP%20Personaje%20Jugador 0)))

(event EventBeginPlay)

(event Collision|EventActorBeginOverlap
  (params (OtherActor :type Actor%20Object%20Reference)))

(event EventTick
  (params (DeltaSeconds :type Float%20%28single-precision%29)))

(fn ConstructionScript
  (bind _tottemspieces_db (Variables|Default|GetTottemsPieces_DB))
  (Variables|Default|SetFragmentsRequired (Utilities|Array|Length _tottemspieces_db))
  (for (_array_element _array_index) _tottemspieces_db
    (bind _asbp_tottem_fragment (Utilities|Casting|CastToBP_TottemFragment (.TottemPiece (Utilities|Struct|BreakTottemPieceSettings _array_element))))
    (bind _structout (Utilities|Struct|SetmembersinTottemPieceSettings _array_element (Default|GetName _asbp_tottem_fragment)))
    (Utilities|Array|SetArrayElem _tottemspieces_db _array_index _structout)))

(fn TurnonTottem
  (Niagara|SpawnSystematLocation "/Game/VFX/Particles/Test_NiagaraEmitter_System.Test_NiagaraEmitter_System" (Transformation|GetWorldLocation (Variables|Default|GetParticleSystemSpawnLoc)))
  (Development|PrintString "Tottem turned On"))