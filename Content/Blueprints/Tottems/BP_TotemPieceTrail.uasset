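; Totem piece trail actor that shows a path by moving a Niagara ribbon effect along a spline.
; ShowPath sets the visibility flag and, if not already playing, restarts the ribbon from the spline start.
; While enabled, Tick advances the ribbon by speed and distance, optionally wrapping at the end.
; Past halfway, a once-gated timeline drives the ribbon's Scale Alpha fade, re-arming if playback has ended when it finishes.
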(event Custom|ShowPath
  (params (bShowPath :type Boolean))
  (bind _fxe_ribbon (Variables|Default|GetFXE_Ribbon))
  (Variables|Default|SetbShowPath bShowPath)
  (if (not (Variables|Default|GetbPlaying))
    (Components|Activation|SetActive _fxe_ribbon true true)
    (Variables|Default|SetCurrentPosition 0.0)
    (Niagara|SetNiagaraVariable(Float) _fxe_ribbon "Scale Alpha" 0.5)
    (Variables|Default|SetbPlaying true)))

(event EventBeginPlay)

(event Collision|EventActorBeginOverlap
  (params (OtherActor :type Actor%20Object%20Reference)))

(event EventTick
  (params (DeltaSeconds :type Float%20%28single-precision%29))
  (bind _spline (Variables|Default|GetSpline))
  (bind _returnvalue (Spline|GetSplineLength _spline))
  (if (Variables|Default|GetbShowPath)
    (bind _output_get (Variables|Default|SetCurrentPosition (+ (* DeltaSeconds (Variables|Default|GetSpeedOnSpline)) (Variables|Default|GetCurrentPosition))))
    (bind _fxe_ribbon (Variables|Default|GetFXE_Ribbon)
      (:then
        (Transformation|SetWorldTransform _fxe_ribbon (Spline|GetTransformatDistanceAlongSpline _spline _output_get "World" false) false false)
        (Utilities|FlowControl|Sequence
          (:then_0
            (if (>= _output_get _returnvalue)
              (if (Variables|Default|GetLoop)
                (Variables|Default|SetCurrentPosition 0.0))
              (Variables|Default|SetbPlaying false)))
          (:then_1
            (if (>= _output_get (/ _returnvalue 2.0))
              (Utilities|FlowControl|DoOnce false :!label _label
                (:Completed
                  (bind _deltafade (Timeline|Timeline PlayFromStart)
                    (:Update
                      (Niagara|SetNiagaraVariable(Float) (Variables|Default|GetFXE_Ribbon) "Scale Alpha" _deltafade))
                    (:Finished
                      (if (not (Variables|Default|GetbPlaying))
                        (goto _label Reset))))))))))
      (:else))))

(fn ConstructionScript)