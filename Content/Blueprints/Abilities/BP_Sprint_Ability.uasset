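; Sprint ability Blueprint that switches the player character between walk and sprint speed based on a stamina pool.
; Starting and stopping the ability toggles a Sprinting flag, which Update reads to drain or regenerate clamped stamina and broadcast it through the character's AbilityComponent.
; Empty stamina forces walk speed unless InfiniteSprint is set, and regeneration only runs while Sprinting is off.
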(event EventStartAbility
  (params (Instigator :type Actor%20Object%20Reference) (SecondActor :type Actor%20Object%20Reference))
  (|CallParentFunction Instigator 0)
  (Development|PrintString "Sprint Ability")
  (Variables|Default|SetbSprinting true))

(event EventStopAbility
  (params (Instigator :type Actor%20Object%20Reference) (SecondActor :type Actor%20Object%20Reference))
  (|CallParentFunction Instigator 0)
  (Variables|Default|SetbSprinting false))

(event EventUpdate
  (params (DeltaTime :type Float%20%28single-precision%29))
  (bind _returnvalue (Class|LLAbility|GetOwningComponent))
  (bind _asplayer_character (Utilities|Casting|CastToPlayerCharacter (Components|GetOwner _returnvalue)))
  (if (Variables|Default|GetbSprinting)
    (bind _output_get (Variables|Default|SetStamine (Math|Float|Clamp(Float) (- (Variables|Default|GetStamine) DeltaTime) 0.0 (Variables|Default|GetMaxStamine))))
    (Default|CallOnStamineChanged (Variables|/Script/LittleLights.PlayerCharacter|GetAbilityComponent _asplayer_character) 0 _output_get 0.0)
    (if (Variables|/Script/LittleLights.PlayerCharacter|GetbInfiniteSprint _asplayer_character)
      (Variables|/Script/LittleLights.PlayerCharacter|SetVelocidadMovimiento _asplayer_character (Variables|Default|GetSprintVelocity) :!label _label)
      (elif (<= _output_get 0.0)
        (Variables|/Script/LittleLights.PlayerCharacter|SetVelocidadMovimiento _asplayer_character (Variables|Default|GetWalkVelocity) :!label _label_2)
        (else
          (goto _label))))
    (else
      (bind _output_get_2 (Variables|Default|SetStamine (Math|Float|Clamp(Float) (+ (Variables|Default|GetStamine) (* DeltaTime (Variables|Default|GetRecoverVelocity))) 0.0 (Variables|Default|GetMaxStamine))))
      (Default|CallOnStamineChanged (Variables|/Script/LittleLights.PlayerCharacter|GetAbilityComponent _asplayer_character) 0 _output_get_2 0.0)
      (goto _label_2))))