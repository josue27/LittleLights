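; Roll-forward ability that launches the player character horizontally along its facing direction.
; Start resets a DoOnce gate, which Update trips after a short accumulated delay to disable movement and apply the launch once.
; Stopping clears the timer and restores movement; the logic for the ability to stop itself by name is unconnected.
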(event EventStartAbility
  (params (Instigator :type Actor%20Object%20Reference) (SecondActor :type Actor%20Object%20Reference))
  (|CallParentFunction Instigator 0)
  (Variables|Default|SetPlayerCharacter Instigator)
  (Utilities|FlowControl|DoOnce false) ; enters at Reset
)

(event EventStopAbility
  (params (Instigator :type Actor%20Object%20Reference) (SecondActor :type Actor%20Object%20Reference))
  (|CallParentFunction Instigator 0)
  (Variables|Default|SetTimePassed 0.0)
  (bind _asbp_player_character (Utilities|Casting|CastToBP_PlayerCharacter Instigator))
  (Variables|/Script/LittleLights.PlayerCharacter|SetbCanMove _asbp_player_character true))

(event EventUpdate
  (params (DeltaTime :type Float%20%28single-precision%29))
  (bind _output_get (Variables|Default|SetTimePassed (+ DeltaTime (Variables|Default|GetTimePassed))))
  (if (>= _output_get 0.25)
    (Utilities|FlowControl|DoOnce false
      (:Completed
        (bind _playercharacter (Variables|Default|GetPlayerCharacter)
          (:then
            (bind _asbp_player_character (Utilities|Casting|CastToBP_PlayerCharacter _playercharacter))
            (Variables|/Script/LittleLights.PlayerCharacter|SetbCanMove _asbp_player_character false)
            (Character|LaunchCharacter _asbp_player_character (Math|Vector|MakeVector (.x (* (Transformation|GetActorForwardVector _asbp_player_character) 1e+03)) (.y (* (Transformation|GetActorForwardVector _asbp_player_character) 1e+03)) 0.0) false false))
          (:else))))))