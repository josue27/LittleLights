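; Jump-vault ability that, on StartAbility, casts the instigator to BP_PlayerCharacter and hands off to its JumpOverAbility.
; The graph also holds a disconnected vault implementation that never runs.
; That unused logic line-traces wall height and thickness, then either falls back to a normal jump or plays a root-motion montage with capsule collision off and Flying movement.
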(event EventStartAbility
  (params (Instigator :type Actor%20Object%20Reference) (SecondActor :type Actor%20Object%20Reference))
  (bind _asbp_player_character (Utilities|Casting|CastToBP_PlayerCharacter Instigator))
  (Default|JumpOverAbility _asbp_player_character))