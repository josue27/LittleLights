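; BP_LL_CrouchCross_Ability is an ability that, judging by its name, handles a crouched crossing for the player character.
; StartAbility calls the parent and caches the instigating BP_PlayerCharacter, and correct or incorrect key press events are forwarded to that character.
; GetClosestPoint compares the character's distance to both spline ends, returning true unless the first is nearer.
; GetKeyToPress returns only an empty string.
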(event EventCorrectKeyPressed
  (bind _bp_playercharacter (Variables|Default|GetBP_PlayerCharacter)
    (:then
      (Default|KeyPressedCorrectly _bp_playercharacter))
    (:else)))

(event EventStartAbility
  (params (Instigator :type Actor%20Object%20Reference) (SecondActor :type Actor%20Object%20Reference))
  (|CallParentFunction Instigator SecondActor)
  (bind _asbp_player_character (Utilities|Casting|CastToBP_PlayerCharacter Instigator))
  (Variables|Default|SetBP_PlayerCharacter _asbp_player_character))

(event EventInCorrectKeyPressed
  (bind _bp_playercharacter (Variables|Default|GetBP_PlayerCharacter)
    (:then
      (Default|KeyPressedIncorrect _bp_playercharacter))
    (:else)))

(fn GetClosestPoint
  (params (BPPlayerCharacter :type BP%20Player%20Character%20Object%20Reference) (SplineComp :type Spline%20Component%20Object%20Reference))
  (bind _returnvalue (Transformation|GetActorLocation BPPlayerCharacter))
  (Utilities|IsValid BPPlayerCharacter
    (:Is%20Valid
      (if (< (Math|Vector|Distance(Vector) _returnvalue (Spline|GetLocationatSplinePoint SplineComp 0 "World")) (Math|Vector|Distance(Vector) _returnvalue (Spline|GetLocationatSplinePoint SplineComp (Spline|GetNumberOfSplinePoints SplineComp) "World")))
        (return false)
        (else
          (return true))))))

(fn GetKeytoPress
  (if true
    (return "")))