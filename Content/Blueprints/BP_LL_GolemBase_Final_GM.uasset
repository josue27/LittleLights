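; Game mode for the final Golem Base level, running cutscene dialogue and the end credits before returning to the menu.
; BeginPlay loads lines by ID from a data table; dialogue events pause the level sequence, display them through the player controller and optionally resume playback.
; Player input advances dialogue, or leaves once credits are up.
; Tick clears the fog-of-war render target; save/load are basic, and beast spawning is unwired.
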(event Custom|QueryLocactionFinished
  (params (QueryInstance :type Env%20Query%20Instance%20Blueprint%20Wrapper%20Object%20Reference) (QueryStatus :type EEnvQueryStatus%20Enum :default "Processing"))
  ;[0.9427 1 0 1 58] SpawnBeast TODO: Fix the C++ implementation
  (if (Utilities|Enum|Equal(Enum) QueryStatus "Success")
    (bind _resultlocations (AI|EQS|GetQueryResultsasLocations QueryInstance))
    (else
      (Development|PrintString "Problem Runnignquery" true true "(R=1.000000,G=0.486477,B=0.000000,A=1.000000)"))))

(event Custom|OnInteractionPressed_Event
  ;[0.2656 0.5753 1] Dialogue Logic
  ;;[1 1 1] Pressing C to continue playing
  (if (Variables|Default|GetOnEndCredits)
    (CallFunction|ChangeLevel)
    (elif (Variables|Default|GetDialogueActivated)
      (bind _bp_player_controller (Variables|Default|GetBP%20Player%20Controller)
        (:then
          (Class|LLPlayerControllerBase|ShowNextDialogue _bp_player_controller))
        (:else)))))

(event Custom|ChangeToCredits
  (bind _levelsequence (Variables|Default|GetLevelSequence)
    (:then
      (Sequencer|Player|Pause (Variables|/Script/LevelSequence.LevelSequenceActor|GetSequencePlayer _levelsequence))
      (bind _returnvalue (UserInterface|CreateWidget "/Game/UIX/MainMenu/WBP_LevelCredits.WBP_LevelCredits_C" (Game|GetPlayerController 0)))
      (UserInterface|Viewport|AddtoViewport _returnvalue 0)
      (Default|FadeinSequence _returnvalue)
      (Utilities|FlowControl|Delay 3.0)
      (Variables|Default|SetOnEndCredits true))
    (:else)))

(event Custom|LoadGame
  ;[0.1 0.15 0.2] Save/Load Game
  (bind _savegame (|AsyncLoadGamefromSlot "LLDebugSaveSlot")
    (:Completed
      (Utilities|Casting|CastToBP_SaveGameObject _savegame)
      (Development|PrintString "Save Game Loaded"))))

(event Custom|ShowNextDialogue
  (params (PauseTimeline :type Boolean) (ShouldPlayAfterClose :type Boolean))
  (bind _indialogue (Variables|Default|GetInDialogue))
  (bind _indialogue_2 (Variables|Default|GetInDialogue))
  (bind _dialogue_lines (Variables|Default|GetDialogue%20Lines))
  ;[0.2656 0.5753 1] Dialogue Logic
  ;;[1 1 1] Shod Dialogue
  ;;;[0.1 0.15 0.2] Comment
  ;;;;[0.1 0.15 0.2] Comment
  (if true
    (bind _levelsequence (Variables|Default|GetLevelSequence)
      (:then
        (Variables|Default|SetShouldPlayAfterClose PauseTimeline)
        (Sequencer|Player|Pause (Variables|/Script/LevelSequence.LevelSequenceActor|GetSequencePlayer _levelsequence)))
      (:else)))
  (bind _asbp_player_character (Utilities|Casting|CastToBP_PlayerCharacter (Game|Player|GetPlayerPawn 0))
    (:then
      (Class|PlayerCharacter|StopCharacter _asbp_player_character))
    (:CastFailed
      _))
  (Variables|Default|SetKeepDialogueWindow ShouldPlayAfterClose)
  (bind _bp_player_controller (Variables|Default|GetBP%20Player%20Controller)
    (:then
      (if (Utilities|Array|IsValidIndex _dialogue_lines _indialogue)
        ;;;[0.1 0.15 0.2] Comment
        (Class|LLPlayerControllerBase|ShowDialogue _bp_player_controller (Utilities|Array|Get(acopy) _dialogue_lines _indialogue) true)
        (Development|PrintString (Utilities|String|ToString(Text) (Utilities|Text|FormatText "DialogueDisplaying {Dialogue Num}" _indialogue)))
        (Math|Integer|IncrementInt _indialogue_2
          (:%20%20
            (Variables|Default|SetDialogueActivated true)
            (bind _bp_player_controller_2 (Variables|Default|GetBP%20Player%20Controller)
              (:then
                (EventDispatchers|AssignOnDialogueLinesOver _bp_player_controller_2 (EventDispatchers|CreateEvent :!event Custom|DialogueEnded))
                (Development|PrintString (Utilities|String|ToString(Text) (Utilities|Text|FormatText "NextDialogue {Dialogue Num}" _indialogue_2)) true true "(R=0.000000,G=0.660000,B=1.000000,A=1.000000)" 3.0))
              (:else))))
        (else
          (Development|PrintString "NO DIALOGUE FOUND"))))
    (:else)))

(event Custom|SaveGame
  ;[0.1 0.15 0.2] Save/Load Game
  (bind _returnvalue (SaveGame|CreateSaveGameObject "/Game/Blueprints/SaveSystem/BP_SaveGameObject.BP_SaveGameObject_C"))
  (bind _output_get (Variables|Default|SetSaveGameInstance _returnvalue))
  (|AsyncSaveGametoSlot _output_get (Variables|/Game/Blueprints/SaveSystem/BP_SaveGameObject.BP_SaveGameObject_C|GetSaveSlotName _output_get) (Variables|/Game/Blueprints/SaveSystem/BP_SaveGameObject.BP_SaveGameObject_C|GetUserIndex _output_get)
    (:Completed
      (Development|PrintString "Save Game Completed"))))

(event Custom|DialogueEnded
  ;[0.2656 0.5753 1] Dialogue Logic
  ;;[1 1 1] Dialogue Ended
  (if (Variables|Default|GetShouldPlayAfterClose)
    (bind _levelsequence (Variables|Default|GetLevelSequence)
      (:then
        (Sequencer|Player|Play (Variables|/Script/LevelSequence.LevelSequenceActor|GetSequencePlayer _levelsequence) :!class /Script/MovieScene.MovieSceneSequencePlayer))
      (:else)))
  (bind _bp_player_controller (Variables|Default|GetBP%20Player%20Controller)
    (:then
      (Class|LLPlayerControllerBase|ShowDialogue _bp_player_controller (Variables|Default|GetEmpty%20Dialogue%20Struct) false)
      (Variables|Default|SetDialogueActivated false))
    (:else)))

(event Custom|ChangeLevel
  (bind _returnvalue (UserInterface|CreateWidget "/Game/UIX/MainMenu/WBP_LevelTransition.WBP_LevelTransition_C" (Game|GetPlayerController 0)))
  (UserInterface|Viewport|AddtoViewport _returnvalue 0)
  (Default|FadeinSequence _returnvalue)
  (Utilities|FlowControl|Delay 2.0)
  (Game|OpenLevel(byObjectReference) "/Game/Maps/LL_Menu.LL_Menu"))

(event EventBeginPlay
  (bind _dialoguesdt (Variables|Default|GetDialoguesDT))
  ;[1 1 1] CARE, begin play starts before StartPlay
  (Utilities|FlowControl|Sequence
    (:then_0
      (bind _outactors (Actor|GetAllActorsOfClass "/Script/LevelSequence.LevelSequenceActor"))
      (Variables|Default|SetLevelSequence (Utilities|Array|Get(acopy) _outactors))
      (bind _asbp_player_controller (Utilities|Casting|CastToBP_PlayerController (Game|GetPlayerController 0)))
      (Variables|Default|SetBP%20Player%20Controller _asbp_player_controller))
    (:then_1
      (Variables|/Script/LittleLights.LL_DialogueSubsystem|SetCharactersData (Subsystems|GetLLDialogueSubsystem) "/Game/DataTables/DT_SpeakersData.DT_SpeakersData"))
    (:then_2
      (bind _outrownames (DataTable|GetDataTableRowNames _dialoguesdt))
      (bind _array_element (Utilities|Array|ForEachLoopwithBreak _outrownames :!label _label)
        (:LoopBody
          (bind _returnvalue (Utilities|GetDataTableRow _dialoguesdt _array_element)
            (:then
              (if (Utilities|Enum|Equal(Enum) (.ID (Utilities|Struct|BreakLL_Dialogue _returnvalue)) (Variables|Default|GetDialoguesID))
                (Variables|Default|SetDialogue%20Lines (.DialogueLines (Utilities|Struct|BreakLL_Dialogue _returnvalue)))
                (goto _label Break)))))))
    (:then_3
      (bind _asbp_player_character (Utilities|Casting|CastToBP_PlayerCharacter (Game|Player|GetPlayerPawn 0)))
      (EventDispatchers|AssignOnDialogueAdvance _asbp_player_character (EventDispatchers|CreateEvent :!event Custom|OnInteractionPressed_Event)))))

(event EventTick
  (params (DeltaSeconds :type Float%20%28single-precision%29))
  (Rendering|ClearRenderTarget2D "/Game/FogOfWarSystem/FogOfWarReveal_Render.FogOfWarReveal_Render"))

(event EventStartSequence
  (Utilities|FlowControl|Sequence
    (:then_0
      (bind _returnvalue (UserInterface|CreateWidget "/Game/UIX/MainMenu/WBP_LevelTransition.WBP_LevelTransition_C"))
      (UserInterface|Viewport|AddtoViewport _returnvalue 10)
      (Default|FadeOutSequence _returnvalue false))
    (:then_1
      (Utilities|Casting|CastToBP_PlayerCharacter (Variables|Default|GetPlayer)))))

(event EventSpawnBeast
  ;[0.1 0.15 0.2] Called by BP Totem when discoverd
)

(fn ConstructionScript)