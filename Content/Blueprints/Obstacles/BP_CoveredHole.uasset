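; BP_CoveredHole is an obstacle Blueprint for a covered hole trap that swings after its PlayerInside event fires.
; The event waits for the TimeActivationReaction delay, then plays the TrapRotation timeline from the start.
; Each timeline update sets the pitch of the Scene component's relative rotation, with roll and yaw held at zero.
; Nothing in these graphs calls PlayerInside or resets the trap.
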(event EventBeginPlay
  (|CallParentFunction) ; This node is disabled and will not be called.\nDrag off pins to build functionality.
)

(event Collision|EventActorBeginOverlap
  (params (OtherActor :type Actor%20Object%20Reference))
  (|CallParentFunction OtherActor) ; This node is disabled and will not be called.\nDrag off pins to build functionality.
)

(event EventTick
  (params (DeltaSeconds :type Float%20%28single-precision%29))
  (|CallParentFunction DeltaSeconds) ; This node is disabled and will not be called.\nDrag off pins to build functionality.
)

(event EventPlayerInside
  (Utilities|FlowControl|Delay (Variables|Default|GetTimeActivationReaction))
  (bind _rotation (Timeline|TrapRotation PlayFromStart)
    (:Update
      (Transformation|SetRelativeRotation (Variables|Default|GetScene) (Math|Rotator|MakeRotator 0.0 _rotation 0.0) false false))))

(fn ConstructionScript
  (|CallParentFunction))