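; Base obstacle zone that lets BP_PersonajeJugador jump over it along a spline from either end.
; TriggerStart overlaps flag the player as in the zone and hand it a reference to this actor.
; StartJumpOver deactivates BlockingZone and the player capsule, then turns the player along the spline from the nearer end.
; After a delay, TravelPlayer plays forward or reversed, moving X and Z along the spline with a height offset while keeping Y, then reactivates both.
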(event OnComponentBeginOverlap(TriggerStart)
  (params (OverlappedComponent :type Primitive%20Component%20Object%20Reference) (OtherActor :type Actor%20Object%20Reference) (OtherComp :type Primitive%20Component%20Object%20Reference) (OtherBodyIndex :type Integer) (bFromSweep :type Boolean) (SweepResult :type Hit%20Result%20Structure%20%28by%20ref%29))
  (bind _asbp_personaje_jugador (Utilities|Casting|CastToBP_PersonajeJugador OtherActor))
  (Variables|Default|SetAs%20BP%20Personaje%20Jugador _asbp_personaje_jugador)
  (Variables|/Script/LittleLights.Personaje|SetbInJumpOverZone _asbp_personaje_jugador true)
  (Variables|/Script/LittleLights.Personaje|SetTemp_JumpOverZone _asbp_personaje_jugador self))

(event OnComponentEndOverlap(TriggerStart)
  (params (OverlappedComponent :type Primitive%20Component%20Object%20Reference) (OtherActor :type Actor%20Object%20Reference) (OtherComp :type Primitive%20Component%20Object%20Reference) (OtherBodyIndex :type Integer))
  (if (not (Variables|Default|GetbIsJumping))
    (if (== OtherActor (Variables|Default|GetAs%20BP%20Personaje%20Jugador))
      (Variables|/Script/LittleLights.Personaje|SetbInJumpOverZone (Variables|Default|GetAs%20BP%20Personaje%20Jugador) false)
      (Variables|Default|SetAs%20BP%20Personaje%20Jugador 0))))

(event EventBeginPlay)

(event Collision|EventActorBeginOverlap
  (params (OtherActor :type Actor%20Object%20Reference)))

(event EventTick
  (params (DeltaSeconds :type Float%20%28single-precision%29)))

(event EventStartJumpOver
  (bind _spline (Variables|Default|GetSpline))
  (bind _as_bp_personaje_jugador (Variables|Default|GetAs%20BP%20Personaje%20Jugador))
  (bind _returnvalue (Transformation|GetActorRotation _as_bp_personaje_jugador))
  (bind _returnvalue_2 (Transformation|GetActorLocation _as_bp_personaje_jugador))
  ;[1 1 1] JumpOver Sequence
  (Variables|Default|SetbIsJumping true)
  (Components|Activation|SetActive (Variables|Default|GetBlockingZone) false false)
  (Components|Activation|SetActive (Variables|/Script/Engine.Character|GetCapsuleComponent (Variables|Default|GetAs%20BP%20Personaje%20Jugador)) false false)
  (bind _bclosertoend (CallFunction|GetCloserPoint))
  (if _bclosertoend
    (Transformation|SetActorRotation _as_bp_personaje_jugador (Math|Rotator|MakeRotator (.roll _returnvalue) (.pitch _returnvalue) (- (.yaw (Spline|GetRotationatSplinePoint _spline (Spline|GetNumberOfSplinePoints _spline) "World")) 1.8e+02)))
    (Variables|Default|SetZ_offset (- (.z _returnvalue_2) (.z (Spline|GetLocationatSplinePoint _spline (Spline|GetNumberOfSplinePoints _spline) "World"))))
    (Utilities|FlowControl|Delay 1.0)
    (bind _newtrack_0 (Timeline|TravelPlayer ReverseFromEnd)
      (:Update
        (Transformation|SetActorLocation _as_bp_personaje_jugador (Math|Vector|MakeVector (.x (Spline|GetLocationatDistanceAlongSpline (Variables|Default|GetSpline) (* _newtrack_0 (Spline|GetSplineLength _spline)) "World")) (.y (Transformation|GetActorLocation (Variables|Default|GetAs%20BP%20Personaje%20Jugador))) (+ (.z (Spline|GetLocationatDistanceAlongSpline (Variables|Default|GetSpline) (* _newtrack_0 (Spline|GetSplineLength _spline)) "World")) (Variables|Default|GetZ_offset))) false false))
      (:Finished
        (Variables|Default|SetbIsJumping false)
        (Components|Activation|SetActive (Variables|Default|GetBlockingZone) true false)
        (Components|Activation|SetActive (Variables|/Script/Engine.Character|GetCapsuleComponent (Variables|Default|GetAs%20BP%20Personaje%20Jugador)) true false)))
    (else
      (Transformation|SetActorRotation _as_bp_personaje_jugador (Math|Rotator|MakeRotator (.roll _returnvalue) (.pitch _returnvalue) (.yaw (Spline|GetRotationatSplinePoint _spline 0 "World"))))
      (Variables|Default|SetZ_offset (- (.z _returnvalue_2) (.z (Spline|GetLocationatSplinePoint _spline 0 "World"))))
      (Utilities|FlowControl|Delay 1.0)
      (Timeline|TravelPlayer PlayFromStart))))

(fn ConstructionScript)

(fn GetCloserPoint
  (bind _spline (Variables|Default|GetSpline))
  (bind _as_bp_personaje_jugador (Variables|Default|GetAs%20BP%20Personaje%20Jugador))
  (bind _returnvalue (Transformation|GetActorLocation _as_bp_personaje_jugador))
  (Utilities|IsValid _as_bp_personaje_jugador
    (:Is%20Valid
      (if (< (Math|Vector|Distance(Vector) _returnvalue (Spline|GetLocationatSplinePoint _spline 0 "World")) (Math|Vector|Distance(Vector) _returnvalue (Spline|GetLocationatSplinePoint _spline (Spline|GetNumberOfSplinePoints _spline) "World")))
        (return false)
        (else
          (return true))))))