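; BP_SpecialMovement_CrossBalance is an obstacle Blueprint, named for a balance-crossing special movement by the player.
; When the player character's overlap with TriggerOutZone ends, it restores TriggerCollider to query-only and BlockerCollider to physics-only collision.
; DisableMeshCollisions is an empty event, and the file shows no other active logic beyond the parent construction script call.
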(event OnComponentEndOverlap(TriggerOutZone)
  (params (OverlappedComponent :type Primitive%20Component%20Object%20Reference) (OtherActor :type Actor%20Object%20Reference) (OtherComp :type Primitive%20Component%20Object%20Reference) (OtherBodyIndex :type Integer))
  (Utilities|Casting|CastToBP_PlayerCharacter OtherActor)
  (Collision|SetCollisionEnabled (Variables|Default|GetTriggerCollider) "QueryOnly")
  (Collision|SetCollisionEnabled (Variables|Default|GetBlockerCollider) "PhysicsOnly"))

(event EventBeginPlay
  (|CallParentFunction) ; This node is disabled and will not be called.\nDrag off pins to build functionality.
)

(event Collision|EventActorBeginOverlap
  (params (OtherActor :type Actor%20Object%20Reference))
  (|CallParentFunction OtherActor) ; This node is disabled and will not be called.\nDrag off pins to build functionality.
)

(event EventTick
  (params (DeltaSeconds :type Float%20%28single-precision%29))
  (|CallParentFunction DeltaSeconds) ; This node is disabled and will not be called.\nDrag off pins to build functionality.
)

(event EventDisableMeshCollisions
  (params (ActivationDelay :type Float%20%28single-precision%29)))

(fn ConstructionScript
  (|CallParentFunction))