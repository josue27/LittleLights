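; Base interactable obstacle for special movement zones (jump over, crouch, balance), with the prompt set by zone type in construction.
; Its Enabled flag gates trigger collision at start, and activation enables it and shows the wood meshes.
; Interacting runs parent logic, then after a short delay activates linked objects through LL_GameplayInterface.
; GetCloserPoint picks the spline end nearer the player, while Tick draws debug spheres at EndPositions.
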(event Custom|ActivateMesh
  (params (bNewVisibility :type Boolean))
  (Rendering|SetVisibility (Variables|Default|GetSM_WoodTrunk_A) bNewVisibility true))

(event EventBeginPlay
  (bind _triggercollider (Variables|Default|GetTriggerCollider))
  (if (Variables|Default|GetbEnabled)
    (Collision|SetCollisionEnabled _triggercollider "QueryOnly")
    (else
      (Collision|SetCollisionEnabled _triggercollider "NoCollision"))))

(event Collision|EventActorBeginOverlap
  (params (OtherActor :type Actor%20Object%20Reference)))

(event EventTick
  (params (DeltaSeconds :type Float%20%28single-precision%29))
  (bind _endpositions (Variables|Default|GetEndPositions))
  (if (> (Utilities|Array|Length _endpositions) 0)
    (for _array_element _endpositions
      (Rendering|Debug|DrawDebugSphere _array_element 1e+01 12 "(R=1.000000,G=0.000000,B=0.123685,A=1.000000)" 0.0))))

(event EventActivateObjectsonList
  ;[0.1 0.15 0.2] Activate logic
  (for _array_element (Variables|Default|GetActivableObjects)
    (if (Utilities|DoesObjectImplementInterface _array_element "/Script/LittleLights.LL_GameplayInterface")
      (Class|LLGameplayInterface|ActivateObject(Message) _array_element))))

(event EventActivateObject
  ;[0.1 0.15 0.2] Activate logic
  (bind _output_get (Variables|Default|SetbEnabled true))
  (CallFunction|ActivateMesh _output_get)
  (Collision|SetCollisionEnabled (Variables|Default|GetTriggerCollider) "QueryOnly"))

(event EventDisableMeshCollisions
  (params (ActivationDelay :type Float%20%28single-precision%29)))

(event EventInteract
  (params (InstigatorPawn :type Pawn%20Object%20Reference))
  (Development|PrintString "Interacting with")
  (|CallParentFunction InstigatorPawn)
  (Utilities|FlowControl|Delay 0.5)
  (Class|LLGameplayInterface|ActivateObjectsonList))

(fn ConstructionScript
  (Utilities|FlowControl|Sequence
    (:then_0
      (switch Utilities|FlowControl|Switch|SwitchonELLSpecialMovementZoneType (Variables|Default|GetMovementZone_Type)
        (:SMZ_JumpOver
          (Variables|Default|SetInteractionMessage "Press E to Jump Over"))
        (:SMZ_Crouch
          (Variables|Default|SetInteractionMessage "Press E to Crouch"))
        (:SMZ_CrossBalancing
          (Variables|Default|SetInteractionMessage "Press E to Balance"))))))

(fn GetCloserPoint
  (bind _splinepath (Variables|Default|GetSplinePath))
  (bind _bp_playercharacter (Variables|Default|GetBP_PlayerCharacter))
  (bind _returnvalue (Transformation|GetActorLocation _bp_playercharacter))
  (Utilities|IsValid _bp_playercharacter
    (:Is%20Valid
      (if (< (Math|Vector|Distance(Vector) _returnvalue (Spline|GetLocationatSplinePoint _splinepath 0 "World")) (Math|Vector|Distance(Vector) _returnvalue (Spline|GetLocationatSplinePoint _splinepath (Spline|GetNumberOfSplinePoints _splinepath) "World")))
        (return false)
        (else
          (return true))))))