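; Level manager for the first tutorial that sequences intro UI, dialogs, player control and camera moves.
; On BeginPlay it disables input, then shows the intro widget in UI-only mode after a delay.
; DialogOneEnded switches on an event index to light the tutorial lantern, restore control, or blend to a road camera for dialog four and back to the player.
; GameStart also restores game input.
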(event Custom|DialogOneEnded
  (params (Event :type Integer))
  (bind _returnvalue (Game|GetPlayerController 0))
  (switch int Event
    (:0
      (bind _lanterntutorial (Variables|Tutorial1|GetLanternTutorial)
        (:then
          (Default|Turnon _lanterntutorial))
        (:else)))
    (:1
      (Input|EnableInput (Game|Player|GetPlayerPawn 0) _returnvalue)
      (Input|SetInputModeGameOnly _returnvalue)
      (Variables|/Script/Engine.PlayerController|SetbShowMouseCursor _returnvalue false))
    (:2
      (CallFunction|ChangetoGameInput)
      (Utilities|FlowControl|Delay 3.0)
      (CallFunction|PlayerCanMove false)
      (Game|Player|SetViewTargetwithBlend (Game|GetPlayerController 0) (Variables|Tutorial1|GetCameraForRoad) 2.0 "VTBlend_EaseIn" 1.0 false)
      (Utilities|FlowControl|Delay 1.0)
      (bind _returnvalue_2 (UserInterface|CreateWidget "/Game/UIX/Tutorial_1/WBP_Tutorial_01_Dialog4.WBP_Tutorial_01_Dialog4_C"))
      (UserInterface|Viewport|AddtoViewport _returnvalue_2 0))
    (:3
      (bind _returnvalue_3 (Actor|GetActorOfClass "/Script/LittleLights.PlayerCharacter"))
      (Game|Player|SetViewTargetwithBlend (Game|GetPlayerController 0) _returnvalue_3 2.0 "VTBlend_EaseIn" 1.0 false)
      (Utilities|FlowControl|Delay 2.0)
      (CallFunction|PlayerCanMove true))))

(event EventBeginPlay
  (bind _returnvalue (Game|GetPlayerController 0))
  (Input|DisableInput (Game|Player|GetPlayerPawn 0) _returnvalue)
  (Utilities|FlowControl|Delay 1.5)
  (bind _returnvalue_2 (UserInterface|CreateWidget "/Game/UIX/WBP_Intro_temp.WBP_Intro_temp_C"))
  (UserInterface|Viewport|AddtoViewport _returnvalue_2 0)
  (Input|SetInputModeUIOnly _returnvalue 0 "DoNotLock")
  (Variables|/Script/Engine.PlayerController|SetbShowMouseCursor _returnvalue true))

(event Collision|EventActorBeginOverlap
  (params (OtherActor :type Actor%20Object%20Reference))
  (|CallParentFunction OtherActor) ; This node is disabled and will not be called.\nDrag off pins to build functionality.
)

(event EventTick
  (params (DeltaSeconds :type Float%20%28single-precision%29))
  (|CallParentFunction DeltaSeconds) ; This node is disabled and will not be called.\nDrag off pins to build functionality.
)

(fn ConstructionScript
  (|CallParentFunction))

(fn GameStart
  (bind _returnvalue (Game|GetPlayerController 0))
  (Input|SetInputModeGameOnly _returnvalue)
  (Variables|/Script/Engine.PlayerController|SetbShowMouseCursor _returnvalue false)
  (Input|EnableInput (Game|Player|GetPlayerPawn 0) _returnvalue))