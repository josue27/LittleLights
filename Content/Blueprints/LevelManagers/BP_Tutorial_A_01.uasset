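; Level manager for the first tutorial, scripting its prompts, orb pickup beats and Golem guide.
; Extends a parent manager that handles dialogue and sequence playback, and stops the player character on BeginPlay.
; Events push timed control hints and video panels for crouch, jump-over and balance obstacles onto the tutorial widget's stack.
; Other events AI-move the Golem between placed points, turn it toward the player on arrival, and position both for conversation.
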(event Custom|ShowJumpControllers
  ;[0.1 0.15 0.2] Show Controllers tutorials
  (Default|PushWidgettoStack (Variables|Default|GetTutorialWBP) "/Game/UIX/Tutorial/WBP_TutorialController_JumpSprint.WBP_TutorialController_JumpSprint_C" "Press [Space] to Jump" true))

(event Custom|ShowSprintControllers
  ;[0.1 0.15 0.2] Show Controllers tutorials
  (Default|PushWidgettoStack (Variables|Default|GetTutorialWBP) "/Game/UIX/Tutorial/WBP_TutorialController_JumpSprint.WBP_TutorialController_JumpSprint_C" "Press [L Shift] to sprint" true))

(event Custom|SetFirstConversationLoc
  (bind _bp_player_controller (Variables|Default|GetBP%20Player%20Controller))
  (bind _golem (Variables|Default|GetGolem))
  (bind _player_firstconversation_loc (Variables|Default|GetPlayer_FirstConversation_Loc))
  (bind _golem_firstconversation_loc (Variables|Default|GetGolem_FirstConversation_Loc))
  (bind _returnvalue (Transformation|GetActorLocation _golem_firstconversation_loc))
  (bind _returnvalue_2 (Transformation|GetActorLocation _player_firstconversation_loc))
  ;[0.1 0.15 0.2] Rotate golem on pond fill conversation
  (Transformation|SetActorLocation _golem (Math|Vector|MakeVector (.x _returnvalue) (.y _returnvalue) (.z (Transformation|GetActorLocation _golem))) false false)
  (Transformation|SetActorLocation _bp_player_controller (Math|Vector|MakeVector (.x _returnvalue_2) (.y _returnvalue_2) (.z (Transformation|GetActorLocation _bp_player_controller))) false false))

(event Custom|FollowGolemToBalance
  ;[0.1 0.15 0.2] Follot balance log
  (Utilities|FlowControl|Sequence
    (:then_0
      (bind _golem (Variables|Default|GetGolem)
        (:then
          (AI|AIMoveTo _golem _golem (Transformation|GetActorLocation (Variables|Default|GetGolemBalanceObstacle)) 0 5.0 false
            (:OnSuccess
              (Transformation|SetActorRotation _golem (Math|Rotator|FindLookatRotation (Transformation|GetActorLocation _golem) (Transformation|GetActorLocation (Pawn|GetControlledPawn (Variables|Default|GetBP%20Player%20Controller))))))))
        (:else)))
    (:then_1
      (Default|PushWidgettoStack (Variables|Default|GetTutorialWBP) "/Game/UIX/Tutorial/WBP_TutorialController.WBP_TutorialController_C" "Keep following the Golem" true))))

(event Custom|FolloGolemToEnd
  (bind _golem (Variables|Default|GetGolem)
    (:then
      (AI|AIMoveTo _golem _golem (Transformation|GetActorLocation (Variables|Default|GetGolemEndLoc)) 0 5.0 false
        (:then
          (CallFunction|PauseSequence))
        (:OnSuccess
          (Transformation|SetActorRotation _golem (Math|Rotator|FindLookatRotation (Transformation|GetActorLocation _golem) (Transformation|GetActorLocation (Pawn|GetControlledPawn (Variables|Default|GetBP%20Player%20Controller))))))))
    (:else)))

(event Custom|PauseSequence
  ;[0.1 0.15 0.2] Pause Sequence
  (|CallParentFunction))

(event Custom|SpawnOrbInPlayer
  ;[0.1 0.15 0.2] Spawn the orb during pick
  (bind _asbp_player_character_tutorial_1 (Utilities|Casting|CastToBP_Player_Character_Tutorial_1 (Game|Player|GetPlayerPawn 0)))
  (Default|SpawnOrbTutorial _asbp_player_character_tutorial_1))

(event Custom|ShowMoveControllers
  ;[0.1 0.15 0.2] Show Controllers tutorials
  (Default|PushWidgettoStack (Variables|Default|GetTutorialWBP) "/Game/UIX/Tutorial/WBP_TutorialController.WBP_TutorialController_C" "Use [W A S D] to move" true))

(event Custom|ShowGrabControllers
  ;[0.1 0.15 0.2] Show Controllers tutorials
  (Default|PushWidgettoStack (Variables|Default|GetTutorialWBP) "/Game/UIX/Tutorial/WBP_TutorialController.WBP_TutorialController_C" "Use [ E ] to grab the ORB" true))

(event Custom|FinishOrbPickup
  (bind _asbp_player_character_tutorial_1 (Utilities|Casting|CastToBP_Player_Character_Tutorial_1 (Game|Player|GetPlayerPawn 0)))
  (Default|SetNewCameraView _asbp_player_character_tutorial_1))

(event Custom|Start%20Follow%20Golem
  ;[0.1 0.15 0.2] Follo golem to Pond fill (1st point)
  (bind _golem (Variables|Default|GetGolem)
    (:then
      (AI|AIMoveTo _golem _golem (Transformation|GetActorLocation (Variables|Default|GetGolemOrbPoint)) 0 5.0 false
        (:then
          (Utilities|FlowControl|DoOnce false
            (:Completed
              (CallFunction|ShowFollowGolem)
              (CallFunction|PlaySequence 42.0 true false))))
        (:OnSuccess
          (Transformation|SetActorRotation _golem (Math|Rotator|FindLookatRotation (Transformation|GetActorLocation _golem) (Transformation|GetActorLocation (Pawn|GetControlledPawn (Variables|Default|GetBP%20Player%20Controller))))))))
    (:else)))

(event Custom|ShowFollowGolem
  ;[0.1 0.15 0.2] Show Controllers tutorials
  (Default|PushWidgettoStack (Variables|Default|GetTutorialWBP) "/Game/UIX/Tutorial/WBP_TutorialController.WBP_TutorialController_C" "Follow the Golem" true))

(event EventBeginPlay
  (|CallParentFunction)
  (Utilities|FlowControl|Sequence
    (:then_0
      (bind _asbp_player_character_tutorial_1 (Utilities|Casting|CastToBP_Player_Character_Tutorial_1 (Game|Player|GetPlayerPawn 0)))
      (Class|PlayerCharacter|StopCharacter _asbp_player_character_tutorial_1))))

(event Collision|EventActorBeginOverlap
  (params (OtherActor :type Actor%20Object%20Reference))
  (|CallParentFunction OtherActor) ; This node is disabled and will not be called.\nDrag off pins to build functionality.
)

(event EventTick
  (params (DeltaSeconds :type Float%20%28single-precision%29))
  (|CallParentFunction DeltaSeconds) ; This node is disabled and will not be called.\nDrag off pins to build functionality.
)

(event EventShowPanel
  (params (Num :type Integer))
  (bind _tutorialwbp (Variables|Default|GetTutorialWBP))
  ;[0.1 0.15 0.2] Tutorial Panels
  (|CallParentFunction Num)
  (switch int Num
    (:Default
      (Development|PrintString "Panel selected invalid")
      (Variables|Default|SetTutorialPanelActive false))
    (:0
      (Default|PushPaneltoStack _tutorialwbp "/Game/UIX/Tutorial/WBP_TutorialPanel.WBP_TutorialPanel_C" "When Lucas encounters an obstacle he can <Highlight>crouch under</>, press the <Highlight>[E]</> key to interact with it.  
 
<Highlight>Three</> different arrows will appear one after another. <img id=\"ArrowUp\"/> They correspond to the movement directions. 
 
Press the corresponding direction before the time runs out, or you will fail." "Crouch Obstacle" "/Game/UIX/Assets2D/Tutoria_Thumb_01.Tutoria_Thumb_01" true)
      (Variables|Default|SetShouldPlayAfterClose false :!label _label))
    (:1
      (Default|PushPaneltoStack _tutorialwbp "/Game/UIX/Tutorial/WBP_TutorialPanel.WBP_TutorialPanel_C" "When Lucas encounters an obstacle he can <Highlight> jump over</>, press the <Highlight>[E]</> key to interact with it.  
 
<Highlight>Three</> different arrows will appear one after another. <img id=\"ArrowUp\"/> They correspond to the movement directions. 
 
Press the corresponding direction before the time runs out, or you will fail." "Jump Over" "/Game/UIX/Assets2D/Tutoria_Thumb_02.Tutoria_Thumb_02" true 1)
      (goto _label))
    (:2
      (Default|PushPaneltoStack _tutorialwbp "/Game/UIX/Tutorial/WBP_TutorialPanel.WBP_TutorialPanel_C" "When there is tree that Lucas can <Highlight>CROSS  OVER </>press the <Highlight>[E]</> key to interact with it. 
 
Move forward or backwards with <Highlight>ARROW UP  </> <img id=\"ArrowUp\"/>  
Balance yourself <Highlight>[ARROW LEFT]</> and <Highlight>[ARROW RIGHT] </> to keep the bar in the green area" "Cross balance" "/Game/UIX/Assets2D/Tutoria_Thumb_03.Tutoria_Thumb_03" true 2)
      (goto _label))))

(event EventShowNextDialogue
  (params (PauseTimeLine :type Boolean) (ShouldPlayAfterClose :type Boolean) (KeepDialoguePanel :type Boolean) (Player%20Can%20Move :type Boolean))
  (|CallParentFunction PauseTimeLine ShouldPlayAfterClose KeepDialoguePanel Player%20Can%20Move))

(event EventShowDialogue
  (params (Num :type Integer) (Pause :type Boolean) (ShoulPlayAfterClose :type Boolean) (KeepDialogue :type Boolean))
  (|CallParentFunction Num Pause ShoulPlayAfterClose KeepDialogue))

(event EventPlaySequence
  (params (Time :type Float%20%28single-precision%29) (Seconds :type Boolean) (ShouldPlay :type Boolean))
  (|CallParentFunction Time Seconds ShouldPlay))

(fn ConstructionScript
  (|CallParentFunction))