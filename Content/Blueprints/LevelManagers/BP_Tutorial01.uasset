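; BP_Tutorial01 is a level manager for the first tutorial that handles its intro screen and camera transition.
; On BeginPlay it runs the parent logic, sets the view to the initial camera (CamaraInicial) and shows the WBP_Intro_temp widget.
; Its GameStart override calls the parent, then blends the player's view to the gameplay camera (CamaraJuego) if that camera is valid.
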(event EventBeginPlay
  (bind _returnvalue (Game|GetPlayerController 0))
  (|CallParentFunction)
  (Game|Player|SetViewTargetwithBlend _returnvalue (Variables|Default|GetCamaraInicial) 0.0 "VTBlend_Linear" 0.0 false)
  (bind _returnvalue_2 (UserInterface|CreateWidget "/Game/UIX/WBP_Intro_temp.WBP_Intro_temp_C" _returnvalue))
  (UserInterface|Viewport|AddtoViewport _returnvalue_2 0))

(event Collision|EventActorBeginOverlap
  (params (OtherActor :type Actor%20Object%20Reference))
  (|CallParentFunction OtherActor) ; This node is disabled and will not be called.\nDrag off pins to build functionality.
)

(event EventTick
  (params (DeltaSeconds :type Float%20%28single-precision%29))
  (|CallParentFunction DeltaSeconds) ; This node is disabled and will not be called.\nDrag off pins to build functionality.
)

(fn ConstructionScript
  (|CallParentFunction))

(fn GameStart
  (bind _camarajuego (Variables|Default|GetCamaraJuego))
  (|CallParentFunction)
  (Utilities|IsValid _camarajuego
    (:Is%20Valid
      (Game|Player|SetViewTargetwithBlend (Variables|Default|GetPlayerController) _camarajuego 2.0 "VTBlend_Linear" 0.0 false))))