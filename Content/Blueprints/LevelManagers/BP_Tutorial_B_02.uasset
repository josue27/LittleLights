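; Level manager for tutorial B_02, extending a parent that supplies dialogue and panel behavior.
; On BeginPlay it loads the game and runs the intro, moving player and golem into place and creating the story widget.
; Event hooks move the golem, push obstacle panels (crouch, jump, balance) and pause the sequence for story frames, resuming it afterward.
; A trigger activates obstacle meshes; the return-from-level spawn logic is disconnected.
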(event OnActorBeginOverlap(TriggerObstacles)
  (params (OverlappedActor :type Actor%20Object%20Reference) (OtherActor :type Actor%20Object%20Reference))
  (Utilities|Casting|CastToBP_PlayerCharacter OtherActor)
  (for _array_element (Variables|TutorialB|GetObstaclesTutorial)
    (Default|ActivateMesh _array_element true))
  (Actor|DestroyActor (Variables|TutorialB|GetTriggerObstacles)))

(event Custom|GolemInCaveEntrance
  ;[0.1 0.15 0.2] Golem is in cave entrance
)

(event Custom|GolemIntroEnded
  ;[0.1 0.15 0.2] Golem Intro
  (CallFunction|ShowNextDialogue true true false true)
  (bind _golemtutorial (Variables|Default|GetGolemTutorial)
    (:then
      (bind _asbp_player_character_tutorial_1 (Utilities|Casting|CastToBP_Player_Character_Tutorial_1 (Game|Player|GetPlayerPawn 0))
        (:then
          (Transformation|SetActorRotation _golemtutorial (Math|Rotator|FindLookatRotation (Transformation|GetActorLocation _golemtutorial) (Transformation|GetActorLocation _asbp_player_character_tutorial_1))))
        (:CastFailed
          _))
      (EventDispatchers|UnbindEventfromAutomaticMovementFinished _golemtutorial (EventDispatchers|CreateEvent :!event Custom|GolemIntroEnded)))
    (:else)))

(event Custom|GameLoaded
  (params (bSuccess :type Boolean))
  ;[0.1 0.15 0.2] A game was loaded so we should spawn the player in other point
)

(event Custom|IntroTutorial
  (bind _returnvalue (Game|Player|GetPlayerPawn 0))
  ;[0.1 0.15 0.2] Intro tuotrial
  (Utilities|FlowControl|Sequence
    (:then_0
      (Input|DisableInput _returnvalue (Game|GetPlayerController 0))
      (bind _asbp_player_character (Utilities|Casting|CastToBP_PlayerCharacter _returnvalue))
      (Variables|/Script/LittleLights.LL_ToolsComponent|SetbStartWithOrb (Variables|/Script/LittleLights.PlayerCharacter|GetToolsComponent _asbp_player_character) true)
      (Default|MovePlayerto _asbp_player_character (Transformation|GetActorLocation (Variables|TutorialB|GetInitialLocation_0)) 4e+02 true true false)
      (EventDispatchers|BindEventtoOnAutomaticMovementEnded _asbp_player_character (EventDispatchers|CreateEvent :!event Custom|PlayerIntroFinished)))
    (:then_1
      (bind _golemtutorial (Variables|Default|GetGolemTutorial)
        (:then
          (Default|MovetoLocation _golemtutorial (Transformation|GetActorLocation (Variables|TutorialB|GetGolemInitialPoint)))
          (EventDispatchers|BindEventtoAutomaticMovementFinished _golemtutorial (EventDispatchers|CreateEvent :!event Custom|GolemIntroEnded)))
        (:else)))
    (:then_2
      (Utilities|Casting|CastToBP_Player_Character_Tutorial_1 (Game|Player|GetPlayerPawn 0)))
    (:then_3
      (Variables|/Script/LittleLights.LL_DialogueSubsystem|SetCharactersData (Subsystems|GetLLDialogueSubsystem) "/Game/DataTables/DT_SpeakersData.DT_SpeakersData"))
    (:then_4
      (bind _returnvalue_2 (UserInterface|CreateWidget "/Game/UIX/PlayerHUDs/Dialogue/WBP_StoryContainer.WBP_StoryContainer_C" (Game|GetPlayerController 0)))
      (bind _output_get (Variables|Default|SetWBP_StoryContainer _returnvalue_2))
      (UserInterface|Viewport|AddtoViewport _output_get 0))))

(event Custom|PlayerIntroFinished
  (params (PlayerCharacter :type Player%20Character%20Object%20Reference) (bLightUpTorch :type Boolean) (bStartDecay :type Boolean))
  ;[0.1 0.15 0.2] Intro tuotrial
)

(event Custom|MoveGolemInsideCave
  ;[0.1 0.15 0.2] Golem inside cave
  (Default|MovetoLocation (Variables|Default|GetGolemTutorial) (Transformation|GetActorLocation (Variables|TutorialB|GetGolemThirdPoint)))
  (Utilities|FlowControl|Delay 1.0))

(event Custom|MoveGolemToLocation
  (params (Destination :type Vector) (ShouldPauseSequence :type Boolean))
  ;[0.1 0.15 0.2] Move Golem to location
  (if (not (Variables|Default|GetTutorialPanelActive))
    (Utilities|FlowControl|Sequence
      (:then_0
        (if ShouldPauseSequence
          (CallFunction|PauseSequence)))
      (:then_1
        (bind _golemtutorial (Variables|Default|GetGolemTutorial)
          (:then
            (Default|MovetoLocation _golemtutorial Destination))
          (:else))))))

(event Custom|ShowStorySequence
  ;[0.1 0.15 0.2] StoryFrames
  (bind _wbp_storycontainer (Variables|Default|GetWBP_StoryContainer)
    (:then
      (Default|StartStoryFrame _wbp_storycontainer)
      (CallFunction|PauseSequence)
      (EventDispatchers|BindEventtoStoryFramesEnded _wbp_storycontainer (delegate Custom|StoryFramesEnded_Event)))
    (:else)))

(event Custom|EndStorySequence
  ;[0.1 0.15 0.2] StoryFrames
)

(event Custom|StoryFramesEnded_Event
  ;[0.1 0.15 0.2] StoryFrames
  (Audio|PlaySound2D "/Game/Audio/SFX/ScratchDisk/SFX_ScratchDisk.SFX_ScratchDisk" 1.5 1.0 0.0 0 0)
  (CallFunction|PlaySequence 0.0 false true))

(event Custom|OnDialogueAdvance_Event
  ;[0.1 0.15 0.2] Intro tuotrial
)

(event EventBeginPlay
  (bind _returnvalue (Subsystems|GetLLGameManager))
  (|CallParentFunction)
  (EventDispatchers|BindEventtoOnLoadGameCompleted _returnvalue (EventDispatchers|CreateEvent :!event Custom|GameLoaded))
  (Class|LLGameManager|LoadGame _returnvalue)
  (CallFunction|IntroTutorial))

(event Collision|EventActorBeginOverlap
  (params (OtherActor :type Actor%20Object%20Reference))
  (|CallParentFunction OtherActor) ; This node is disabled and will not be called.\nDrag off pins to build functionality.
)

(event EventTick
  (params (DeltaSeconds :type Float%20%28single-precision%29)))

(event EventShowNextDialogue
  (params (PauseTimeLine :type Boolean) (ShouldPlayAfterClose :type Boolean) (KeepDialoguePanel :type Boolean) (Player%20Can%20Move :type Boolean))
  ;[0.1 0.15 0.2] Dialogues Override
  (|CallParentFunction PauseTimeLine ShouldPlayAfterClose KeepDialoguePanel true))

(event EventShowPanel
  (params (Num :type Integer))
  (bind _tutorialwbp (Variables|Default|GetTutorialWBP))
  ;[0.1 0.15 0.2] PANELS SPECIALM MOVEMENTS TUORIALS
  (|CallParentFunction Num)
  (switch int Num
    (:Default
      (Development|PrintString "Panel selected invalid")
      (Variables|Default|SetTutorialPanelActive false))
    (:0
      (Default|PushPaneltoStack _tutorialwbp "/Game/UIX/Tutorial/WBP_TutorialPanel.WBP_TutorialPanel_C" "Remember if there is an obstacle that Lucas can crouh press the [E] key to interact with it after that 3 different keys will appear one after another press them before the time indicator finishes or you will fail and will need to repeat  the process" "Crouch obstacle" "/Game/UIX/Assets2D/Tutoria_Thumb_01.Tutoria_Thumb_01" true)
      (Variables|Default|SetShouldPlayAfterClose false :!label _label))
    (:1
      (Default|PushPaneltoStack _tutorialwbp "/Game/UIX/Tutorial/WBP_TutorialPanel.WBP_TutorialPanel_C" "When there is an obstacle that Lucas can jump  press the [E] key to interact with it after that 3 different keys will appear one after another press them before the time indicator finishes or you will fail and will need to repeat  the process" "Jump Over" "/Game/UIX/Assets2D/Tutoria_Thumb_02.Tutoria_Thumb_02" true 1)
      (goto _label))
    (:2
      (Default|PushPaneltoStack _tutorialwbp "/Game/UIX/Tutorial/WBP_TutorialPanel.WBP_TutorialPanel_C" "When there is tree that Lucas can CROSS  press the [E] key to interact with it 
Move forward with [ W ] 
Balance yourself [A] and [D] so the bar doesnt get to the red zone" "Cross balance" "/Game/UIX/Assets2D/Tutoria_Thumb_03.Tutoria_Thumb_03" true 2)
      (goto _label))))

(fn ConstructionScript
  (|CallParentFunction))