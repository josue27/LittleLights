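; BP_Tutorial_C_01 is a tutorial level manager that starts the level's sequence and directs the tutorial golem.
; It binds to the player character's automatic-movement-ended event and plays the level sequence the first time it fires, guarded by a DialogueDisplayed flag marked as hacky.
; MoveGolemToLocation sends the golem to a destination while no tutorial panel is active, optionally pausing the sequence first.
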(event Custom|OnAutomaticMovementEnded_Event_0
  (params (PlayerCharacter :type Player%20Character%20Object%20Reference) (bLightUpTorch :type Boolean) (bStartDecay :type Boolean))
  ;[0.1564 0.2 0.1287] HACKY
  (if (not (Variables|Default|GetDialogueDisplayed))
    (Variables|Default|SetDialogueDisplayed true)
    (Sequencer|Player|Play (Variables|/Script/LevelSequence.LevelSequenceActor|GetSequencePlayer (Variables|Default|GetLevelSequence)) :!class /Script/MovieScene.MovieSceneSequencePlayer)))

(event Custom|MoveGolemToLocation
  (params (Destination :type Vector) (ShouldPauseSequence :type Boolean))
  ;[0.1 0.15 0.2] Move Golem to location
  (if (not (Variables|Default|GetTutorialPanelActive))
    (Utilities|FlowControl|Sequence
      (:then_0
        (if ShouldPauseSequence
          (CallFunction|PauseSequence)))
      (:then_1
        (bind _golemtutorial (Variables|Default|GetGolemTutorial)
          (:then
            (Default|MovetoLocation _golemtutorial Destination))
          (:else))))))

(event EventBeginPlay
  (|CallParentFunction)
  (bind _asbp_player_character (Utilities|Casting|CastToBP_PlayerCharacter (Game|GetPlayerCharacter 0)))
  (EventDispatchers|AssignOnAutomaticMovementEnded _asbp_player_character (delegate Custom|OnAutomaticMovementEnded_Event_0))
  (Development|PrintString "GM: Binded"))

(event EventTick
  (params (DeltaSeconds :type Float%20%28single-precision%29))
  (|CallParentFunction DeltaSeconds) ; This node is disabled and will not be called.\nDrag off pins to build functionality.
)

(fn ConstructionScript
  (|CallParentFunction))