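; Base level manager actor that handles level timing data, game over, restarts and level transitions, with empty hooks for countdown and dialog events.
; Its construction script reads the current level's time from the game instance's level list.
; GameOver locks player input and shows the game-over widget, while completed levels fade before opening NextLevel.
; A timeline brightens the moonlight after zeroing a fog parameter; beast activation is stubbed, its spawn code disconnected.
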(event Custom|DialogEnded
  (params (NumEvent :type Integer)))

(event Custom|RestartLevel
  ;[1 1 1] Restart Game
  (bind _returnvalue (Game|GetCurrentLevelName true))
  (Game|OpenLevel(byName) (Utilities|String|StringToName _returnvalue)))

(event Custom|StartCountDown)

(event Custom|ChangeToNextLevel
  ;[1 1 1] ChangeLevel
  (if (Utilities|Enum|Equal(Enum) (Variables|Default|GetCurrentGameState) "LevelCompleted")
    ;;[1 1 1] Sequence UI trees
    (bind _returnvalue (UserInterface|CreateWidget "/Game/UIX/WBP_Fade.WBP_Fade_C"))
    (UserInterface|Viewport|AddtoViewport _returnvalue 0)
    (Default|StartFadein _returnvalue)
    (bind _fadetime (Default|GetFadeinLenght _returnvalue))
    (Utilities|FlowControl|Delay _fadetime)
    (Game|OpenLevel(byObjectReference) (Variables|Default|GetNextLevel))))

(event EventBeginPlay)

(event Collision|EventActorBeginOverlap
  (params (OtherActor :type Actor%20Object%20Reference)))

(event EventTick
  (params (DeltaSeconds :type Float%20%28single-precision%29)))

(event EventLightUpMoon
  ;[1 1 1] Turn on Directional Moon Light
  (Rendering|Material|SetScalarParameterValue "/Game/Material/MC_Fog_Parametros.MC_Fog_Parametros" "DivideMultiplier" 0.0 :!class /Script/Engine.KismetMaterialLibrary)
  (bind _finaldirectionallight (Variables|Default|GetFinalDirectionalLight)
    (:then
      (bind _delta (Timeline|MoonIntensityAnim Play)
        (:Update
          (Rendering|Components|Light|SetIntensity (Variables|/Script/Engine.Light|GetLightComponent _finaldirectionallight) (Math|Float|Lerp 0.0 1e+01 _delta)))))
    (:else)))

(fn ConstructionScript
  (CallFunction|SetLevelTimer))

(fn SetLevelTimer
  (bind _asbp_ll_game_instance (Utilities|Casting|CastToBP_LL_GameInstance (Game|GetGameInstance)))
  (bind _returnvalue (Game|GetCurrentLevelName true))
  (bind _array_element (Utilities|Array|ForEachLoopwithBreak (Variables|/Game/Blueprints/BP_LL_GameInstance.BP_LL_GameInstance_C|GetNiveles _asbp_ll_game_instance) :!label _label)
    (:LoopBody
      (if (Utilities|Enum|Equal(Enum) _returnvalue (Utilities|String|ToString(Name) (.nombrenivel _array_element)))
        (Variables|Default|SetLevelTIme (.tiemponivel _array_element))
        (goto _label Break)))))

(fn GameOver
  (Development|PrintString "Out of time")
  (bind _asbp_player_character (Utilities|Casting|CastToBP_PlayerCharacter (Game|Player|GetPlayerPawn 0)))
  (Default|ToggleInput _asbp_player_character false)
  (Variables|/Script/LittleLights.PlayerCharacter|SetbCanMove _asbp_player_character false)
  (Variables|Default|SetCanCountDown false)
  (bind _returnvalue (UserInterface|CreateWidget "/Game/UIX/PlayerHUDs/WBP_GameOver.WBP_GameOver_C"))
  (UserInterface|Viewport|AddtoViewport _returnvalue 0))

(fn ActivateBeast)

(fn GetGameState
  (return (Variables|Default|GetCurrentGameState)))