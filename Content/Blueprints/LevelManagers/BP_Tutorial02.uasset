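; Level manager for the second tutorial, handling the intro camera and the handover to gameplay.
; On BeginPlay, with a valid intro camera, it blends the view there, disables player input and shows an intro widget.
; Its GameStart override blends to the gameplay camera, restores input and triggers SpawnBengala, which spawns a flare actor at a marker point after a short delay.
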(event Custom|SpawnBengala
  (bind _puntoflarespawn (Variables|Default|GetPuntoFlareSpawn))
  (Utilities|FlowControl|Delay 2.0)
  (Game|SpawnActorfromClass "/Game/Blueprints/BP_Bengala.BP_Bengala_C" (Math|Transform|MakeTransform (Transformation|GetActorLocation _puntoflarespawn) (Transformation|GetActorRotation _puntoflarespawn) "1,1,1") "Undefined" 0 0))

(event EventBeginPlay
  (bind _camarainicial (Variables|Default|GetCamaraInicial))
  (|CallParentFunction)
  (Utilities|IsValid _camarainicial
    (:Is%20Valid
      (Game|Player|SetViewTargetwithBlend (Variables|Default|GetPlayerController) _camarainicial 2.0 "VTBlend_Linear" 0.0 false)
      (bind _asbp_player_character (Utilities|Casting|CastToBP_PlayerCharacter (Game|Player|GetPlayerPawn 0)))
      (Default|ToggleInput _asbp_player_character false)
      (bind _returnvalue (UserInterface|CreateWidget "/Game/UIX/WBP_Intro2_tmp.WBP_Intro2_tmp_C"))
      (UserInterface|Viewport|AddtoViewport _returnvalue 0))))

(event Collision|EventActorBeginOverlap
  (params (OtherActor :type Actor%20Object%20Reference))
  (|CallParentFunction OtherActor) ; This node is disabled and will not be called.\nDrag off pins to build functionality.
)

(event EventTick
  (params (DeltaSeconds :type Float%20%28single-precision%29))
  (|CallParentFunction DeltaSeconds) ; This node is disabled and will not be called.\nDrag off pins to build functionality.
)

(fn ConstructionScript
  (|CallParentFunction))

(fn GameStart
  (bind _camarajuego (Variables|Default|GetCamaraJuego))
  (|CallParentFunction)
  (Utilities|IsValid _camarajuego
    (:Is%20Valid
      (Game|Player|SetViewTargetwithBlend (Variables|Default|GetPlayerController) _camarajuego 2.0 "VTBlend_Linear" 0.0 false)
      (bind _asbp_player_character (Utilities|Casting|CastToBP_PlayerCharacter (Game|Player|GetPlayerPawn 0)))
      (Default|ToggleInput _asbp_player_character true)
      (CallFunction|SpawnBengala))))