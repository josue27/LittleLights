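; Level manager for the third tutorial level that runs its opening sequence on BeginPlay.
; After the parent BeginPlay and a validity check, it blends the player controller's view target, toggles player character input off and calls SetLevelTimer.
; It then adds the Tutorial 03 intro widget to the viewport.
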(event EventBeginPlay
  (|CallParentFunction)
  (Utilities|IsValid 0
    (:Is%20Valid
      (Game|Player|SetViewTargetwithBlend (Variables|Default|GetPlayerController) 0 2.0 "VTBlend_Linear" 0.0 false)
      (bind _asbp_player_character (Utilities|Casting|CastToBP_PlayerCharacter (Game|Player|GetPlayerPawn 0)))
      (Default|ToggleInput _asbp_player_character false)
      (CallFunction|SetLevelTimer)
      (bind _returnvalue (UserInterface|CreateWidget "/Game/Blueprints/Tutorial_03/WBP_Intro_Tutorial03.WBP_Intro_Tutorial03_C"))
      (UserInterface|Viewport|AddtoViewport _returnvalue 0))))

(event Collision|EventActorBeginOverlap
  (params (OtherActor :type Actor%20Object%20Reference))
  (|CallParentFunction OtherActor) ; This node is disabled and will not be called.\nDrag off pins to build functionality.
)

(event EventTick
  (params (DeltaSeconds :type Float%20%28single-precision%29))
  (|CallParentFunction DeltaSeconds) ; This node is disabled and will not be called.\nDrag off pins to build functionality.
)

(fn ConstructionScript
  (|CallParentFunction))