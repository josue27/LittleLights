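; BP_Bloque_Bosque is a forest block that can randomly rearrange its two pines and three white-flower bushes.
; NuevoOrdenElemntos loops over those components and moves each to a random world position within the Box component's bounds, setting only X and Y from the random point.
; The event graph and construction script are empty, so nothing in this Blueprint calls the shuffle itself.
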(event EventBeginPlay)

(event Collision|EventActorBeginOverlap
  (params (OtherActor :type Actor%20Object%20Reference)))

(event EventTick
  (params (DeltaSeconds :type Float%20%28single-precision%29)))

(fn ConstructionScript)

(fn NuevoOrdenElemntos
  (bind _box (Variables|Default|GetBox))
  (bind (_origin _boxextent) (Collision|GetComponentBounds _box))
  (bind _returnvalue (Math|Random|RandomPointinBoundingBox _origin (Math|Vector|MakeVector (.x _boxextent) (.y _boxextent) (.z _boxextent))))
  (for _array_element (Utilities|Array|MakeArray (Variables|Default|GetPino_L1) (Variables|Default|GetArbusto_FloresBlancas1) (Variables|Default|GetArbusto_FloresBlancas) (Variables|Default|GetArbusto_FloresBlancas2) (Variables|Default|GetPino_L))
    (Transformation|SetWorldLocation _array_element (Math|Vector|MakeVector (.x _returnvalue) (.y _returnvalue) 0.0) false false)))