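; BP_StartDoor is a door that blocks the player character with a warning dialogue when it hits the door's box.
; A hit stops the character and shows the warning through the player controller, with a flag preventing repeat triggers.
; The bound dialogue-advance event hides the dialogue, resumes movement and clears the flag.
; A particle system activates shortly after BeginPlay.
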(event OnComponentHit(Box)
  (params (HitComponent :type Primitive%20Component%20Object%20Reference) (OtherActor :type Actor%20Object%20Reference) (OtherComp :type Primitive%20Component%20Object%20Reference) (NormalImpulse :type Vector :default "0, 0, 0") (Hit :type Hit%20Result%20Structure%20%28by%20ref%29))
  (bind _asbp_player_character (Utilities|Casting|CastToBP_PlayerCharacter OtherActor))
  (bind _output_get (Variables|Default|SetAs%20BP%20Player%20Character _asbp_player_character))
  (if (not (Variables|Default|GetDisplayingMsg))
    (Variables|Default|SetDisplayingMsg true)
    (EventDispatchers|AssignOnDialogueAdvance _output_get (delegate Custom|InteractionEvent))
    (Class|PlayerCharacter|StopCharacter _output_get)
    (Development|PrintString "HALO")
    (bind _asbp_player_controller (Utilities|Casting|CastToBP_PlayerController (Game|GetPlayerController 0)))
    (Class|LLPlayerControllerBase|ShowDialogue _asbp_player_controller (Variables|Default|GetDoorWarningDialogue) true)))

(event Custom|InteractionEvent
  (bind _asbp_player_controller (Utilities|Casting|CastToBP_PlayerController (Game|GetPlayerController 0)))
  (Class|LLPlayerControllerBase|ShowDialogue :self _asbp_player_controller)
  (Class|PlayerCharacter|ContinueMovement (Variables|Default|GetAs%20BP%20Player%20Character))
  (Variables|Default|SetDisplayingMsg false))

(event EventBeginPlay
  (Utilities|FlowControl|Delay 0.2)
  (Components|Activation|Activate (Variables|Default|GetParticleSystem) false))

(event Collision|EventActorBeginOverlap
  (params (OtherActor :type Actor%20Object%20Reference)))

(event EventTick
  (params (DeltaSeconds :type Float%20%28single-precision%29)))

(fn ConstructionScript)