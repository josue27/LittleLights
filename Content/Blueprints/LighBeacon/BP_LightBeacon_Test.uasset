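; BP_LightBeacon_Test is a light beacon that the player lights by delivering fragments.
; Its point light starts dark, and player overlap with the trigger moves all carried fragments into the beacon's running total.
; Reaching the required count, or needing none, plays a timeline that raises light intensity and radius.
; The same timeline drives the fog's exponential radius through a Material Parameter Collection.
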(event OnComponentBeginOverlap(Trigger)
  (params (OverlappedComponent :type Primitive%20Component%20Object%20Reference) (OtherActor :type Actor%20Object%20Reference) (OtherComp :type Primitive%20Component%20Object%20Reference) (OtherBodyIndex :type Integer) (bFromSweep :type Boolean) (SweepResult :type Hit%20Result%20Structure%20%28by%20ref%29))
  (bind _asbp_personaje_jugador (Utilities|Casting|CastToBP_PersonajeJugador OtherActor))
  (if (> (Variables|Default|GetFragmentsRequired) 0)
    (if (> (Variables|/Script/LittleLights.Personaje|GetFragmentsAmount _asbp_personaje_jugador) 0)
      (bind _output_get (Variables|Default|SetFragmentsRecieved (+ (Variables|/Script/LittleLights.Personaje|GetFragmentsAmount _asbp_personaje_jugador) (Variables|Default|GetFragmentsRecieved))))
      (Variables|/Script/LittleLights.Personaje|SetFragmentsAmount _asbp_personaje_jugador 0)
      (if (>= _output_get (Variables|Default|GetFragmentsRequired))
        (CallFunction|TurnonBeacon)))
    (else
      (CallFunction|TurnonBeacon))))

(event Custom|TurnOnBeacon
  (bind _pointlight (Variables|Default|GetPointLight))
  ;[1 1 1] Turning Beacon On
  (bind (_direction _lightintensity _radius _fogradiusexp) (Timeline|LigthtingOn PlayFromStart)
    (:Update
      (Rendering|Components|Light|SetIntensity _pointlight (* _lightintensity 1e+03))
      (Rendering|Lighting|SetAttenuationRadius _pointlight (* _radius 1e+03))
      (Rendering|Material|SetScalarParameterValue "/Game/Material/MC_Fog_Parametros.MC_Fog_Parametros" "RadiusExponential" _fogradiusexp :!class /Script/Engine.KismetMaterialLibrary))))

(event EventBeginPlay
  (bind _pointlight (Variables|Default|GetPointLight))
  (|CallParentFunction)
  (Rendering|Components|Light|SetIntensity _pointlight 0.0)
  (Rendering|Lighting|SetAttenuationRadius _pointlight 0.0))

(event Collision|EventActorBeginOverlap
  (params (OtherActor :type Actor%20Object%20Reference))
  (|CallParentFunction OtherActor) ; This node is disabled and will not be called.\nDrag off pins to build functionality.
)

(event EventTick
  (params (DeltaSeconds :type Float%20%28single-precision%29))
  (|CallParentFunction DeltaSeconds) ; This node is disabled and will not be called.\nDrag off pins to build functionality.
)

(fn ConstructionScript
  (|CallParentFunction))