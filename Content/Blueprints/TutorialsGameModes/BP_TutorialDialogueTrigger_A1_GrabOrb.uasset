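; Interactable tutorial trigger, named for the A1 grab-orb step, that starts a tutorial sequence or dialogue when the player character interacts with it.
; Interact either plays BPTutorial's sequence player or has TutorialManager show the configured dialogue with pause and play-after-close options, depending on UseTimeline.
; It can optionally destroy itself afterward, and supplies its interaction prompt from TextToDisplay.
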(event EventBeginPlay)

(event Collision|EventActorBeginOverlap
  (params (OtherActor :type Actor%20Object%20Reference)))

(event EventTick
  (params (DeltaSeconds :type Float%20%28single-precision%29)))

(event EventInteract
  (params (InstigatorPawn :type Pawn%20Object%20Reference))
  (Utilities|Casting|CastToBP_PlayerCharacter InstigatorPawn)
  (if (Variables|Default|GetUseTimeline)
    (Sequencer|Player|Play (Variables|/Script/LevelSequence.LevelSequenceActor|GetSequencePlayer (Variables|Default|GetBP_Tutorial)) :!class /Script/MovieScene.MovieSceneSequencePlayer)
    (else
      (Default|ShowDialog (Variables|Default|GetTutorialManager) (Variables|Default|GetDialogueToDisplay) (Variables|Default|GetPausTimeLine) (Variables|Default|GetShoul%20Play%20After%20Close))))
  (if (Variables|Default|GetDestroyAfterActivation)
    (Actor|DestroyActor)))

(fn ConstructionScript)

(fn GetInteractText
  (params (InstigatorPawn :type Pawn%20Object%20Reference))
  (return (Variables|Default|GetTextToDisplay)))