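; Game mode for Tutorial A that sets up dialogue data and handles transitions to other levels.
; BeginPlay assigns the speakers table to the dialogue subsystem and casts the player pawn, while Tick clears the fog-of-war reveal render target to black every frame.
; ChangeLevel restores game-only input, plays a fade widget, then opens the given level after a delay.
; DialogEnded looks up tutorial managers but does nothing with them.
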(event Custom|DialogEnded
  (params (NewParam :type Boolean))
  (bind _outactors (Actor|GetAllActorsOfClass "/Game/Blueprints/LevelManagers/BP_TutorialManager_Base.BP_TutorialManager_Base_C")))

(event Custom|ChangeLevel
  (params (Level :type World%20Soft%20Object%20Reference))
  (Input|SetInputModeGameOnly (Game|GetPlayerController 0) false)
  (bind _returnvalue (UserInterface|CreateWidget "/Game/UIX/MainMenu/WBP_LevelTransition.WBP_LevelTransition_C"))
  (UserInterface|Viewport|AddtoViewport _returnvalue 0)
  (Default|FadeinSequence _returnvalue)
  (Utilities|FlowControl|Delay 2.0)
  (Game|OpenLevel(byObjectReference) Level))

(event EventBeginPlay
  (Variables|/Script/LittleLights.LL_DialogueSubsystem|SetCharactersData (Subsystems|GetLLDialogueSubsystem) "/Game/DataTables/DT_SpeakersData.DT_SpeakersData")
  (bind _asbp_player_character (Utilities|Casting|CastToBP_PlayerCharacter (Game|Player|GetPlayerPawn 0))))

(event EventTick
  (params (DeltaSeconds :type Float%20%28single-precision%29))
  (Rendering|ClearRenderTarget2D "/Game/FogOfWarSystem/FogOfWarReveal_Render.FogOfWarReveal_Render"))

(fn ConstructionScript)