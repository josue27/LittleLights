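; Base tutorial trigger actor that fires when the player overlaps its collider while enabled, or on BeaconCompleted if that check is set.
; ActivateUsing selects the action: play its level sequence, or have TutorialManager show a panel, jump to a sequence time, or show next or specific dialogue.
; Successful actions wait briefly, call ActivateObjectsOnList, then optionally destroy the trigger.
; It also implements interact-text getters.
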(event OnComponentBeginOverlap(TriggerCollider)
  (params (OverlappedComponent :type Primitive%20Component%20Object%20Reference) (OtherActor :type Actor%20Object%20Reference) (OtherComp :type Primitive%20Component%20Object%20Reference) (OtherBodyIndex :type Integer) (bFromSweep :type Boolean) (SweepResult :type Hit%20Result%20Structure%20%28by%20ref%29))
  (bind _bshouldplayafterclose (Variables|Default|GetbShouldPlayAfterClose))
  (bind _dialoguetodisplay (Variables|Default|GetDialogueToDisplay))
  (bind _bpausetimeline (Variables|Default|GetbPauseTimeLine))
  (bind _tutorialmanager (Variables|Default|GetTutorialManager))
  (if (Variables|Default|GetbEnabled)
    (Utilities|Casting|CastToBP_PlayerCharacter OtherActor)
    ;[0.1 0.15 0.2] Comment
    (switch Utilities|FlowControl|Switch|SwitchonELLDialogueActivationType (Variables|Default|GetActivateUsing)
      (:Timeline
        (Sequencer|Player|Play (Variables|/Script/LevelSequence.LevelSequenceActor|GetSequencePlayer (Variables|Default|GetLevelSequence)) :!class /Script/MovieScene.MovieSceneSequencePlayer)
        (Utilities|FlowControl|Delay 1.0 :!label _label)
        (Class|LLGameplayInterface|ActivateObjectsonList)
        (if (Variables|Default|GetbDestroyAfterActivation)
          (Actor|DestroyActor)))
      (:ShowPanel
        (bind _tutorialmanager_2 (Variables|Default|GetTutorialManager)
          (:then
            (Default|ShowPanel _tutorialmanager_2 (Variables|Default|GetPanelToDisplay))
            (goto _label))
          (:else)))
      (:JumpToTime
        (bind _tutorialmanager_3 (Variables|Default|GetTutorialManager)
          (:then
            (Default|PlaySequence _tutorialmanager_3 (Variables|Default|GetTimeInSequence) true true)
            (goto _label))
          (:else)))
      (:ShowNextDialogue
        (Default|ShowNextDialogue _tutorialmanager _bpausetimeline _bshouldplayafterclose false)
        (goto _label))
      (:ShowSpecificDialogue
        (if (>= _dialoguetodisplay 0)
          (Default|ShowDialogue _tutorialmanager _dialoguetodisplay _bpausetimeline _bshouldplayafterclose false)
          (goto _label)
          (else
            (Development|PrintString "No Valid Dialogue")))))))

(event EventBeginPlay)

(event Collision|EventActorBeginOverlap
  (params (OtherActor :type Actor%20Object%20Reference)))

(event EventTick
  (params (DeltaSeconds :type Float%20%28single-precision%29)))

(event EventBeaconCompleted
  (bind _bshouldplayafterclose (Variables|Default|GetbShouldPlayAfterClose))
  (bind _dialoguetodisplay (Variables|Default|GetDialogueToDisplay))
  (bind _bpausetimeline (Variables|Default|GetbPauseTimeLine))
  (bind _tutorialmanager (Variables|Default|GetTutorialManager))
  (if (Variables|LLDialogue|GetCheckBeaconCompleted)
    ;[0.1 0.15 0.2] Comment
    (switch Utilities|FlowControl|Switch|SwitchonELLDialogueActivationType (Variables|Default|GetActivateUsing)
      (:Timeline
        (Sequencer|Player|Play (Variables|/Script/LevelSequence.LevelSequenceActor|GetSequencePlayer (Variables|Default|GetLevelSequence)) :!class /Script/MovieScene.MovieSceneSequencePlayer)
        (Utilities|FlowControl|Delay 1.0 :!label _label)
        (Class|LLGameplayInterface|ActivateObjectsonList)
        (if (Variables|Default|GetbDestroyAfterActivation)
          (Actor|DestroyActor)))
      (:ShowPanel
        (bind _tutorialmanager_2 (Variables|Default|GetTutorialManager)
          (:then
            (Default|ShowPanel _tutorialmanager_2 (Variables|Default|GetPanelToDisplay))
            (goto _label))
          (:else)))
      (:JumpToTime
        (bind _tutorialmanager_3 (Variables|Default|GetTutorialManager)
          (:then
            (Default|PlaySequence _tutorialmanager_3 (Variables|Default|GetTimeInSequence) true true)
            (goto _label))
          (:else)))
      (:ShowNextDialogue
        (Default|ShowNextDialogue _tutorialmanager _bpausetimeline _bshouldplayafterclose false)
        (goto _label))
      (:ShowSpecificDialogue
        (if (>= _dialoguetodisplay 0)
          (Default|ShowDialogue _tutorialmanager _dialoguetodisplay _bpausetimeline _bshouldplayafterclose false)
          (goto _label)
          (else
            (Development|PrintString "No Valid Dialogue")))))))

(fn ConstructionScript)

(fn GetInteractTextDisplay
  (params (InstigatorPawn :type Pawn%20Object%20Reference))
  (return (Variables|Default|GetTextToDisplay)))

(fn GetInteractText
  (params (InstigatorPawn :type Pawn%20Object%20Reference))
  (return ""))