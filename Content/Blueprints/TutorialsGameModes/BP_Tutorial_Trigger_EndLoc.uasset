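; Tutorial trigger volume that ends the current tutorial section and sends the player on to Tutorial_B_03.
; When BP_Player_Character_Tutorial_1 overlaps the box and EndLoc is valid, it moves the player to that actor's location without lighting the orb or starting its decay.
; It then calls ChangeLevel on BP_Tutorial_A_GM, with the destination level hardcoded.
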(event OnComponentBeginOverlap(Box)
  (params (OverlappedComponent :type Primitive%20Component%20Object%20Reference) (OtherActor :type Actor%20Object%20Reference) (OtherComp :type Primitive%20Component%20Object%20Reference) (OtherBodyIndex :type Integer) (bFromSweep :type Boolean) (SweepResult :type Hit%20Result%20Structure%20%28by%20ref%29))
  (bind _asbp_player_character_tutorial_1 (Utilities|Casting|CastToBP_Player_Character_Tutorial_1 OtherActor))
  (bind _endloc (Variables|Default|GetEndLoc)
    (:then
      (Class|PlayerCharacter|MovePlayerto _asbp_player_character_tutorial_1 (Transformation|GetActorLocation _endloc) 1.5e+02 false false false)
      (bind _asbp_tutorial_a_gm (Utilities|Casting|CastToBP_Tutorial_A_GM (Game|GetGameMode)))
      (Default|ChangeLevel _asbp_tutorial_a_gm "/Game/Maps/Tutorials/Tutorial_B_03.Tutorial_B_03"))
    (:else)))

(event EventBeginPlay
  (|CallParentFunction) ; This node is disabled and will not be called.\nDrag off pins to build functionality.
)

(event EventTick
  (params (DeltaSeconds :type Float%20%28single-precision%29))
  (|CallParentFunction DeltaSeconds) ; This node is disabled and will not be called.\nDrag off pins to build functionality.
)

(fn ConstructionScript
  (|CallParentFunction))