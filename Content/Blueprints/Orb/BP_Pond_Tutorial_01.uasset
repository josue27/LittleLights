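; Tutorial pond interactable where the player fills their Orb, advancing the tutorial.
; On first interaction in tutorial mode it halts Orb decay, stops the character and plays the fill montage.
; After a delay it signals refill completion, advances the tutorial actor's dialogue and golem follow, spawns the tutorial orb and switches camera.
; A delayed, self-described hacky follow-up stops decay again and resets the refill flag.
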(event EventBeginPlay)

(event Collision|EventActorBeginOverlap
  (params (OtherActor :type Actor%20Object%20Reference)))

(event EventTick
  (params (DeltaSeconds :type Float%20%28single-precision%29)))

(event EventInteract
  (params (InstigatorPawn :type Pawn%20Object%20Reference))
  (if (Variables|Default|GetbIsTutorial)
    (if (not (Variables|Default|GetbCompleted))
      (bind _asbp_player_character_tutorial_1 (Utilities|Casting|CastToBP_Player_Character_Tutorial_1 InstigatorPawn))
      (bind _orb (Variables|/Script/LittleLights.LL_ToolsComponent|GetOrb (Variables|/Script/LittleLights.PlayerCharacter|GetToolsComponent _asbp_player_character_tutorial_1))
        (:then
          (Class|LLOrb|StopDecay _orb))
        (:else
          _))
      (Class|PlayerCharacter|StopCharacter _asbp_player_character_tutorial_1)
      (Animation|PlayAnimMontage _asbp_player_character_tutorial_1 "/Game/Animation/LucasControl/Lucas_FillOrb_Montage.Lucas_FillOrb_Montage" 1.0 "None")
      ;[0.1 0.15 0.2] 23
      (Variables|Default|SetbCompleted true)
      (Utilities|FlowControl|Delay 2.7)
      (Class|PlayerCharacter|StopCharacter _asbp_player_character_tutorial_1)
      (Class|LLToolsComponent|OrbRefillFinishedTutorial (Variables|/Script/LittleLights.PlayerCharacter|GetToolsComponent _asbp_player_character_tutorial_1) true)
      (Utilities|FlowControl|Sequence
        (:then_0
          (bind _returnvalue (Actor|GetActorOfClass "/Game/Blueprints/LevelManagers/BP_Tutorial_A_01.BP_Tutorial_A_01_C"))
          (Utilities|IsValid _returnvalue
            (:Is%20Valid
              (Default|ShowNextDialogue _returnvalue true false false true)
              (Utilities|FlowControl|Delay 1.0)
              (Default|FollowGolemtoBalance _returnvalue))))
        (:then_1
          (Default|SpawnOrbTutorial _asbp_player_character_tutorial_1)
          (Default|SetNewCameraView _asbp_player_character_tutorial_1))
        (:then_2
          ;[0.1 0.15 0.2] Hacky
          (Utilities|FlowControl|Delay 3.0)
          (Class|LLOrb|StopDecay (Variables|/Script/LittleLights.LL_ToolsComponent|GetOrb (Variables|/Script/LittleLights.PlayerCharacter|GetToolsComponent _asbp_player_character_tutorial_1)))
          ;[1 1 1] HACKY
          (Class|LLToolsComponent|OrbRefillFinishedTutorial (Variables|/Script/LittleLights.PlayerCharacter|GetToolsComponent _asbp_player_character_tutorial_1) false))))))

(fn ConstructionScript
  (|CallParentFunction))