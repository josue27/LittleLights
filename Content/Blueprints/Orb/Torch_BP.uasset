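; Torch Blueprint with a liquid orb material whose glow follows an intensity value.
; The construction script creates a dynamic instance of the liquid material on the DMLiquid component and caches its starting emission.
; Every Tick sets that emission by lerping from a base of one to the cached value, using DeltaIntensity as alpha.
; Nothing in these graphs writes DeltaIntensity.
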(event EventBeginPlay)

(event Collision|EventActorBeginOverlap
  (params (OtherActor :type Actor%20Object%20Reference)))

(event EventTick
  (params (DeltaSeconds :type Float%20%28single-precision%29))
  ;[1 1 1] Emission Update of the material orb
  (Rendering|Material|SetScalarParameterValue (Variables|Default|GetOrbMaterial_Inst) (Variables|Default|GetEmissionParameter) (Math|Float|Lerp 1.0 (Variables|Default|GetInitialEmission) (Variables|Default|GetDeltaIntensity)) :!class /Script/Engine.MaterialInstanceDynamic))

(fn ConstructionScript
  (bind _returnvalue (Rendering|Material|CreateDynamicMaterialInstance (Variables|Default|GetDM_Liquid) 0 "/Game/Materials/Instances/OrbStick/MI_Liquid.MI_Liquid" "None" :!class /Script/Engine.PrimitiveComponent))
  (bind _output_get (Variables|Default|SetOrbMaterial_Inst _returnvalue))
  (bind _returnvalue_2 (Rendering|Material|GetScalarParameterValue _output_get (Variables|Default|GetEmissionParameter) :!class /Script/Engine.MaterialInstanceDynamic))
  (Variables|Default|SetInitialEmission _returnvalue_2))