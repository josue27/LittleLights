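; Tutorial torch orb that the player character can light when standing near it.
; Overlapping its Sphere sets this actor as the player character's LanterOrb reference, and leaving clears it.
; The TurnOn event plays the IntensityOrb timeline from the start to drive the TorchLight intensity.
; GetInteractText returns an empty string.
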(event OnComponentBeginOverlap(Sphere)
  (params (OverlappedComponent :type Primitive%20Component%20Object%20Reference) (OtherActor :type Actor%20Object%20Reference) (OtherComp :type Primitive%20Component%20Object%20Reference) (OtherBodyIndex :type Integer) (bFromSweep :type Boolean) (SweepResult :type Hit%20Result%20Structure%20%28by%20ref%29))
  (bind _asbp_player_character_tutorial_1 (Utilities|Casting|CastToBP_Player_Character_Tutorial_1 OtherActor))
  (Variables|/Game/Blueprints/CharacterPlayer/BP_Player_Character_Tutorial_1.BP_Player_Character_Tutorial_1_C|SetLanterOrb _asbp_player_character_tutorial_1 self))

(event OnComponentEndOverlap(Sphere)
  (params (OverlappedComponent :type Primitive%20Component%20Object%20Reference) (OtherActor :type Actor%20Object%20Reference) (OtherComp :type Primitive%20Component%20Object%20Reference) (OtherBodyIndex :type Integer))
  (bind _asbp_player_character_tutorial_1 (Utilities|Casting|CastToBP_Player_Character_Tutorial_1 OtherActor))
  (Variables|/Game/Blueprints/CharacterPlayer/BP_Player_Character_Tutorial_1.BP_Player_Character_Tutorial_1_C|SetLanterOrb _asbp_player_character_tutorial_1 0))

(event Custom|TurnOn
  (bind _delta (Timeline|IntensityOrb PlayFromStart)
    (:Update
      (Rendering|Components|Light|SetIntensity (Variables|Default|GetTorchLight) _delta))))

(event EventBeginPlay)

(event Collision|EventActorBeginOverlap
  (params (OtherActor :type Actor%20Object%20Reference)))

(fn ConstructionScript)

(fn GetInteractText
  (params (InstigatorPawn :type Pawn%20Object%20Reference))
  (return ""))