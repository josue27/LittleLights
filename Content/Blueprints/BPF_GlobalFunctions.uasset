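; Blueprint function library of global helpers for finding key actors, switching input modes, toggling player control and changing levels.
; Lookups fetch the tutorial manager, exit door and player character by class, while input helpers toggle pawn input, input mode and cursor.
; ChangeLevel starts a fade widget and immediately opens the level.
; A manual view-projection helper maps world points to scaled screen positions, but always returns Valid as false.
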(fn GetLevelManager
  (bind _returnvalue (Actor|GetActorOfClass (LocalVariables|Get__WorldContext) "/Game/Blueprints/LevelManagers/BP_TutorialManager_Base.BP_TutorialManager_Base_C"))
  (Utilities|IsValid _returnvalue
    (:Is%20Valid
      (return true _returnvalue))
    (:Is%20Not%20Valid
      (return false 0))))

(fn GetExitDoor
  (bind _returnvalue (Actor|GetActorOfClass 0 "/Game/Blueprints/BP_FinalDoor.BP_FinalDoor_C"))
  (Utilities|IsValid _returnvalue
    (:Is%20Valid
      (return _returnvalue true))
    (:Is%20Not%20Valid
      (return 0 false))))

(fn ChangetoUIInput
  (bind ___worldcontext (LocalVariables|Get__WorldContext))
  (bind _returnvalue (Game|GetPlayerController ___worldcontext))
  (Input|DisableInput (Game|Player|GetPlayerPawn ___worldcontext) _returnvalue)
  (Input|SetInputModeUIOnly _returnvalue 0 "DoNotLock" false)
  (Variables|/Script/Engine.PlayerController|SetbShowMouseCursor _returnvalue true))

(fn ChangetoGameInput
  (bind ___worldcontext (LocalVariables|Get__WorldContext))
  (bind _returnvalue (Game|GetPlayerController ___worldcontext))
  (Input|EnableInput (Game|Player|GetPlayerPawn ___worldcontext) _returnvalue)
  (Input|SetInputModeGameOnly _returnvalue false)
  (Variables|/Script/Engine.PlayerController|SetbShowMouseCursor _returnvalue false))

(fn PlayerCanMove
  (params (canMove :type Boolean))
  (bind _returnvalue (Actor|GetActorOfClass 0 "/Script/LittleLights.PlayerCharacter"))
  (Variables|/Script/LittleLights.PlayerCharacter|SetbCanMove _returnvalue canMove))

(fn ChangeLevel
  (params (NewParam :type Boolean) (Level :type World%20Soft%20Object%20Reference))
  (bind _returnvalue (UserInterface|CreateWidget "/Game/UIX/MainMenu/WBP_LevelTransition.WBP_LevelTransition_C"))
  (UserInterface|Viewport|AddtoViewport _returnvalue 0)
  (Default|FadeinSequence _returnvalue 1.0)
  (Game|OpenLevel(byObjectReference) 0 Level))

(fn GetTutorialManager
  (bind _outactors (Actor|GetAllActorsOfClass (LocalVariables|Get__WorldContext) "/Game/Blueprints/LevelManagers/BP_TutorialManager_Base.BP_TutorialManager_Base_C"))
  (Utilities|IsValid (Utilities|Array|Get(acopy) _outactors)
    (:Is%20Valid
      (return (Utilities|Array|Get(acopy) _outactors)))
    (:Is%20Not%20Valid
      (return 0))))

(fn ProjectWorldLocationtoScreen
  (params (ViewLocation :type Vector) (ViewRotation :type Rotator) (ViewFOV :type Float%20%28double-precision%29) (WorldLocation :type Vector))
  (bind (_x _y _z) (Math|Vector|BreakVector WorldLocation))
  (LocalVariables|SetThisViewportSize (Viewport|GetViewportSize))
  (bind _output_get (LocalVariables|SetThisProjectedView4 (Class|KismetMathLibrary|MatrixTransformVector4 (.ViewProjectionMatrix (Class|GameplayStatics|GetViewProjectionMatrix (Utilities|Struct|MakeMinimalViewInfo ViewLocation ViewRotation ViewFOV 512.0 true 0.0 false false 0.0 2097152.0 -1.0 (/ (.X (Math|Vector2D|BreakVector2D (LocalVariables|GetThisViewportSize))) (.Y (Math|Vector2D|BreakVector2D (LocalVariables|GetThisViewportSize)))) false true "Perspective" 0.0 "(bOverride_TemperatureType=False,bOverride_WhiteTemp=False,bOverride_WhiteTint=False,bOverride_ColorSaturation=False,bOverride_ColorContrast=False,bOverride_ColorGamma=False,bOverride_ColorGain=False,bOverride_ColorOffset=False,bOverride_ColorSaturationShadows=False,bOverride_ColorContrastShadows=False,bOverride_ColorGammaShadows=False,bOverride_ColorGainShadows=False,bOverride_ColorOffsetShadows=False,bOverride_ColorSaturationMidtones=False,bOverride_ColorContrastMidtones=False,bOverride_ColorGammaMidtones=False,bOverride_ColorGainMidtones=False,bOverride_ColorOffsetMidtones=False,bOverride_ColorSaturationHighlights=False,bOverride_ColorContrastHighlights=False,bOverride_ColorGammaHighlights=False,bOverride_ColorGainHighlights=False,bOverride_ColorOffsetHighlights=False,bOverride_ColorCorrectionShadowsMax=False,bOverride_ColorCorrectionHighlightsMin=False,bOverride_ColorCorrectionHighlightsMax=False,bOverride_BlueCorrection=False,bOverride_ExpandGamut=False,bOverride_ToneCurveAmount=False,bOverride_FilmSlope=False,bOverride_FilmToe=False,bOverride_FilmShoulder=False,bOverride_FilmBlackClip=False,bOverride_FilmWhiteClip=False,bOverride_SceneColorTint=False,bOverride_SceneFringeIntensity=False,bOverride_ChromaticAberrationStartOffset=False,bOverride_AmbientCubemapTint=False,bOverride_AmbientCubemapIntensity=False,bOverride_BloomMethod=False,bOverride_BloomIntensity=False,bOverride_BloomThreshold=False,bOverride_Bloom1Tint=False,bOverride_Bloom1Size=False,bOverride_Bloom2Size=False,bOverride_Bloom2Tint=False,bOverride_Bloom3Tint=False,bOverride_Bloom3Size=False,bOverride_Bloom4Tint=False,bOverride_Bloom4Size=False,bOverride_Bloom5Tint=False,bOverride_Bloom5Size=False,bOverride_Bloom6Tint=False,bOverride_Bloom6Size=False,bOverride_BloomSizeScale=False,bOverride_BloomConvolutionTexture=False,bOverride_BloomConvolutionScatterDispersion=False,bOverride_BloomConvolutionSize=False,bOverride_BloomConvolutionCenterUV=False,bOverride_BloomConvolutionPreFilterMin=False,bOverride_BloomConvolutionPreFilterMax=False,bOverride_BloomConvolutionPreFilterMult=False,bOverride_BloomConvolutionBufferScale=False,bOverride_BloomDirtMaskIntensity=False,bOverride_BloomDirtMaskTint=False,bOverride_BloomDirtMask=False,bOverride_CameraShutterSpeed=False,bOverride_CameraISO=False,bOverride_AutoExposureMethod=False,bOverride_AutoExposureLowPercent=False,bOverride_AutoExposureHighPercent=False,bOverride_AutoExposureMinBrightness=False,bOverride_AutoExposureMaxBrightness=False,bOverride_AutoExposureSpeedUp=False,bOverride_AutoExposureSpeedDown=False,bOverride_AutoExposureBias=False,bOverride_AutoExposureBiasCurve=False,bOverride_AutoExposureMeterMask=False,bOverride_AutoExposureApplyPhysicalCameraExposure=False,bOverride_HistogramLogMin=False,bOverride_HistogramLogMax=False,bOverride_LocalExposureHighlightContrastScale=False,bOverride_LocalExposureShadowContrastScale=False,bOverride_LocalExposureHighlightContrastCurve=False,bOverride_LocalExposureShadowContrastCurve=False,bOverride_LocalExposureHighlightThreshold=False,bOverride_LocalExposureShadowThreshold=False,bOverride_LocalExposureDetailStrength=False,bOverride_LocalExposureBlurredLuminanceBlend=False,bOverride_LocalExposureBlurredLuminanceKernelSizePercent=False,bOverride_LocalExposureMiddleGreyBias=False,bOverride_LensFlareIntensity=False,bOverride_LensFlareTint=False,bOverride_LensFlareTints=False,bOverride_LensFlareBokehSize=False,bOverride_LensFlareBokehShape=False,bOverride_LensFlareThreshold=False,bOverride_VignetteIntensity=False,bOverride_Sharpen=False,bOverride_FilmGrainIntensity=False,bOverride_FilmGrainIntensityShadows=False,bOverride_FilmGrainIntensityMidtones=False,bOverride_FilmGrainIntensityHighlights=False,bOverride_FilmGrainShadowsMax=False,bOverride_FilmGrainHighlightsMin=False,bOverride_FilmGrainHighlightsMax=False,bOverride_FilmGrainTexelSize=False,bOverride_FilmGrainTexture=False,bOverride_AmbientOcclusionIntensity=False,bOverride_AmbientOcclusionStaticFraction=False,bOverride_AmbientOcclusionRadius=False,bOverride_AmbientOcclusionFadeDistance=False,bOverride_AmbientOcclusionFadeRadius=False,bOverride_AmbientOcclusionRadiusInWS=False,bOverride_AmbientOcclusionPower=False,bOverride_AmbientOcclusionBias=False,bOverride_AmbientOcclusionQuality=False,bOverride_AmbientOcclusionMipBlend=False,bOverride_AmbientOcclusionMipScale=False,bOverride_AmbientOcclusionMipThreshold=False,bOverride_AmbientOcclusionTemporalBlendWeight=False,bOverride_RayTracingAO=False,bOverride_RayTracingAOSamplesPerPixel=False,bOverride_RayTracingAOIntensity=False,bOverride_RayTracingAORadius=False,bOverride_IndirectLightingColor=False,bOverride_IndirectLightingIntensity=False,bOverride_ColorGradingIntensity=False,bOverride_ColorGradingLUT=False,bOverride_DepthOfFieldFocalDistance=False,bOverride_DepthOfFieldFstop=False,bOverride_DepthOfFieldMinFstop=False,bOverride_DepthOfFieldBladeCount=False,bOverride_DepthOfFieldSensorWidth=False,bOverride_DepthOfFieldSqueezeFactor=False,bOverride_DepthOfFieldDepthBlurRadius=False,bOverride_DepthOfFieldUseHairDepth=False,bOverride_DepthOfFieldDepthBlurAmount=False,bOverride_DepthOfFieldFocalRegion=False,bOverride_DepthOfFieldNearTransitionRegion=False,bOverride_DepthOfFieldFarTransitionRegion=False,bOverride_DepthOfFieldScale=False,bOverride_DepthOfFieldNearBlurSize=False,bOverride_DepthOfFieldFarBlurSize=False,bOverride_MobileHQGaussian=False,bOverride_DepthOfFieldOcclusion=False,bOverride_DepthOfFieldSkyFocusDistance=False,bOverride_DepthOfFieldVignetteSize=False,bOverride_MotionBlurAmount=False,bOverride_MotionBlurMax=False,bOverride_MotionBlurTargetFPS=False,bOverride_MotionBlurPerObjectSize=False,bOverride_ReflectionMethod=False,bOverride_LumenReflectionQuality=False,bOverride_ScreenSpaceReflectionIntensity=False,bOverride_ScreenSpaceReflectionQuality=False,bOverride_ScreenSpaceReflectionMaxRoughness=False,bOverride_ScreenSpaceReflectionRoughnessScale=False,bOverride_RayTracingReflectionsMaxRoughness=False,bOverride_RayTracingReflectionsMaxBounces=False,bOverride_RayTracingReflectionsSamplesPerPixel=False,bOverride_RayTracingReflectionsShadows=False,bOverride_RayTracingReflectionsTranslucency=False,bOverride_TranslucencyType=False,bOverride_RayTracingTranslucencyMaxRoughness=False,bOverride_RayTracingTranslucencyRefractionRays=False,bOverride_RayTracingTranslucencySamplesPerPixel=False,bOverride_RayTracingTranslucencyShadows=False,bOverride_RayTracingTranslucencyRefraction=False,bOverride_DynamicGlobalIlluminationMethod=False,bOverride_LumenSceneLightingQuality=False,bOverride_LumenSceneDetail=False,bOverride_LumenSceneViewDistance=False,bOverride_LumenSceneLightingUpdateSpeed=False,bOverride_LumenFinalGatherQuality=False,bOverride_LumenFinalGatherLightingUpdateSpeed=False,bOverride_LumenFinalGatherScreenTraces=False,bOverride_LumenMaxTraceDistance=False,bOverride_LumenDiffuseColorBoost=False,bOverride_LumenSkylightLeaking=False,bOverride_LumenFullSkylightLeakingDistance=False,bOverride_LumenRayLightingMode=False,bOverride_LumenReflectionsScreenTraces=False,bOverride_LumenFrontLayerTranslucencyReflections=False,bOverride_LumenMaxRoughnessToTraceReflections=False,bOverride_LumenMaxReflectionBounces=False,bOverride_LumenMaxRefractionBounces=False,bOverride_LumenSurfaceCacheResolution=False,bOverride_RayTracingGI=False,bOverride_RayTracingGIMaxBounces=False,bOverride_RayTracingGISamplesPerPixel=False,bOverride_PathTracingMaxBounces=False,bOverride_PathTracingSamplesPerPixel=False,bOverride_PathTracingMaxPathExposure=False,bOverride_PathTracingEnableEmissiveMaterials=False,bOverride_PathTracingEnableReferenceDOF=False,bOverride_PathTracingEnableReferenceAtmosphere=False,bOverride_PathTracingEnableDenoiser=False,bOverride_PathTracingIncludeEmissive=False,bOverride_PathTracingIncludeDiffuse=False,bOverride_PathTracingIncludeIndirectDiffuse=False,bOverride_PathTracingIncludeSpecular=False,bOverride_PathTracingIncludeIndirectSpecular=False,bOverride_PathTracingIncludeVolume=False,bOverride_PathTracingIncludeIndirectVolume=False,bMobileHQGaussian=False,BloomMethod=BM_SOG,AutoExposureMethod=AEM_Histogram,TemperatureType=TEMP_WhiteBalance,WhiteTemp=6500.000000,WhiteTint=0.000000,ColorSaturation=(X=1.000000,Y=1.000000,Z=1.000000,W=1.000000),ColorContrast=(X=1.000000,Y=1.000000,Z=1.000000,W=1.000000),ColorGamma=(X=1.000000,Y=1.000000,Z=1.000000,W=1.000000),ColorGain=(X=1.000000,Y=1.000000,Z=1.000000,W=1.000000),ColorOffset=(X=0.000000,Y=0.000000,Z=0.000000,W=0.000000),ColorSaturationShadows=(X=1.000000,Y=1.000000,Z=1.000000,W=1.000000),ColorContrastShadows=(X=1.000000,Y=1.000000,Z=1.000000,W=1.000000),ColorGammaShadows=(X=1.000000,Y=1.000000,Z=1.000000,W=1.000000),ColorGainShadows=(X=1.000000,Y=1.000000,Z=1.000000,W=1.000000),ColorOffsetShadows=(X=0.000000,Y=0.000000,Z=0.000000,W=0.000000),ColorSaturationMidtones=(X=1.000000,Y=1.000000,Z=1.000000,W=1.000000),ColorContrastMidtones=(X=1.000000,Y=1.000000,Z=1.000000,W=1.000000),ColorGammaMidtones=(X=1.000000,Y=1.000000,Z=1.000000,W=1.000000),ColorGainMidtones=(X=1.000000,Y=1.000000,Z=1.000000,W=1.000000),ColorOffsetMidtones=(X=0.000000,Y=0.000000,Z=0.000000,W=0.000000),ColorSaturationHighlights=(X=1.000000,Y=1.000000,Z=1.000000,W=1.000000),ColorContrastHighlights=(X=1.000000,Y=1.000000,Z=1.000000,W=1.000000),ColorGammaHighlights=(X=1.000000,Y=1.000000,Z=1.000000,W=1.000000),ColorGainHighlights=(X=1.000000,Y=1.000000,Z=1.000000,W=1.000000),ColorOffsetHighlights=(X=0.000000,Y=0.000000,Z=0.000000,W=0.000000),ColorCorrectionHighlightsMin=0.500000,ColorCorrectionHighlightsMax=1.000000,ColorCorrectionShadowsMax=0.090000,BlueCorrection=0.600000,ExpandGamut=1.000000,ToneCurveAmount=1.000000,FilmSlope=0.880000,FilmToe=0.550000,FilmShoulder=0.260000,FilmBlackClip=0.000000,FilmWhiteClip=0.040000,SceneColorTint=(R=1.000000,G=1.000000,B=1.000000,A=1.000000),SceneFringeIntensity=0.000000,ChromaticAberrationStartOffset=0.000000,BloomIntensity=0.675000,BloomThreshold=-1.000000,BloomSizeScale=4.000000,Bloom1Size=0.300000,Bloom2Size=1.000000,Bloom3Size=2.000000,Bloom4Size=10.000000,Bloom5Size=30.000000,Bloom6Size=64.000000,Bloom1Tint=(R=0.346500,G=0.346500,B=0.346500,A=1.000000),Bloom2Tint=(R=0.138000,G=0.138000,B=0.138000,A=1.000000),Bloom3Tint=(R=0.117600,G=0.117600,B=0.117600,A=1.000000),Bloom4Tint=(R=0.066000,G=0.066000,B=0.066000,A=1.000000),Bloom5Tint=(R=0.066000,G=0.066000,B=0.066000,A=1.000000),Bloom6Tint=(R=0.061000,G=0.061000,B=0.061000,A=1.000000),BloomConvolutionScatterDispersion=1.000000,BloomConvolutionSize=1.000000,BloomConvolutionTexture=None,BloomConvolutionCenterUV=(X=0.500000,Y=0.500000),BloomConvolutionPreFilterMin=7.000000,BloomConvolutionPreFilterMax=15000.000000,BloomConvolutionPreFilterMult=15.000000,BloomConvolutionBufferScale=0.133000,BloomDirtMask=None,BloomDirtMaskIntensity=0.000000,BloomDirtMaskTint=(R=0.500000,G=0.500000,B=0.500000,A=1.000000),DynamicGlobalIlluminationMethod=Lumen,IndirectLightingColor=(R=1.000000,G=1.000000,B=1.000000,A=1.000000),IndirectLightingIntensity=1.000000,LumenSceneLightingQuality=1.000000,LumenSceneDetail=1.000000,LumenSceneViewDistance=20000.000000,LumenSceneLightingUpdateSpeed=1.000000,LumenFinalGatherQuality=1.000000,LumenFinalGatherLightingUpdateSpeed=1.000000,LumenFinalGatherScreenTraces=True,LumenMaxTraceDistance=20000.000000,LumenDiffuseColorBoost=1.000000,LumenSkylightLeaking=0.000000,LumenFullSkylightLeakingDistance=1000.000000,LumenSurfaceCacheResolution=1.000000,ReflectionMethod=Lumen,LumenReflectionQuality=1.000000,LumenRayLightingMode=Default,LumenReflectionsScreenTraces=True,LumenFrontLayerTranslucencyReflections=False,LumenMaxRoughnessToTraceReflections=0.400000,LumenMaxReflectionBounces=1,LumenMaxRefractionBounces=0,ScreenSpaceReflectionIntensity=100.000000,ScreenSpaceReflectionQuality=50.000000,ScreenSpaceReflectionMaxRoughness=0.600000,AmbientCubemapTint=(R=1.000000,G=1.000000,B=1.000000,A=1.000000),AmbientCubemapIntensity=1.000000,AmbientCubemap=None,CameraShutterSpeed=60.000000,CameraISO=100.000000,DepthOfFieldFstop=4.000000,DepthOfFieldMinFstop=1.200000,DepthOfFieldBladeCount=5,AutoExposureBias=1.000000,AutoExposureBiasBackup=0.000000,bOverride_AutoExposureBiasBackup=False,AutoExposureApplyPhysicalCameraExposure=True,AutoExposureBiasCurve=None,AutoExposureMeterMask=None,AutoExposureLowPercent=10.000000,AutoExposureHighPercent=90.000000,AutoExposureMinBrightness=0.030000,AutoExposureMaxBrightness=8.000000,AutoExposureSpeedUp=3.000000,AutoExposureSpeedDown=1.000000,HistogramLogMin=-8.000000,HistogramLogMax=4.000000,LocalExposureHighlightContrastScale=1.000000,LocalExposureShadowContrastScale=1.000000,LocalExposureHighlightContrastCurve=None,LocalExposureShadowContrastCurve=None,LocalExposureHighlightThreshold=0.000000,LocalExposureShadowThreshold=0.000000,LocalExposureDetailStrength=1.000000,LocalExposureBlurredLuminanceBlend=0.600000,LocalExposureBlurredLuminanceKernelSizePercent=50.000000,LocalExposureMiddleGreyBias=0.000000,LensFlareIntensity=1.000000,LensFlareTint=(R=1.000000,G=1.000000,B=1.000000,A=1.000000),LensFlareBokehSize=3.000000,LensFlareThreshold=8.000000,LensFlareBokehShape=None,LensFlareTints[0]=(R=1.000000,G=0.800000,B=0.400000,A=0.600000),LensFlareTints[1]=(R=1.000000,G=1.000000,B=0.600000,A=0.530000),LensFlareTints[2]=(R=0.800000,G=0.800000,B=1.000000,A=0.460000),LensFlareTints[3]=(R=0.500000,G=1.000000,B=0.400000,A=0.390000),LensFlareTints[4]=(R=0.500000,G=0.800000,B=1.000000,A=0.310000),LensFlareTints[5]=(R=0.900000,G=1.000000,B=0.800000,A=0.270000),LensFlareTints[6]=(R=1.000000,G=0.800000,B=0.400000,A=0.220000),LensFlareTints[7]=(R=0.900000,G=0.700000,B=0.700000,A=0.150000),VignetteIntensity=0.400000,Sharpen=0.000000,FilmGrainIntensity=0.000000,FilmGrainIntensityShadows=1.000000,FilmGrainIntensityMidtones=1.000000,FilmGrainIntensityHighlights=1.000000,FilmGrainShadowsMax=0.090000,FilmGrainHighlightsMin=0.500000,FilmGrainHighlightsMax=1.000000,FilmGrainTexelSize=1.000000,FilmGrainTexture=None,AmbientOcclusionIntensity=0.500000,AmbientOcclusionStaticFraction=1.000000,AmbientOcclusionRadius=200.000000,AmbientOcclusionRadiusInWS=False,AmbientOcclusionFadeDistance=8000.000000,AmbientOcclusionFadeRadius=5000.000000,AmbientOcclusionPower=2.000000,AmbientOcclusionBias=3.000000,AmbientOcclusionQuality=50.000000,AmbientOcclusionMipBlend=0.600000,AmbientOcclusionMipScale=1.700000,AmbientOcclusionMipThreshold=0.010000,AmbientOcclusionTemporalBlendWeight=0.100000,RayTracingAO=False,RayTracingAOSamplesPerPixel=1,RayTracingAOIntensity=1.000000,RayTracingAORadius=200.000000,ColorGradingIntensity=1.000000,ColorGradingLUT=None,DepthOfFieldSensorWidth=24.576000,DepthOfFieldSqueezeFactor=1.000000,DepthOfFieldFocalDistance=0.000000,DepthOfFieldDepthBlurAmount=1.000000,DepthOfFieldDepthBlurRadius=0.000000,DepthOfFieldUseHairDepth=False,DepthOfFieldFocalRegion=0.000000,DepthOfFieldNearTransitionRegion=300.000000,DepthOfFieldFarTransitionRegion=500.000000,DepthOfFieldScale=0.000000,DepthOfFieldNearBlurSize=15.000000,DepthOfFieldFarBlurSize=15.000000,DepthOfFieldOcclusion=0.400000,DepthOfFieldSkyFocusDistance=0.000000,DepthOfFieldVignetteSize=200.000000,MotionBlurAmount=0.500000,MotionBlurMax=5.000000,MotionBlurTargetFPS=30,MotionBlurPerObjectSize=0.000000,TranslucencyType=Raster,RayTracingTranslucencyMaxRoughness=0.600000,RayTracingTranslucencyRefractionRays=3,RayTracingTranslucencySamplesPerPixel=1,RayTracingTranslucencyShadows=Hard_shadows,RayTracingTranslucencyRefraction=True,PathTracingMaxBounces=32,PathTracingSamplesPerPixel=16384,PathTracingMaxPathExposure=30.000000,PathTracingEnableEmissiveMaterials=True,PathTracingEnableReferenceDOF=False,PathTracingEnableReferenceAtmosphere=False,PathTracingEnableDenoiser=True,PathTracingIncludeEmissive=True,PathTracingIncludeDiffuse=True,PathTracingIncludeIndirectDiffuse=True,PathTracingIncludeSpecular=True,PathTracingIncludeIndirectSpecular=True,PathTracingIncludeVolume=True,PathTracingIncludeIndirectVolume=True,WeightedBlendables=(Array=))" "(X=0.000000,Y=0.000000)"))) (Math|Vector4|MakeVector4 _x _y _z 1.0))))
  (if (> (.W (Math|Vector4|BreakVector4 _output_get)) 0.0)
    (return (Math|Vector2D|MakeVector2D (* (+ (/ (/ (.X (Math|Vector4|BreakVector4 _output_get)) (.W (Math|Vector4|BreakVector4 _output_get))) 2.0) 0.5) (.X (Math|Vector|BreakVector (/ (LocalVariables|GetThisViewportSize) (Class|WidgetLayoutLibrary|GetViewportScale))))) (* (- (- 1.0 (/ (/ (.Y (Math|Vector4|BreakVector4 _output_get)) (.Z (Math|Vector4|BreakVector4 _output_get))) 2.0)) 0.5) (.Y (Math|Vector|BreakVector (/ (LocalVariables|GetThisViewportSize) (Class|WidgetLayoutLibrary|GetViewportScale)))))) false)
    (else
      (return "" false))))

(fn DisableInteractionComponent
  (params (disable :type Boolean))
  (bind _returnvalue (Actor|GetActorOfClass (LocalVariables|Get__WorldContext) "/Script/LittleLights.PlayerCharacter"))
  (Class|PlayerCharacter|DisableInteraction _returnvalue disable))