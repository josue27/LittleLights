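; Golem base actor for Tutorial B that tracks travel along a list of externally supplied waypoints.
; A player entering its sphere calls MoveNextPoint; while moving, Tick checks distance to the current waypoint and clears the moving flag on arrival, with debug prints.
; StepReceived spawns a water track decal at the left foot socket.
; The timeout branch does nothing, and the destroy-at-end logic is unconnected.
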(event OnComponentBeginOverlap(Sphere)
  (params (OverlappedComponent :type Primitive%20Component%20Object%20Reference) (OtherActor :type Actor%20Object%20Reference) (OtherComp :type Primitive%20Component%20Object%20Reference) (OtherBodyIndex :type Integer) (bFromSweep :type Boolean) (SweepResult :type Hit%20Result%20Structure%20%28by%20ref%29))
  (Utilities|Casting|CastToBP_PlayerCharacter_Tut_B_02 OtherActor)
  (Class|LLGolem|MoveNextPoint))

(event Custom|HasArrivedToPoint
  (params (delta :type Float%20%28single-precision%29))
  (bind _returnvalue (Transformation|GetActorLocation))
  (bind _waypoints (Variables|Default|GetWaypoints))
  (bind _currentpoint (Variables|Default|GetCurrentPoint))
  (bind _output (Utilities|Array|Get(acopy) _waypoints _currentpoint))
  (bind _returnvalue_2 (Transformation|GetActorLocation _output))
  (bind _returnvalue_3 (Math|Vector|Distance(Vector) _returnvalue _returnvalue_2))
  (Development|PrintString (Utilities|String|ToString(Float) _returnvalue_3) true true "(R=0.000000,G=0.660000,B=1.000000,A=1.000000)" 0.1)
  (if (<= _returnvalue_3 1e+02)
    (Variables|Default|SetbMovingToPoint false)
    (Development|PrintString "Golem stop moving" true true "(R=1.000000,G=0.000000,B=0.004872,A=1.000000)" 3.0)
    (else
      (bind _output_get (Variables|Default|SetTimePased (+ delta (Variables|Default|GetTimePased))))
      (if (>= _output_get 2.0)
        _))))

(event Custom|AddWayPoints
  (params (WayPointsForGolem :type Array%20of%20Actor%20Object%20References))
  (Variables|Default|SetWaypoints WayPointsForGolem))

(event Custom|StepReceived
  (Game|SpawnActorfromClass "/Game/Blueprints/Tutorial_B_01/BP_WaterTrackDecal.BP_WaterTrackDecal_C" (Math|Transform|MakeTransform (Transformation|GetSocketLocation (Variables|Character|GetMesh) "LeftFootSocket") "90.000000, 0, 0" "1,1,1") "Undefined" 0 0))

(event EventBeginPlay
  (|CallParentFunction))

(event Collision|EventActorBeginOverlap
  (params (OtherActor :type Actor%20Object%20Reference))
  (|CallParentFunction OtherActor) ; This node is disabled and will not be called.\nDrag off pins to build functionality.
)

(event EventTick
  (params (DeltaSeconds :type Float%20%28single-precision%29))
  (|CallParentFunction DeltaSeconds)
  (if (Variables|Default|GetbMovingToPoint)
    (CallFunction|HasArrivedtoPoint DeltaSeconds)))

(fn ConstructionScript
  (|CallParentFunction))