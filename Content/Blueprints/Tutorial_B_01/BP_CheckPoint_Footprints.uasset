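; BP_CheckPoint_Footprints is a tutorial checkpoint trigger that reveals footprint track decals when the player reaches it.
; On BeginPlay it hides the Decal component of every entry in its TracksDB array.
; When a BP_PlayerCharacter_Tut_B_02 begins overlapping its Box, it prints a debug message and makes all those decals visible.
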(event OnComponentBeginOverlap(Box)
  (params (OverlappedComponent :type Primitive%20Component%20Object%20Reference) (OtherActor :type Actor%20Object%20Reference) (OtherComp :type Primitive%20Component%20Object%20Reference) (OtherBodyIndex :type Integer) (bFromSweep :type Boolean) (SweepResult :type Hit%20Result%20Structure%20%28by%20ref%29))
  (Utilities|Casting|CastToBP_PlayerCharacter_Tut_B_02 OtherActor)
  (Development|PrintString "Checkpoint footprints")
  (for _array_element (Variables|Default|GetTracksDB)
    (Rendering|SetVisibility (Variables|/Game/Blueprints/Tutorial_B_01/BP_WaterTrackDecal.BP_WaterTrackDecal_C|GetDecal _array_element) true false)))

(event EventBeginPlay
  (for _array_element (Variables|Default|GetTracksDB)
    (Rendering|SetVisibility (Variables|/Game/Blueprints/Tutorial_B_01/BP_WaterTrackDecal.BP_WaterTrackDecal_C|GetDecal _array_element) false false)))

(event Collision|EventActorBeginOverlap
  (params (OtherActor :type Actor%20Object%20Reference)))

(event EventTick
  (params (DeltaSeconds :type Float%20%28single-precision%29)))

(fn ConstructionScript)