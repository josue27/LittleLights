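; Water track decal actor that animates a scalar material parameter, apparently emissive intensity, on a dynamic instance created in the construction script.
; ActivateTrack plays a turn-on timeline, though its updates write a constant zero.
; StartDecay runs once, scaling the captured parameter value by the Delta timeline.
; Decay starts when ActorToRespond overlaps the sphere, or after WaitForPlayer's delay of Offset plus TimeTurnOff.
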(event OnComponentBeginOverlap(Sphere)
  (params (OverlappedComponent :type Primitive%20Component%20Object%20Reference) (OtherActor :type Actor%20Object%20Reference) (OtherComp :type Primitive%20Component%20Object%20Reference) (OtherBodyIndex :type Integer) (bFromSweep :type Boolean) (SweepResult :type Hit%20Result%20Structure%20%28by%20ref%29))
  (if (== OtherActor (Variables|Default|GetActorToRespond))
    (CallFunction|StartDecay)))

(event Custom|StartDecay
  (bind _decalmat (Variables|Default|GetDecalMat))
  (if (not (Variables|Default|GetActivated))
    (Variables|Default|SetActivated true)
    (bind _returnvalue (Rendering|Material|GetScalarParameterValue _decalmat (Variables|Default|GetParameter%20Name) :!class /Script/Engine.MaterialInstanceDynamic))
    (Variables|Default|SetFinalEmissiveIntensity _returnvalue)
    (bind _delta (Timeline|Delta PlayFromStart)
      (:Update
        (Rendering|Material|SetScalarParameterValue _decalmat (Variables|Default|GetParameter%20Name) (* _delta (Variables|Default|GetFinalEmissiveIntensity)) :!class /Script/Engine.MaterialInstanceDynamic)))))

(event Custom|WaitForPlayer
  (params (Offset :type Float%20%28single-precision%29))
  ;[1 1 1] Called when activated to automatically Start the Decay even if player has not passed in X amount of time
  (Utilities|FlowControl|Delay (+ Offset (Variables|Default|GetTime_TurnOff)))
  (CallFunction|StartDecay))

(event Custom|ActivateTrack
  (if (not (Variables|Default|GetActivated))
    (Rendering|Material|GetScalarParameterValue (Variables|Default|GetDecalMat) (Variables|Default|GetParameter%20Name) :!class /Script/Engine.MaterialInstanceDynamic)
    (Variables|Default|SetFinalEmissiveIntensity 0.0)
    (Timeline|DeltaTurnON PlayFromStart
      (:Update
        (Rendering|Material|SetScalarParameterValue (Variables|Default|GetDecalMat) (Variables|Default|GetParameter%20Name) 0.0 :!class /Script/Engine.MaterialInstanceDynamic)))))

(event EventBeginPlay)

(event Collision|EventActorBeginOverlap
  (params (OtherActor :type Actor%20Object%20Reference)))

(event EventTick
  (params (DeltaSeconds :type Float%20%28single-precision%29)))

(fn ConstructionScript
  (bind _decal (Variables|Default|GetDecal))
  (bind _returnvalue (Rendering|Material|CreateDynamicMaterialInstance (Variables|/Script/Engine.DecalComponent|GetDecalMaterial _decal) "None" "None" :!class /Script/Engine.KismetMaterialLibrary))
  (bind _output_get (Variables|Default|SetDecalMat _returnvalue))
  (Rendering|Components|Decal|SetDecalMaterial _decal _output_get))