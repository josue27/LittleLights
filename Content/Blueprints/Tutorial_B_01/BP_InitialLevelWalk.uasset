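; BP_InitialLevelWalk is a tutorial actor meant to walk the player character into the level along a spline.
; On BeginPlay, WalkInPlayer finds and stores all BP_PlayerCharacter_Tut_B_02 actors, but does nothing further.
; The DeltaWalk timeline, which would move the first player along the spline in X and Y while keeping its Z, is never triggered, so no movement occurs.
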(event Custom|WalkInPlayer
  (bind _outactors (Actor|GetAllActorsOfClass "/Game/Blueprints/CharacterPlayer/BP_PlayerCharacter_Tut_B_02.BP_PlayerCharacter_Tut_B_02_C"))
  (Variables|Default|SetBP_Player _outactors))

(event EventBeginPlay
  (CallFunction|WalkinPlayer))

(event Collision|EventActorBeginOverlap
  (params (OtherActor :type Actor%20Object%20Reference)))

(event EventTick
  (params (DeltaSeconds :type Float%20%28single-precision%29)))

(fn ConstructionScript)