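; BP_Meta is a level goal whose point light brightens as the player approaches and which ends the level when reached.
; BeginPlay stores the light's intensity and switches it off; Sphere overlap caches the player and entry position.
; Tick then lerps intensity by current distance over entry distance.
; Box overlap by the player prints a message and calls FinNivel on BP_Tutorial01, found by class.
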(event OnComponentBeginOverlap(Box)
  (params (OverlappedComponent :type Primitive%20Component%20Object%20Reference) (OtherActor :type Actor%20Object%20Reference) (OtherComp :type Primitive%20Component%20Object%20Reference) (OtherBodyIndex :type Integer) (bFromSweep :type Boolean) (SweepResult :type Hit%20Result%20Structure%20%28by%20ref%29))
  (Utilities|Casting|CastToBP_PersonajeJugador OtherActor)
  (Development|PrintString "Jugador llego a meta")
  (bind _returnvalue (Actor|GetActorOfClass "/Game/Blueprints/LevelManagers/BP_Tutorial01.BP_Tutorial01_C"))
  (Default|FinNivel _returnvalue))

(event OnComponentBeginOverlap(Sphere)
  (params (OverlappedComponent :type Primitive%20Component%20Object%20Reference) (OtherActor :type Actor%20Object%20Reference) (OtherComp :type Primitive%20Component%20Object%20Reference) (OtherBodyIndex :type Integer) (bFromSweep :type Boolean) (SweepResult :type Hit%20Result%20Structure%20%28by%20ref%29))
  (bind _asbp_personaje_jugador (Utilities|Casting|CastToBP_PersonajeJugador OtherActor))
  ;[1 1 1] Obtener jugador y posicion inicial
  (bind _output_get (Variables|Default|SetJugador _asbp_personaje_jugador))
  (Variables|Default|SetPosicionInicialJugador (Transformation|GetActorLocation _output_get))
  (Variables|Default|SetSeguirPosicionJugador true))

(event EventBeginPlay
  (bind _pointlight (Variables|Default|GetPointLight))
  ;[1 1 1] Obtener Intencidad Inicial
  (Variables|Default|SetIntencidadFinal (Variables|/Script/Engine.LightComponentBase|GetIntensity _pointlight))
  (Rendering|Components|Light|SetIntensity _pointlight 0.0))

(event Collision|EventActorBeginOverlap
  (params (OtherActor :type Actor%20Object%20Reference)))

(event EventTick
  (params (DeltaSeconds :type Float%20%28single-precision%29))
  (bind _returnvalue (Transformation|GetActorLocation))
  (bind _jugador (Variables|Default|GetJugador))
  (if (Variables|Default|GetSeguirPosicionJugador)
    (Utilities|IsValid _jugador
      (:Is%20Valid
        (Rendering|Components|Light|SetIntensity (Variables|Default|GetPointLight) (Math|Float|Lerp (Variables|Default|GetIntencidadFinal) 0.0 (/ (Math|Vector|Distance(Vector) (Transformation|GetActorLocation _jugador) _returnvalue) (Math|Vector|Distance(Vector) (Variables|Default|GetPosicionInicialJugador) _returnvalue))))))))

(fn ConstructionScript)