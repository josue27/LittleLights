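; Player character Blueprint that handles the HUD, camera, fog of war, totem fragments and debug puzzle input.
; Tick writes player position to the fog parameter collection, offsets the spring arm forward, and scales fog radius and FOV by torch intensity.
; TorchOff has the level manager activate the beast and starts the HUD chase, which BeastChasing feeds with distance.
; A timeline clears fog on beacon completion, though its level-manager binding is disconnected.
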(event Custom|FolowMouse
  (if (Variables|Puzzle|GetbWithPuzzlePart)
    _))

(event Custom|DisappearFog
  ;[1 1 1] Desapear FOG
  (Variables|Default|SetbBeaconCompleted true)
  (bind _radiusdelta (Timeline|FogDissapeared PlayFromStart)
    (:Update
      (Rendering|Material|SetScalarParameterValue "/Game/Material/MC_Fog_Parametros.MC_Fog_Parametros" "RadiusExponential" _radiusdelta :!class /Script/Engine.KismetMaterialLibrary))))

(event Custom|BeaconActivated_Event
  ;[1 1 1] BeginPlay
  (CallFunction|DisappearFog))

(event Custom|Add%20HUD
  ;[1 1 1] Add  Gameplay HUD
  (bind _returnvalue (UserInterface|CreateWidget "/Game/UIX/PlayerHUDs/WBP_HUD.WBP_HUD_C" (Game|GetPlayerController 0)))
  (bind _output_get (Variables|Default|SetHUD_Jugador _returnvalue))
  (UserInterface|Viewport|AddtoViewport _output_get 0)
  (Variables|/Game/UIX/PlayerHUDs/WBP_HUD.WBP_HUD_C|SetStamine _output_get (Variables|Default|GetStamine))
  (Variables|/Script/LittleLights.Base_HUD_Widget|SetDeltaStamine _output_get 0.0))

(event Custom|UpdateFOV
  (bind _torch (Variables|Default|GetTorch))
  (Utilities|IsValid _torch
    (:Is%20Valid
      (Camera|SetFieldOfView (Variables|Default|GetCamera) (Math|Float|Lerp 7e+01 9e+01 (Variables|/Script/LittleLights.Torch|GetDeltaIntensity _torch))))))

(event Custom|BeastChasing
  (params (DistanceRatio :type Float%20%28single-precision%29))
  (bind _hud_jugador (Variables|Default|GetHUD_Jugador))
  (Variables|Default|SetDistanceRatio DistanceRatio)
  (Utilities|IsValid _hud_jugador
    (:Is%20Valid
      (Variables|/Game/UIX/PlayerHUDs/WBP_HUD.WBP_HUD_C|SetDeltaDistanceBeast _hud_jugador DistanceRatio))))

(event Custom|PossessView
  ;[1 1 1] Posses View
  (Game|Player|SetViewTargetwithBlend (Game|GetPlayerController 0) self 2.0 "VTBlend_Linear" 0.0 false))

(event EventBeginPlay
  ;[1 1 1] BeginPlay
  (bind (_bvalid _levelmanager) (CallFunction|GetLevelManager))
  (if _bvalid
    (Variables|Default|SetLevelManager _levelmanager))
  (CallFunction|AddHUD)
  (Variables|Default|SetSpringArmRef (Variables|Default|GetSpringArm)))

(event Collision|EventActorBeginOverlap
  (params (OtherActor :type Actor%20Object%20Reference)))

(event EventTick
  (params (DeltaSeconds :type Float%20%28single-precision%29))
  ;[1 1 1] FogWar Update posicion de jugador
  (Rendering|Material|SetVectorParameterValue "/Game/Material/MC_Fog_Parametros.MC_Fog_Parametros" "Pos" (Math|Conversions|ToLinearColor(Vector) (+ (Transformation|GetActorLocation) (Variables|Default|GetOffsetFogWar))) :!class /Script/Engine.KismetMaterialLibrary)
  ;[1 1 1] Makes the camera center offset alway X distance in front of the player (Try to implement in C++)
  (Variables|/Script/Engine.SpringArmComponent|SetTargetOffset (Variables|Default|GetSpringArm) (* (Transformation|GetActorForwardVector) 1.2e+02))
  (CallFunction|UpdateFogRadius)
  (CallFunction|UpdateFOV))

(event EventFinJuegoEvento
  ;[1 1 1] FinNivel o Juego
  (Development|PrintString "Mensaje a jugador:Fin Juego")
  (Variables|Default|SetVelocidadMovimiento 0.0))

(event EventEmpezarJuegoEvento
  ;[1 1 1] Game Started Signal
  (CallFunction|AddHUD)
  (Utilities|FlowControl|Delay 2.0))

(event EventTorchOff
  ;[1 1 1] Called from Torch when light is down
  ;;[0 1 0] TorchOff (c++ delcared)
  (bind _asbp_level_manager_base (Utilities|Casting|CastToBP_LevelManagerBase (Variables|Default|GetLevelManager)))
  (Default|ActivateBeast _asbp_level_manager_base)
  (Default|ChaseStarted (Variables|Default|GetHUD_Jugador)))

(event Input|ActionEvents|InputActionPuzzleDebug
  (params (Key :type Key%20Structure :default "None"))
  (:Pressed
    (Variables|Puzzle|SetbPuzzleSolving (not (Variables|Puzzle|GetbPuzzleSolving)))
    (CallFunction|ToggleInput (not (Variables|Default|GetbCanMove)))
    (Variables|Default|SetbCanMove (not (Variables|Default|GetbCanMove)))))

(event Input|KeyboardEvents|Escape
  (params (Key :type Key%20Structure :default "None"))
  ;[0.4334 1 0.4037] Input
  (:Pressed
    (Game|QuitGame 0 "Quit" false)))

(event Input|MouseEvents|LeftMouseButton
  (params (Key :type Key%20Structure :default "None"))
  (:Pressed
    (Development|PrintString (Utilities|GetDisplayName (.hitactor (.HitResult (Game|Player|GetHitResultUnderCursorbyChannel (Game|GetPlayerController 0) "TraceTypeQuery1" false)))))
    (Variables|Puzzle|SetbWithPuzzlePart true)))

(fn ConstructionScript
  (bind _springarm (Variables|Default|GetSpringArm))
  (bind _returnvalue (Transformation|GetWorldRotation _springarm))
  (Rendering|Material|SetVectorParameterValue "/Game/Material/MC_Fog_Parametros.MC_Fog_Parametros" "Pos" (Math|Conversions|ToLinearColor(Vector) (Transformation|GetActorLocation)) :!class /Script/Engine.KismetMaterialLibrary)
  (Transformation|SetRelativeRotation _springarm (Math|Rotator|MakeRotator (.roll _returnvalue) (.pitch _returnvalue) (- (.yaw (Transformation|GetActorRotation)) (Variables|Default|GetSpringArmZAngle))) false false)
  (Variables|/Script/Engine.SpringArmComponent|SetTargetOffset _springarm (* (Math|Vector|GetForwardVector (Transformation|GetActorRotation)) "120.000000, 0, 0")))

(fn ToggleInput
  (params (EnableGameInput :type Boolean))
  (bind _returnvalue (Game|GetPlayerController 0))
  (if EnableGameInput
    (Input|SetInputModeGameOnly _returnvalue)
    (Variables|/Script/Engine.PlayerController|SetbShowMouseCursor _returnvalue false)
    (else
      (Variables|/Script/Engine.PlayerController|SetbShowMouseCursor _returnvalue true))))

(fn UpdateFogRadius
  (bind _torch (Variables|Default|GetTorch))
  (if (not (Variables|Default|GetbBeaconCompleted))
    (Utilities|IsValid _torch
      (:Is%20Valid
        (Rendering|Material|SetScalarParameterValue "/Game/Material/MC_Fog_Parametros.MC_Fog_Parametros" "RadiusExponential" (Math|Float|Lerp (Variables|Default|GetMinFogVisibility) (Variables|Default|GetMaxFogVisibility) (Variables|/Script/LittleLights.Torch|GetDeltaIntensity _torch)) :!class /Script/Engine.KismetMaterialLibrary)))))

(fn AddTottemPiece
  (params (TotemPiece :type BP%20Tottem%20Fragment%20Object%20Reference))
  (Utilities|Array|AddUnique (Variables|Default|GetTottemFragments) TotemPiece))

(fn RestToottemPiece
  (params (Amount :type Integer))
  (Variables|Default|SetFragmentsAmount (- (Variables|Default|GetFragmentsAmount) Amount)))