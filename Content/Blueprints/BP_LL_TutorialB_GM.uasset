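; Game mode for the TutorialB level, running the intro transition, post-movement orb handoff, ambient sound and per-tick fog-of-war render target clearing.
; SpawnBeast, called on totem discovery, waits, then spawns the beast above the first spawn point and shows its presence image; the EQS query path is disconnected.
; Beacon completion removes the beast and briefly shows a completion widget.
; Async save/load events only create or load a save object and log.
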(event Custom|QueryLocactionFinished
  (params (QueryInstance :type Env%20Query%20Instance%20Blueprint%20Wrapper%20Object%20Reference) (QueryStatus :type EEnvQueryStatus%20Enum :default "Processing"))
  ;[0.9427 1 0 1 58] SpawnBeast TODO: Fix the C++ implementation
  (if (Utilities|Enum|Equal(Enum) QueryStatus "Success")
    (bind _resultlocations (AI|EQS|GetQueryResultsasLocations QueryInstance))
    (else
      (Development|PrintString "Problem Runnignquery" true true "(R=1.000000,G=0.486477,B=0.000000,A=1.000000)"))))

(event Custom|OnAutomaticMovementEnded_Event_0
  (params (PlayerCharacter :type Player%20Character%20Object%20Reference) (bLightUpTorch :type Boolean) (bStartDecay :type Boolean))
  (Class|LLGameModeBase|PlayerEndedIntroMovement bLightUpTorch bStartDecay))

(event Custom|SaveGame
  ;[0.1 0.15 0.2] Save/Load Game
  (bind _returnvalue (SaveGame|CreateSaveGameObject "/Game/Blueprints/SaveSystem/BP_SaveGameObject.BP_SaveGameObject_C"))
  (bind _output_get (Variables|Default|SetSaveGameInstance _returnvalue))
  (|AsyncSaveGametoSlot _output_get (Variables|/Game/Blueprints/SaveSystem/BP_SaveGameObject.BP_SaveGameObject_C|GetSaveSlotName _output_get) (Variables|/Game/Blueprints/SaveSystem/BP_SaveGameObject.BP_SaveGameObject_C|GetUserIndex _output_get)
    (:Completed
      (Development|PrintString "Save Game Completed"))))

(event Custom|LoadGame
  ;[0.1 0.15 0.2] Save/Load Game
  (bind _savegame (|AsyncLoadGamefromSlot "LLDebugSaveSlot")
    (:Completed
      (Utilities|Casting|CastToBP_SaveGameObject _savegame)
      (Development|PrintString "Save Game Loaded"))))

(event EventBeginPlay
  ;[1 1 1] CARE, begin play starts before StartPlay
  (Audio|PlaySound2D "/Game/Audio/OST/MysteriousForest_Cue.MysteriousForest_Cue" 0.3 1.0 0.0 0 0))

(event EventTick
  (params (DeltaSeconds :type Float%20%28single-precision%29))
  (Rendering|ClearRenderTarget2D "/Game/FogOfWarSystem/FogOfWarReveal_Render.FogOfWarReveal_Render"))

(event EventStartSequence
  (|CallParentFunction)
  (Utilities|FlowControl|Sequence
    (:then_0
      (bind _returnvalue (UserInterface|CreateWidget "/Game/UIX/MainMenu/WBP_LevelTransition.WBP_LevelTransition_C"))
      (UserInterface|Viewport|AddtoViewport _returnvalue 10)
      (Default|FadeOutSequence _returnvalue false 1.0))
    (:then_1
      (bind _asbp_player_character (Utilities|Casting|CastToBP_PlayerCharacter (Variables|Default|GetPlayer)))
      (EventDispatchers|AssignOnAutomaticMovementEnded _asbp_player_character (delegate Custom|OnAutomaticMovementEnded_Event_0))
      (Development|PrintString "GM: Binded"))))

(event EventTottemCompleted
  ;[1 1 1] Unused
  (|CallParentFunction))

(event EventBeaconCompleted
  (|CallParentFunction)
  (Utilities|FlowControl|Sequence
    (:then_0
      (bind _beastai (Variables|Default|GetBeastAI)
        (:then
          (Actor|SetLifeSpan _beastai 1.0)
          (Development|PrintString "Beast killed")
          (bind _asbp_player_controller (Utilities|Casting|CastToBP_PlayerController (Game|GetPlayerController 0)))
          (Class|LLPlayerControllerBase|ShowBeastPresenceImg _asbp_player_controller false))
        (:else)))
    (:then_1
      (Utilities|FlowControl|Delay 3.0)
      (bind _returnvalue (UserInterface|CreateWidget "/Game/UIX/PlayerHUDs/WBP_TottemCompleted.WBP_TottemCompleted_C"))
      (UserInterface|Viewport|AddtoViewport _returnvalue 0)
      (Utilities|FlowControl|Delay 3.0)
      (Widget|RemovefromParent _returnvalue))
    (:then_2
      (bind _beastai_2 (Variables|Default|GetBeastAI)
        (:then
          (Actor|DestroyActor _beastai_2)
          (bind _beastlocationwidget (Variables|Default|GetBeastLocationWidget)
            (:then
              (Widget|RemovefromParent _beastlocationwidget))
            (:else
              _))
          (Development|PrintString "GBeast Destroyed"))
        (:else)))))

(event EventSpawnBeast
  (bind _timetobeast (Variables|Default|GetTimeToBeast))
  ;[0.1 0.15 0.2] Called by BP Totem when discoverd
  (Variables|Default|GetBeastAI
    (:then)
    (:else
      ;[0.9427 1 0 1 58] SpawnBeast TODO: Fix the C++ implementation
      (if (not (< _timetobeast 0.0))
        (Utilities|FlowControl|Delay _timetobeast)
        (bind _outactors (Actor|GetAllActorsOfClass "/Game/Blueprints/BeastAI/BP_Beast_SpawnPoint.BP_Beast_SpawnPoint_C"))
        (Utilities|IsValid (.OutItem (Utilities|Array|Random _outactors))
          (:Is%20Valid
            (bind _returnvalue (Game|SpawnActorfromClass (Variables|Default|GetBeastAI_Class) (Math|Transform|MakeTransform (Math|Vector|MakeVector (.x (Transformation|GetActorLocation (Utilities|Array|Get(acopy) _outactors))) (.y (Transformation|GetActorLocation (Utilities|Array|Get(acopy) _outactors))) (+ (.z (Transformation|GetActorLocation (Utilities|Array|Get(acopy) _outactors))) 2.5e+02)) "0, 0, 0" "1.000000,1.000000,1.000000") "AdjustIfPossibleButAlwaysSpawn" "SelectDefaultAtRuntime" 0 0))
            (bind _output_get (Variables|Default|SetBeastAI _returnvalue))
            (Utilities|FlowControl|Sequence
              (:then_0
                (bind _asbp_player_controller (Utilities|Casting|CastToBP_PlayerController (Game|GetPlayerController 0)))
                (Class|LLPlayerControllerBase|ShowBeastPresenceImg _asbp_player_controller true))))
          (:Is%20Not%20Valid
            (Development|PrintString "Problem Runnignquery" true true "(R=1.000000,G=0.486477,B=0.000000,A=1.000000)")))))))

(fn ConstructionScript)