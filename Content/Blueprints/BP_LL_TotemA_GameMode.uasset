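; Game mode for the Totem A level that presents the "Scape the Beast" tutorial, explaining how to evade the beast.
; ShowBeastTutorial pushes a video-enabled panel onto a tutorial container widget, stops player movement, pauses the game and shows the cursor.
; BeginPlay binds to the player character's dialogue-advance dispatcher, whose handler pops the panel and restores movement, interaction and play.
; StartSequence only calls its parent, and nothing live here triggers the tutorial.
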(event Custom|ShowBeastTutorial
  (bind _returnvalue (Game|GetPlayerController 0))
  ;[1 1 1] SPAWN BEAST TUTORIAL
  (bind _returnvalue_2 (UserInterface|CreateWidget "/Game/UIX/Tutorial/WBP_TutorialContainer.WBP_TutorialContainer_C" _returnvalue))
  (bind _output_get (Variables|Default|SetTutorialWBP _returnvalue_2))
  (UserInterface|Viewport|AddtoViewport _returnvalue_2 0)
  (Default|PushPaneltoStack _output_get "/Game/UIX/Tutorial/WBP_TutorialPanel.WBP_TutorialPanel_C" "The beast will follow Lucas when found and no the orb is empty, try to escpe by crossing different <Highlight>obstacles</> or by  <Highlight>filling the orb </> . 
 
When the beat attacks it's  <Highlight>Claws will glow </> ,  <Highlight> Jump</> to avoid being captured." "Scape the Beast " "/Game/UIX/Assets2D/Tutoria_Thumb_01.Tutoria_Thumb_01" true 3)
  (CallFunction|PlayerCanMove false)
  ;;[1 1 1] maybe we should a function in LLPlayerController
  (Game|SetGamePaused true)
  (Variables|/Script/Engine.PlayerController|SetbShowMouseCursor _returnvalue true))

(event Custom|OnDialogueAdvance_Event
  ;[1 1 1] SPAWN BEAST TUTORIAL
  ;;[1 1 1] CLOSE BEAST TUTORIAL
  (Default|RemoveWidgetfromStack (Variables|Default|GetTutorialWBP))
  (CallFunction|PlayerCanMove true)
  (CallFunction|DisableInteractionComponent false)
  (Game|SetGamePaused false)
  (Variables|/Script/Engine.PlayerController|SetbShowMouseCursor (Game|GetPlayerController 0) false))

(event EventBeginPlay
  ;[1 1 1] CARE, begin play starts before StartPlay
  (|CallParentFunction)
  (bind _asbp_player_character (Utilities|Casting|CastToBP_PlayerCharacter (Game|Player|GetPlayerPawn 0)))
  (EventDispatchers|AssignOnDialogueAdvance _asbp_player_character (EventDispatchers|CreateEvent :!event Custom|OnDialogueAdvance_Event)))

(event EventStartSequence
  (|CallParentFunction))

(fn ConstructionScript)