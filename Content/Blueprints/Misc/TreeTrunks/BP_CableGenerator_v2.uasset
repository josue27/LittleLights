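; Construction-script spline actor that generates a cable-like mesh along a spline, with optional start and end cap meshes.
; MiddleMeshSection lays spline mesh segments of MiddleSegment at intervals of actor X scale times 100, clamping tangents to that length.
; Optional StartSegment and EndSegment static meshes take position, pitch, yaw and roll from the first and last spline meshes, plus rotation offsets.
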(event EventBeginPlay)

(event Collision|EventActorBeginOverlap
  (params (OtherActor :type Actor%20Object%20Reference)))

(event EventTick
  (params (DeltaSeconds :type Float%20%28single-precision%29)))

(fn ConstructionScript
  (CallFunction|MiddleMeshSection)
  (if (Variables|StartSegment|GetAddStartSegment)
    (CallFunction|StartMeshSection))
  (if (Variables|EndSegment|GetAddEndSegment)
    (CallFunction|EndMeshSection)))

(fn MiddleMeshSection
  (bind _spline (Variables|Default|GetSpline))
  (Utilities|Array|Clear (Variables|Default|GetSplineObjects))
  (Variables|Default|SetSectionLenght (* (.x (Transformation|GetActorScale3D)) 1e+02))
  (for _index (range 0 (Math|Float|Truncate (/ (Spline|GetSplineLength (Variables|Default|GetSpline)) (Variables|Default|GetSectionLenght))))
    (bind _returnvalue (AddComponent|AddSplineMeshComponent false))
    (Utilities|Array|SetArrayElem (Variables|Default|GetSplineObjects) _index _returnvalue true)
    (Components|StaticMesh|SetStaticMesh _returnvalue (Variables|MiddleSegment|GetMiddleSegment))
    (SplineMesh|SetForwardAxis _returnvalue "X" true)
    (Transformation|AttachComponentToComponent _returnvalue (Variables|Default|GetSpline) "None" "KeepRelative" "KeepRelative" "KeepRelative" true)
    (SplineMesh|SetStartandEnd _returnvalue (Spline|GetLocationatDistanceAlongSpline _spline (* _index (Variables|Default|GetSectionLenght)) "Local") (Math|Vector|ClampVectorSize (Spline|GetTangentatDistanceAlongSpline _spline (* _index (Variables|Default|GetSectionLenght)) "Local") 0.0 (Variables|Default|GetSectionLenght)) (Spline|GetLocationatDistanceAlongSpline _spline (* (+ _index 1) (Variables|Default|GetSectionLenght)) "Local") (Math|Vector|ClampVectorSize (Spline|GetTangentatDistanceAlongSpline _spline (* (+ _index 1) (Variables|Default|GetSectionLenght)) "Local") 0.0 (Variables|Default|GetSectionLenght)) true :!class /Script/Engine.SplineMeshComponent)))

(fn StartMeshSection
  (bind _splineobjects (Variables|Default|GetSplineObjects))
  (bind _output (Utilities|Array|Get(acopy) _splineobjects))
  (bind _returnvalue (SplineMesh|GetStartTangent _output))
  (bind _returnvalue_2 (Math|Conversions|RotationFromXVector _returnvalue))
  (bind _returnvalue_3 (AddComponent|AddStaticMeshComponent false))
  (Components|StaticMesh|SetStaticMesh _returnvalue_3 (Variables|StartSegment|GetStartSegment))
  (Rendering|Material|SetMaterial _returnvalue_3 0 0)
  (Transformation|AttachComponentToComponent _returnvalue_3 (Variables|Default|GetSpline) "None" "KeepRelative" "KeepRelative" "KeepRelative" true)
  (Transformation|SetRelativeLocationAndRotation _returnvalue_3 (SplineMesh|GetStartPosition _output) (Math|Rotator|CombineRotators (Math|Rotator|MakeRotator (SplineMesh|GetStartRoll _output) (.pitch _returnvalue_2) (.yaw _returnvalue_2)) (Variables|StartSegment|GetStartMeshRotation)) false false))

(fn EndMeshSection
  (bind _splineobjects (Variables|Default|GetSplineObjects))
  (bind _returnvalue (Utilities|Array|Length _splineobjects))
  (bind _returnvalue_2 (- _returnvalue 1))
  (bind _output (Utilities|Array|Get(acopy) _splineobjects _returnvalue_2))
  (bind _returnvalue_3 (SplineMesh|GetEndTangent _output))
  (bind _returnvalue_4 (Math|Conversions|RotationFromXVector _returnvalue_3))
  (bind _returnvalue_5 (AddComponent|AddStaticMeshComponent false))
  (Components|StaticMesh|SetStaticMesh _returnvalue_5 (Variables|EndSegment|GetEndSegment))
  (Rendering|Material|SetMaterial _returnvalue_5 0 0)
  (Transformation|AttachComponentToComponent _returnvalue_5 (Variables|Default|GetSpline) "None" "KeepRelative" "KeepRelative" "KeepRelative" true)
  (Transformation|SetRelativeLocationAndRotation _returnvalue_5 (SplineMesh|GetEndPosition _output) (Math|Rotator|CombineRotators (Math|Rotator|MakeRotator (SplineMesh|GetEndRoll _output) (* (.pitch _returnvalue_4) 1.0) (.yaw _returnvalue_4)) (Variables|EndSegment|GetEndMeshRotation)) false false))