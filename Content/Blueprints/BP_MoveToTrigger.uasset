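; BP_MoveToTrigger is a trigger volume that takes control from the player and moves their character to a set destination.
; When a BP_PlayerCharacter overlaps its Box, it disables input on player 0's pawn and calls MovePlayerTo with the EndPosition component's world location and the Speed variable.
; It then destroys itself if AutoDestroy is set, and never re-enables input itself.
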(event OnComponentBeginOverlap(Box)
  (params (OverlappedComponent :type Primitive%20Component%20Object%20Reference) (OtherActor :type Actor%20Object%20Reference) (OtherComp :type Primitive%20Component%20Object%20Reference) (OtherBodyIndex :type Integer) (bFromSweep :type Boolean) (SweepResult :type Hit%20Result%20Structure%20%28by%20ref%29))
  (bind _asbp_player_character (Utilities|Casting|CastToBP_PlayerCharacter OtherActor))
  (Input|DisableInput (Game|Player|GetPlayerPawn 0) (Game|GetPlayerController 0))
  (Default|MovePlayerto _asbp_player_character (Transformation|GetWorldLocation (Variables|Default|GetEndPosition)) (Variables|Default|GetSpeed))
  (if (Variables|Default|GetAutoDestroy)
    (Actor|DestroyActor)))

(event EventBeginPlay)

(event Collision|EventActorBeginOverlap
  (params (OtherActor :type Actor%20Object%20Reference)))

(event EventTick
  (params (DeltaSeconds :type Float%20%28single-precision%29)))

(fn ConstructionScript)