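; Base interactable actor for special movement zones (jump over, crouch, balance crossing), with the construction script setting the prompt by zone type.
; StartCrossing snaps the player to the nearer spline end, and losing balance launches them sideways before restoring movement.
; Much is unwired: the overlap and jump-over events are empty, and the crossing dispatch and axis-driven lerp between spline ends never run.
; Tick draws debug spheres at end positions.
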(event Custom|StartCrossing
  (bind _bp_playercharacter (Variables|Default|GetBP_PlayerCharacter))
  (bind _bp_playercharacter_2 (Variables|Default|GetBP_PlayerCharacter))
  (bind _bp_playercharacter_3 (Variables|Default|GetBP_PlayerCharacter))
  (bind _splinepath (Variables|Default|GetSplinePath))
  (bind _returnvalue (Transformation|GetActorLocation _bp_playercharacter))
  (bind _returnvalue_2 (Spline|GetLocationatSplinePoint _splinepath 0 "World"))
  (bind _returnvalue_3 (Spline|GetNumberOfSplinePoints _splinepath))
  (bind _returnvalue_4 (Transformation|GetActorRotation _bp_playercharacter))
  (bind _returnvalue_5 (Spline|GetLocationatSplinePoint _splinepath _returnvalue_3 "World"))
  ;[1 1 1] Balancing
  (Development|PrintString "Cross balancing")
  (Variables|Default|SetbIsBalancing true)
  (Variables|Default|SetbIsJumping true)
  (Collision|SetCollisionResponsetoChannel (Variables|Default|GetBlockerCollider) "ECC_Pawn" "ECR_Overlap")
  (Components|Activation|SetActive (Variables|/Script/Engine.Character|GetCapsuleComponent _bp_playercharacter_2) false false)
  (Default|StartUnbalnce _bp_playercharacter_2)
  (bind _bclosertoend (CallFunction|GetCloserPoint))
  (if _bclosertoend
    ;;[1 1 1] All this could be in closerpoint function
    (Transformation|SetActorRotation _bp_playercharacter (Math|Rotator|MakeRotator (.roll _returnvalue_4) (.pitch _returnvalue_4) (- (.yaw (Spline|GetRotationatSplinePoint _splinepath (Spline|GetNumberOfSplinePoints _splinepath) "World")) 1.8e+02)))
    (Variables|Default|SetZ_offset (- (.z _returnvalue) (.z _returnvalue_5)))
    (Transformation|SetActorLocation _bp_playercharacter_3 (Math|Vector|MakeVector (.x _returnvalue_5) (.y _returnvalue_5) (.z _returnvalue)) false false)
    (Variables|Default|SetbEndLocation true)
    (else
      (Transformation|SetActorRotation _bp_playercharacter (Math|Rotator|MakeRotator (.roll _returnvalue_4) (.pitch _returnvalue_4) (.yaw (Spline|GetRotationatSplinePoint _splinepath 0 "World"))))
      (Variables|Default|SetZ_offset (- (.z _returnvalue) (.z _returnvalue_2)))
      ;;[1 1 1] Close to start
      (Transformation|SetActorLocation _bp_playercharacter_3 (Math|Vector|MakeVector (.x _returnvalue_2) (.y _returnvalue_2) (.z _returnvalue)) false false)
      (Variables|Default|SetbEndLocation false))))

(event Custom|StartJumpOver_1
  (params (TypeOfMovement :type EspecialMovementZoneType%20Enum%20%28by%20ref%29 :default "JumpOver") (Player :type Player%20Character%20Object%20Reference)))

(event Custom|MovePlayerAlongSpline_1
  (params (axisValue :type Float%20%28single-precision%29))
  ;[1 1 1] Balancing
  ;;[1 1 1] Balancing input
  (if (!= (* axisValue (Variables|Default|GetCrossingVelocityMultiplier)) 0.0)
    _))

(event Custom|PlayerLostBalance_1
  (bind _bp_playercharacter (Variables|Default|GetBP_PlayerCharacter))
  ;[1 1 1] Balancing
  (Development|PrintString "Player unbalanced" true true "(R=1.000000,G=0.000000,B=0.023671,A=1.000000)")
  (Utilities|FlowControl|Delay 1.0)
  (Variables|/Script/LittleLights.PlayerCharacter|SetbBalancing _bp_playercharacter false)
  (Variables|Default|SetDistanceWalked_X 0.0)
  (Character|LaunchCharacter _bp_playercharacter (* (Transformation|GetActorRightVector _bp_playercharacter) (* (Variables|/Script/LittleLights.PlayerCharacter|GetBalancing_X _bp_playercharacter) 3e+02)) false false)
  (Variables|/Script/LittleLights.PlayerCharacter|SetBalancing_X _bp_playercharacter 0.0)
  (Utilities|FlowControl|Delay 2.0)
  (Variables|/Script/LittleLights.PlayerCharacter|SetbCanMove _bp_playercharacter true)
  (Variables|/Script/LittleLights.PlayerCharacter|SetbInJumpOverZone _bp_playercharacter false))

(event EventBeginPlay
  (Utilities|FlowControl|Sequence
    (:then_0
      (if (Utilities|Enum|Equal(Enum) (Variables|Default|GetMovementZone_Type) "SMZ_Crouch")
        _))))

(event Collision|EventActorBeginOverlap
  (params (OtherActor :type Actor%20Object%20Reference)))

(event EventTick
  (params (DeltaSeconds :type Float%20%28single-precision%29))
  (bind _endpositions (Variables|Default|GetEndPositions))
  (if (> (Utilities|Array|Length _endpositions) 0)
    (for _array_element _endpositions
      (Rendering|Debug|DrawDebugSphere _array_element 1e+01 12 "(R=1.000000,G=0.000000,B=0.123685,A=1.000000)" 0.0))))

(event EventInteract
  (params (InstigatorPawn :type Pawn%20Object%20Reference))
  (Development|PrintString "Interacting with")
  (|CallParentFunction InstigatorPawn))

(fn ConstructionScript
  (Utilities|FlowControl|Sequence
    (:then_0
      (switch Utilities|FlowControl|Switch|SwitchonELLSpecialMovementZoneType (Variables|Default|GetMovementZone_Type)
        (:SMZ_JumpOver
          (Variables|Default|SetInteractionMessage "Press E to Jump Over"))
        (:SMZ_Crouch
          (Variables|Default|SetInteractionMessage "Press E to Crouch"))
        (:SMZ_CrossBalancing
          (Variables|Default|SetInteractionMessage "Press E to Balance"))))))

(fn GetCloserPoint
  (bind _splinepath (Variables|Default|GetSplinePath))
  (bind _bp_playercharacter (Variables|Default|GetBP_PlayerCharacter))
  (bind _returnvalue (Transformation|GetActorLocation _bp_playercharacter))
  (Utilities|IsValid _bp_playercharacter
    (:Is%20Valid
      (if (< (Math|Vector|Distance(Vector) _returnvalue (Spline|GetLocationatSplinePoint _splinepath 0 "World")) (Math|Vector|Distance(Vector) _returnvalue (Spline|GetLocationatSplinePoint _splinepath (Spline|GetNumberOfSplinePoints _splinepath) "World")))
        (return false)
        (else
          (return true))))))