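; Level-exit door that, once unlocked by event or flag, opens when the player overlaps its trigger.
; A timeline drives the vine grow mask on a dynamic material and shifts totem emissive and rect light colors, then clears blocking and enables the auto-walk trigger.
; That trigger moves the player toward EndWalkPoint and changes level a quarter of the way through the estimated walk time.
; BeginPlay sets initial collision from CanOpenDoor and IsReturnDoor.
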(event OnComponentBeginOverlap(DoorTrigger)
  (params (OverlappedComponent :type Primitive%20Component%20Object%20Reference) (OtherActor :type Actor%20Object%20Reference) (OtherComp :type Primitive%20Component%20Object%20Reference) (OtherBodyIndex :type Integer) (bFromSweep :type Boolean) (SweepResult :type Hit%20Result%20Structure%20%28by%20ref%29))
  ;[1 1 1] Detects the player to open the door
  (Utilities|Casting|CastToBP_PlayerCharacter OtherActor)
  (CallFunction|OpenDoor))

(event OnComponentBeginOverlap(AutoWalkTrigger)
  (params (OverlappedComponent :type Primitive%20Component%20Object%20Reference) (OtherActor :type Actor%20Object%20Reference) (OtherComp :type Primitive%20Component%20Object%20Reference) (OtherBodyIndex :type Integer) (bFromSweep :type Boolean) (SweepResult :type Hit%20Result%20Structure%20%28by%20ref%29))
  ;[1 1 1] Trigger the end walk for the player
  (bind _asbp_player_character (Utilities|Casting|CastToBP_PlayerCharacter OtherActor))
  (Development|PrintString "Aking player to autowalk")
  (Collision|SetCollisionEnabled (Variables|Default|GetBlockCollision) "NoCollision")
  (bind _endwalkpoint (Variables|Default|GetEndWalkPoint)
    (:then
      (Default|MovePlayerto _asbp_player_character (Transformation|GetActorLocation _endwalkpoint) 4e+02 false true true)
      (bind _returnvalue (Class|LLGamePlayFunctionLibrary|TimetoLocation 1.5e+02 (Transformation|GetActorLocation (Game|Player|GetPlayerPawn 0)) (Transformation|GetActorLocation _endwalkpoint)))
      (Utilities|FlowControl|Delay (/ _returnvalue 4.0))
      (CallFunction|ChangeLevel false (Variables|DoorBase|GetLevelToChange)))
    (:else)))

(event Custom|OpenDoor
  ;[1 1 1] Opern Door animation
  (if (and (Variables|Default|GetbDoorUnlocked) (not (Variables|Default|GetbDoorOpened)))
    (Variables|Default|SetbDoorOpened true)
    (bind _alpha (Timeline|VineAlpha PlayFromStart)
      (:Update
        (Rendering|Material|SetScalarParameterValue (Variables|DoorBase|GetVineMAT) (Variables|DoorBase|GetGrowMask) (Math|Float|Lerp -0.6 2.0 _alpha) :!class /Script/Engine.MaterialInstanceDynamic)
        (Rendering|Material|SetVectorParameterValue (Variables|Default|GetTottemMAT) "EmissiveColor_Ctrl" (Math|Color|Lerp(LinearColor) "(R=1.000000,G=0.000000,B=0.000000,A=1.000000)" "(R=0.000000,G=0.969695,B=1.000000,A=1.000000)" (* _alpha 1.5)) :!class /Script/Engine.MaterialInstanceDynamic)
        (Rendering|Components|Light|SetLightColor (Variables|Default|GetRectLight) (Math|Color|Lerp(LinearColor) (Math|Conversions|ToLinearColor(Color) (Variables|DoorBase|GetCloseColor)) (Math|Conversions|ToLinearColor(Color) (Variables|DoorBase|GetOpenColor)) (* _alpha 1.5)) true))
      (:Finished
        (Collision|SetCollisionResponsetoAllChannels (Variables|Default|GetBlockCollision) "ECR_Ignore")
        (Collision|SetCollisionEnabled (Variables|Default|GetAutoWalkTrigger) "QueryOnly")))))

(event Custom|UnlockDoor
  (Variables|Default|SetbDoorUnlocked true))

(event EventBeginPlay
  (Utilities|FlowControl|Sequence
    (:then_0
      (Rendering|Material|SetVectorParameterValue (Variables|Default|GetTottemMAT) "EmissiveColor_Ctrl" "(R=1.000000,G=0.021061,B=0.000000,A=1.000000)" :!class /Script/Engine.MaterialInstanceDynamic))
    (:then_1
      (if (Variables|Default|GetbDoorUnlocked)
        (if (Class|DoorBase|CanOpenDoor)
          (Collision|SetCollisionEnabled (Variables|Default|GetBlockCollision) "NoCollision"))))
    (:then_2
      (if (Variables|DoorBase|GetbIsReturnDoor)
        (Collision|SetCollisionEnabled (Variables|Default|GetBlockCollision) "QueryAndPhysics")))))

(event Collision|EventActorBeginOverlap
  (params (OtherActor :type Actor%20Object%20Reference)))

(event EventTick
  (params (DeltaSeconds :type Float%20%28single-precision%29)))

(event EventEndGameEvent
  (Variables|Default|SetbDoorUnlocked true))

(fn ConstructionScript
  (Utilities|FlowControl|Sequence
    (:then_0
      (bind _returnvalue (Rendering|Material|CreateDynamicMaterialInstance (Variables|Default|GetDM_Tottem_C) 0 "/Game/Materials/Instances/Tottems/MI_Tottems.MI_Tottems" "None" :!class /Script/Engine.PrimitiveComponent))
      (Variables|Default|SetTottemMAT _returnvalue)
      (bind _returnvalue_2 (Rendering|Material|CreateDynamicMaterialInstance (Variables|Default|GetVinesMesh) 0 "/Game/Materials/Instances/GateTree/MI_GrowingVines.MI_GrowingVines" "None" :!class /Script/Engine.PrimitiveComponent))
      (Variables|DoorBase|SetVineMAT _returnvalue_2))
    (:then_1
      (Variables|DoorBase|SetCloseColor (Math|Conversions|ToColor(LinearColor) (Rendering|Components|Light|GetLightColor (Variables|Default|GetRectLight)))))))