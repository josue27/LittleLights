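; Tutorial orb Blueprint that pulses a referenced point light together with the glow of its liquid mesh.
; Construction creates a dynamic instance of MI_Liquid and caches its initial emission.
; TurnOnLight starts a timeline that lerps light intensity and material emission, with a FlipFlop on Finished alternating forward and reverse playback to loop indefinitely.
; BeginPlay only runs an unconnected delay, and nothing here calls TurnOnLight.
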(event Custom|TurnOnLight
  (bind _pointlight (Variables|Default|GetPointLight)
    (:then
      (Utilities|FlowControl|FlipFlop :!label _label
        (:A
          (bind (_direction _intensity) (Timeline|Timeline Play)
            (:Update
              (Rendering|Components|Light|SetIntensity (Variables|/Script/Engine.PointLight|GetPointLightComponent _pointlight) (Math|Float|Lerp 1e+01 3.0 _intensity))
              (Rendering|Material|SetScalarParameterValue (Variables|Default|GetLiquidMaterial) (Variables|Default|GetEmissionParameter) (Math|Float|Lerp 1e+01 1.0 _intensity) :!class /Script/Engine.MaterialInstanceDynamic))
            (:Finished
              (goto _label))))
        (:B
          (Timeline|Timeline ReverseFromEnd))))
    (:else)))

(event EventBeginPlay
  (Utilities|FlowControl|Delay 1e+01))

(event Collision|EventActorBeginOverlap
  (params (OtherActor :type Actor%20Object%20Reference)))

(event EventTick
  (params (DeltaSeconds :type Float%20%28single-precision%29)))

(fn ConstructionScript
  (bind _returnvalue (Rendering|Material|CreateDynamicMaterialInstance (Variables|Default|GetDM_Liquid) 0 "/Game/Materials/Instances/OrbStick/MI_Liquid.MI_Liquid" "None" :!class /Script/Engine.PrimitiveComponent))
  (bind _output_get (Variables|Default|SetLiquidMaterial _returnvalue))
  (bind _returnvalue_2 (Rendering|Material|GetScalarParameterValue _output_get (Variables|Default|GetEmissionParameter) :!class /Script/Engine.MaterialInstanceDynamic))
  (Variables|Default|SetInitialEmission _returnvalue_2))