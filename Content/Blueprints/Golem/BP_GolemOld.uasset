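; Golem AI pawn that walks to requested locations and turns to face the player.
; MoveToLocation uses SimpleMoveToLocation and assumes arrival after a Delay estimated from distance and fixed speed, then signals AutomaticMovementFinished.
; VisionTrigger overlaps start and clear a looping timer for yaw-only, interpolated look-at rotation.
; ShouldLookPlayer and velocity are checked only when that timer starts.
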(event OnComponentBeginOverlap(VisionTrigger)
  (params (OverlappedComponent :type Primitive%20Component%20Object%20Reference) (OtherActor :type Actor%20Object%20Reference) (OtherComp :type Primitive%20Component%20Object%20Reference) (OtherBodyIndex :type Integer) (bFromSweep :type Boolean) (SweepResult :type Hit%20Result%20Structure%20%28by%20ref%29))
  (Utilities|Casting|CastToBP_PlayerCharacter OtherActor)
  (if (not (and (Variables|Default|GetShouldLookPlayer) (> (Math|Vector|VectorLength (Transformation|GetVelocity)) 0.0)))
    (bind _returnvalue (Utilities|Time|SetTimerbyEvent (EventDispatchers|CreateEvent :!event Custom|LookAtPlayer) 0.01 true))
    (Variables|Default|SetLookAtPlayerTimer _returnvalue)))

(event OnComponentEndOverlap(VisionTrigger)
  (params (OverlappedComponent :type Primitive%20Component%20Object%20Reference) (OtherActor :type Actor%20Object%20Reference) (OtherComp :type Primitive%20Component%20Object%20Reference) (OtherBodyIndex :type Integer))
  (Utilities|Casting|CastToBP_PlayerCharacter OtherActor)
  (Utilities|Time|ClearandInvalidateTimerbyHandle (Variables|Default|GetLookAtPlayerTimer)))

(event Custom|LookAtPlayer
  (bind _asbp_player_character (Utilities|Casting|CastToBP_PlayerCharacter (Game|Player|GetPlayerPawn 0)))
  ;[0.1 0.15 0.2] Comment
  (Transformation|SetActorRotation (Math|Rotator|MakeRotator 0.0 0.0 (.yaw (Math|Interpolation|RInterpTo (Transformation|GetActorRotation) (Math|Rotator|FindLookatRotation (Transformation|GetActorLocation) (Transformation|GetActorLocation _asbp_player_character)) (Utilities|Time|GetWorldDeltaSeconds) 1e+01)))))

(event Custom|MoveToLocation
  (params (Destination :type Vector))
  (Variables|Default|SetShouldLookPlayer false)
  (Rendering|Debug|DrawDebugBox Destination "10.000000,10.000000,10.000000" "(R=0.000000,G=1.000000,B=0.075730,A=1.000000)" "0, 0, 0" 5.0 3.0)
  (bind _returnvalue (Class|LLGamePlayFunctionLibrary|TimetoLocation 1.5e+02 (Transformation|GetActorLocation) Destination))
  (AI|Navigation|SimpleMovetoLocation (Pawn|GetController) Destination)
  (Utilities|FlowControl|Delay _returnvalue)
  (Variables|Default|SetShouldLookPlayer true)
  (Development|PrintString "Golem Finished Movement")
  (Default|CallAutomaticMovementFinished))

(event EventBeginPlay
  (|CallParentFunction) ; This node is disabled and will not be called.\nDrag off pins to build functionality.
)

(event Collision|EventActorBeginOverlap
  (params (OtherActor :type Actor%20Object%20Reference))
  (|CallParentFunction OtherActor) ; This node is disabled and will not be called.\nDrag off pins to build functionality.
)

(event EventTick
  (params (DeltaSeconds :type Float%20%28single-precision%29))
  (|CallParentFunction DeltaSeconds) ; This node is disabled and will not be called.\nDrag off pins to build functionality.
)

(fn ConstructionScript
  (|CallParentFunction))