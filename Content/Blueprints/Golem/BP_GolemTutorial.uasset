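; BP_GolemTutorial is the tutorial golem, an AI-controlled actor that walks to requested destinations and can turn to face the player.
; MoveToLocation stops the look timer and starts a simple AI move, whose successful completion calls AutomaticMovementFinished.
; A looping timer, restarted on arrival if ShouldLookPlayer is set or via TriggerLookAtPlayer, drives smoothed yaw-only rotation toward the player.
; CanLookPlayer sets that flag.
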(event Custom|TriggerLookAtPlayer
  (bind _returnvalue (Utilities|Time|SetTimerbyEvent (EventDispatchers|CreateEvent :!event Custom|LookAtPlayer) 0.05 true))
  (Variables|LLGolem|SetLookAtPlayerTimer _returnvalue))

(event Custom|LookAtPlayer
  ;[0.1 0.15 0.2] Look at player
  (bind _asbp_player_character (Utilities|Casting|CastToBP_PlayerCharacter (Game|Player|GetPlayerPawn 0)))
  (Transformation|SetActorRotation (Math|Rotator|MakeRotator 0.0 0.0 (.yaw (Math|Interpolation|RInterpTo (Transformation|GetActorRotation) (Math|Rotator|FindLookatRotation (Transformation|GetActorLocation) (Transformation|GetActorLocation _asbp_player_character)) (Utilities|Time|GetWorldDeltaSeconds) 2e+01)))))

(event Custom|MoveToLocation
  (params (Destination :type Vector))
  (Utilities|Time|ClearandInvalidateTimerbyHandle (Variables|LLGolem|GetLookAtPlayerTimer))
  (bind _returnvalue (Class|LLGamePlayFunctionLibrary|TimetoLocation 1.5e+02 (Transformation|GetActorLocation) Destination))
  (AI|Navigation|SimpleMovetoLocation (Pawn|GetController) Destination)
  (EventDispatchers|BindEventtoReceiveMoveCompleted (AI|GetAIController self) (delegate Custom|CustomEvent)))

(event Custom|CustomEvent
  (params (RequestID :type AI%20Request%20ID%20Structure) (Result :type EPathFollowingResult%20Enum :default "Success"))
  (if (Utilities|Enum|Equal(Enum) Result "Success")
    (Default|CallAutomaticMovementFinished)
    (Development|PrintString "Golem Finished Movement")
    (if (Variables|LLGolem|GetShouldLookPlayer)
      (bind _returnvalue (Utilities|Time|SetTimerbyEvent (EventDispatchers|CreateEvent :!event Custom|LookAtPlayer) 0.05 true))
      (Variables|LLGolem|SetLookAtPlayerTimer _returnvalue))))

(event EventBeginPlay
  (|CallParentFunction) ; This node is disabled and will not be called.\nDrag off pins to build functionality.
)

(event Collision|EventActorBeginOverlap
  (params (OtherActor :type Actor%20Object%20Reference))
  (|CallParentFunction OtherActor) ; This node is disabled and will not be called.\nDrag off pins to build functionality.
)

(event EventTick
  (params (DeltaSeconds :type Float%20%28single-precision%29))
  (|CallParentFunction DeltaSeconds) ; This node is disabled and will not be called.\nDrag off pins to build functionality.
)

(fn ConstructionScript
  (|CallParentFunction))

(fn CanLookPlayer
  (params (ShouldLookPlayer :type Boolean))
  (Utilities|FlowControl|Sequence
    (:then_0
      (if ShouldLookPlayer
        _
        (else
          _))
      (Utilities|Time|ClearandInvalidateTimerbyHandle (Variables|LLGolem|GetLookAtPlayerTimer))
      (CallFunction|LookatPlayer))
    (:then_1
      (Variables|LLGolem|SetShouldLookPlayer ShouldLookPlayer))))