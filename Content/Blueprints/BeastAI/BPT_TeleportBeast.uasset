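; Behavior tree task that teleports the AI-controlled beast back near the player when it falls too far behind.
; It reads the PlayerTarget blackboard key and, past a distance threshold, moves the pawn to a random reachable navigation point around the player without sweeping.
; It finishes successfully whether or not it moves, but never calls FinishExecute if the player cast fails.
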(event EventReceiveExecuteAI
  (params (OwnerController :type AI%20Controller%20Object%20Reference) (ControlledPawn :type Pawn%20Object%20Reference))
  (bind _asbp_player_character (Utilities|Casting|CastToBP_PlayerCharacter (AI|BehaviorTree|GetBlackboardValueasActor (Variables|Default|GetPlayerTarget))))
  (if (>= (Math|Vector|Distance(Vector) (Transformation|GetActorLocation _asbp_player_character) (Transformation|GetActorLocation ControlledPawn)) 1e+03)
    (Transformation|SetActorLocation ControlledPawn (.RandomLocation (AI|Navigation|GetRandomReachablePointinRadius (Transformation|GetActorLocation _asbp_player_character) 7e+02 0 0)) false false)
    (AI|BehaviorTree|FinishExecute true)
    (else
      (AI|BehaviorTree|FinishExecute true))))