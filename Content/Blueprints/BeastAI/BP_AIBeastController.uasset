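; AI controller for the beast that turns perception of the player and orb-area state into Blackboard values.
; Sight sets TargetActor; losing sight starts a short grace timer, after which the target is cleared and the stimulus location becomes TargetLocation.
; Other senses cancel that timer and write the stimulus location directly.
; InsideOrbArea sets the escape-from-light flag.
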(event OnTargetPerceptionUpdated(AIPerception)
  (params (Actor :type Actor%20Object%20Reference) (Stimulus :type AI%20Stimulus%20Structure))
  (bind (_age _expirationage _strength _stimuluslocation _receiverlocation _tag _bsuccessfullysensed) (Utilities|Struct|BreakAIStimulus Stimulus))
  (bind _blackboard (Variables|Default|GetBlackboard))
  (Utilities|Casting|CastToBP_PlayerCharacter Actor)
  (bind _returnvalue (Class|AIPerceptionSystem|GetSenseClassforStimulus Stimulus))
  (if (== _returnvalue "/Script/AIModule.AISense_Sight")
    (if _bsuccessfullysensed
      (Utilities|Time|ClearandInvalidateTimerbyHandle (Variables|Default|GetTargetLostTimer))
      (AI|Components|Blackboard|SetValueasObject _blackboard (Utilities|Name|MakeLiteralName "TargetActor") Actor)
      (else
        (bind _returnvalue_2 (Utilities|Time|SetTimerbyEvent (delegate Custom|TargetLost) 3.0))
        (Variables|Default|SetTargetLostTimer _returnvalue_2)))
    (else
      (Utilities|Time|ClearandInvalidateTimerbyHandle (Variables|Default|GetTargetLostTimer))
      (AI|Components|Blackboard|SetValueasVector _blackboard (Utilities|Name|MakeLiteralName "TargetLocation") _stimuluslocation))))

(event Custom|InsideOrbArea
  (params (InsideArea :type Boolean))
  ;[0.1 0.15 0.2] Is the beast inside the orb area and is it on?
  (bind _output_get (Variables|Default|SetEscaping InsideArea))
  (AI|Components|Blackboard|SetValueasBool (Variables|Default|GetBlackboard) (Variables|Default|GetEscapeLight_Key) _output_get))

(event Custom|TargetLost
  (bind _blackboard (Variables|Default|GetBlackboard))
  (AI|Components|Blackboard|ClearValue _blackboard (Utilities|Name|MakeLiteralName "TargetActor"))
  (AI|Components|Blackboard|SetValueasVector _blackboard (Utilities|Name|MakeLiteralName "TargetLocation") (.StimulusLocation (Utilities|Struct|BreakAIStimulus (stale OnTargetPerceptionUpdated(AIPerception) Stimulus)))))

(event EventBeginPlay)

(event EventTick
  (params (DeltaSeconds :type Float%20%28single-precision%29)))

(fn ConstructionScript)