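; AI beast enemy that chases, grabs and flees from the player, tracking path distance each tick for walk camera shake and a first-encounter tutorial.
; Orb refilling slows its time dilation; completion makes it scream and flee through its AI controller.
; Right-hand overlap captures non-immune players, revealing a child-actor stand-in at the hand socket.
; An EQS teleport toward the player exists, but the distance check only sets its flag.
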(event OnComponentBeginOverlap(RighHandCollision)
  (params (OverlappedComponent :type Primitive%20Component%20Object%20Reference) (OtherActor :type Actor%20Object%20Reference) (OtherComp :type Primitive%20Component%20Object%20Reference) (OtherBodyIndex :type Integer) (bFromSweep :type Boolean) (SweepResult :type Hit%20Result%20Structure%20%28by%20ref%29))
  (bind _childactor (Variables|Default|GetChildActor))
  (if (and (Variables|Default|GetbIsAttacking) (not (Variables|Default|GetPlayerCaptured)))
    (bind _asbp_player_character (Utilities|Casting|CastToBP_PlayerCharacter OtherActor))
    (if (not (GameplayTags|HasTag (Variables|/Script/LittleLights.LL_AbilityComponent|GetActiveGameplayTags (Variables|/Script/LittleLights.PlayerCharacter|GetAbilityComponent _asbp_player_character)) "(TagName=\"Action.Inmune\")"))
      (Default|Captured _asbp_player_character)
      (Variables|Default|SetPlayerCaptured true)
      (Transformation|SetWorldLocation _childactor (Transformation|GetSocketLocation (Variables|Character|GetMesh) "RightHand") false true)
      (Rendering|SetVisibility _childactor true false)
      (bind _asbp_player_captured (Utilities|Casting|CastToBP_PlayerCaptured (Variables|/Script/Engine.ChildActorComponent|GetChildActor _childactor)))
      (Default|ActivateDragRoll _asbp_player_captured)
      (Utilities|FlowControl|Delay 1.0)
      (Animation|Montage|PlayMontage (Variables|Character|GetMesh) "/Game/Assets3D/Beast/Beast_Temp/ZombieScream_Montage.ZombieScream_Montage"))))

(event Custom|DisableGrabZone
  (bind _righhandcollision (Variables|Default|GetRighHandCollision))
  ;[1 1 1] Disabled, not workign for the moment
  (Development|PrintString "animnotify")
  (CallFunction|ActivateParryVisual false)
  (Collision|SetCollisionEnabled _righhandcollision "NoCollision")
  (Rendering|SetVisibility _righhandcollision false false))

(event Custom|ActivateGrabZone
  (bind _righhandcollision (Variables|Default|GetRighHandCollision))
  ;[1 1 1] Disabled, not workign for the moment
  (Development|PrintString "Start animnotify")
  (CallFunction|ActivateParryVisual true)
  (Collision|SetCollisionEnabled _righhandcollision "QueryOnly")
  (Rendering|SetVisibility _righhandcollision true false))

(event Custom|OnQueryFinishedEvent_Event_0
  (params (QueryInstance :type Env%20Query%20Instance%20Blueprint%20Wrapper%20Object%20Reference) (QueryStatus :type EEnvQueryStatus%20Enum :default "Processing"))
  ;[0.1 0.15 0.2] TELEPORT DISTANCE TO A POSITION CLOSER TO THE PLAYER
  (bind (_resultlocations _returnvalue) (AI|EQS|GetQueryResultsasLocations QueryInstance))
  (if _returnvalue
    (bind _returnvalue_2 (Transformation|SetActorLocation (Utilities|Array|Get(acopy) _resultlocations) false true))
    (if _returnvalue_2
      _
      (else
        _)))
  (Utilities|FlowControl|RetriggerableDelay 3.0)
  (Variables|Default|SetStartedTeleport false))

(event Custom|BeastTeleported
  ;[0.102 0.149 0.2] CHECK PLAYER DISTANCE FROM BEAST
  (Utilities|FlowControl|DoOnce false ; enters at Reset
    (:Completed
      (Utilities|Time|SetTimerbyFunctionName 0 "TeleportBeast" 3.0))))

(event Custom|ActivateParryVisual
  (params (Activate :type Boolean))
  (Rendering|SetVisibility (Variables|Default|GetClawGlow_Dummy) Activate false))

(event Custom|OnRefillingOrb_Event_0
  (params (bRefilling :type Boolean))
  ;[0.1 0.15 0.2] Refilling orb
  (if bRefilling
    (Variables|Default|SetCustomTimeDilation 0.2)
    (else
      (Variables|Default|SetCustomTimeDilation 1.0))))

(event Custom|Flee
  (params (InsideArea :type Boolean))
  ;[0.102 0.149 0.2] Flee trigger logic
  (if InsideArea
    ;;[0.1 0.15 0.2] This changes the walk speed
    (CallFunction|ChangeWalkSpeed "Flee")
    (else
      (Utilities|FlowControl|Delay 3.0)
      (CallFunction|ChangeWalkSpeed "Normal")))
  (bind _asbp_aibeast_controller (Utilities|Casting|CastToBP_AIBeastController (Pawn|GetController)))
  (Default|InsideOrbArea _asbp_aibeast_controller InsideArea)
  (Collision|SetCollisionEnabled (Variables|Default|GetRighHandCollision) "NoCollision"))

(event Custom|ChangeWalkSpeed
  (params (Type :type String))
  (bind _charactermovement (Variables|Character|GetCharacterMovement))
  ;[0.1 0.15 0.2] Change Walk speed
  (switch string Type
    (:Normal
      (Variables|/Script/Engine.CharacterMovementComponent|SetMaxWalkSpeed _charactermovement (Variables|Default|GetNormalWalkSpeed)))
    (:Flee
      (Variables|/Script/Engine.CharacterMovementComponent|SetMaxWalkSpeed _charactermovement (Variables|Default|GetFleeWalkSpeed)))
    (:Stop
      (Variables|/Script/Engine.CharacterMovementComponent|SetMaxWalkSpeed _charactermovement 0.0))))

(event Custom|OnOrbRefillFinished_Event_0
  (params (bRefillingFinished :type Boolean))
  ;[0.1 0.15 0.2] Check when finishing the orb filling if the beast needs to flee
  (Variables|Default|SetCustomTimeDilation 1.0)
  (bind _asbp_player_character (Utilities|Casting|CastToBP_PlayerCharacter (Game|Player|GetPlayerPawn 0)))
  (CallFunction|Flee true)
  (Audio|PlaySoundatLocation "/Game/Audio/SFX/MonsterScream_Cue.MonsterScream_Cue" (Transformation|GetActorLocation) "0, 0, 0" 1.0 1.0 0.0 0 0 0 0))

(event Custom|CheckPlayerDistance
  ;[0.102 0.149 0.2] CHECK PLAYER DISTANCE FROM BEAST
  (Utilities|FlowControl|Sequence
    (:then_0
      (bind _llplayer (Variables|Default|GetLLPlayer)
        (:then
          (bind _returnvalue (Class|NavigationSystemV1|FindPathtoActorSynchronously (Transformation|GetActorLocation) _llplayer 5e+01 (Pawn|GetController) "/Game/Blueprints/Navigation/BP_QueryBeastFilter.BP_QueryBeastFilter_C"))
          (bind _output_get (Variables|Default|SetNavPathRef _returnvalue))
          (Utilities|FlowControl|Sequence
            (:then_0
              (if (> (Class|NavigationPath|GetPathLength _output_get) 2e+03)
                (if (not (Variables|Default|GetStartedTeleport))
                  (Variables|Default|SetStartedTeleport true))
                (else
                  (Utilities|FlowControl|Sequence
                    (:then_1
                      (if (> (Math|Vector|VectorLength (Transformation|GetVelocity)) 1.0)
                        (bind _llplayer_2 (Variables|Default|GetLLPlayer)
                          (:then
                            (Camera|PlayWorldCameraShake "/Game/Blueprints/FX/BP_BeastWalk_CamShake.BP_BeastWalk_CamShake_C" (Transformation|GetWorldLocation (Variables|/Script/LittleLights.PlayerCharacter|GetCameraComp _llplayer_2)) 0.0 5e+02 0.5))
                          (:else))))))))
            (:then_2
              (if (<= (Class|NavigationPath|GetPathLength _output_get) 5.5e+02)
                ;[1 1 1] THIS WIL TRIGGER EVERYTIME THE FIRST TIME THE USER ENCOUNTER THE MONSTER IN LEVEL A
                (if (Variables|Default|GetbFirstTime)
                  (bind _asbp_ll_totem_a_game_mode (Utilities|Casting|CastToBP_LL_TotemA_GameMode (Game|GetGameMode)))
                  (Default|ShowBeastTutorial _asbp_ll_totem_a_game_mode)
                  (Variables|Default|SetbFirstTime false))))))
        (:else)))))

(event Custom|TeleportBeast
  ;[0.1 0.15 0.2] TELEPORT DISTANCE TO A POSITION CLOSER TO THE PLAYER
  (bind _returnvalue (AI|EQS|RunEQSQuery "/Game/Blueprints/BeastAI/QueryTeleportAroundPlayer.QueryTeleportAroundPlayer" self "SingleResult"))
  (EventDispatchers|AssignOnQueryFinishedEvent _returnvalue (delegate Custom|OnQueryFinishedEvent_Event_0)))

(event EventBeginPlay
  (bind _asbp_ll_player_state (Utilities|Casting|CastToBP_LL_PlayerState (Game|GetPlayerState 0)))
  (EventDispatchers|AssignOnRefillingOrb _asbp_ll_player_state (EventDispatchers|CreateEvent :!event Custom|OnRefillingOrb_Event_0))
  (EventDispatchers|AssignOnOrbRefillFinished _asbp_ll_player_state (EventDispatchers|CreateEvent :!event Custom|OnOrbRefillFinished_Event_0)))

(event Collision|EventActorBeginOverlap
  (params (OtherActor :type Actor%20Object%20Reference)))

(event EventTick
  (params (DeltaSeconds :type Float%20%28single-precision%29))
  (CallFunction|CheckPlayerDistance))

(event EventBasicAttackSequence
  (Development|PrintString "Beast Basic attack" true true "(R=0.859922,G=1.000000,B=0.000000,A=1.000000)" 5.0))

(event EventSetBeastAlerted
  (params (Alert%20State :type EBeastState%20Enum :default "EBS_Neutral"))
  (bind _beaststate_text (Variables|Default|GetBeastState_Text))
  (switch Utilities|FlowControl|Switch|SwitchonEBeastState Alert%20State
    (:EBS_Neutral
      (Rendering|Components|TextRender|SetText _beaststate_text (Utilities|Text|FormatText "Neutral"))
      (Class|LLAIBeast|ResetTeleports :!label _label)
      (Collision|SetCollisionEnabled (Variables|Default|GetRighHandCollision) "NoCollision"))
    (:EBS_InvestigateNoise
      (Rendering|Components|TextRender|SetText _beaststate_text (Utilities|Text|FormatText "INv Noise"))
      (goto _label))
    (:EBS_Alerted
      (Rendering|Components|TextRender|SetText _beaststate_text (Utilities|Text|FormatText "Chasing Alerted")))))

(event EventPlayerEvation
  (params (PlayerPawn :type Pawn%20Object%20Reference))
  ;[0.1 0.15 0.2] User escaped signal
  (|CallParentFunction PlayerPawn)
  (bind _llplayer (Variables|Default|GetLLPlayer)
    (:then
      (CallFunction|ChangeWalkSpeed "Stop")
      (Transformation|SetActorRotation (Math|Rotator|FindLookatRotation (Transformation|GetActorLocation) (Transformation|GetActorLocation _llplayer)))
      (Audio|PlaySoundatLocation "/Game/Audio/SFX/MonsterScream_Cue.MonsterScream_Cue" (Transformation|GetActorLocation) "0, 0, 0" 1.0 1.0 0.0 0 0 0 0)
      (Animation|Montage|PlayMontage (Variables|Character|GetMesh) "/Game/Assets3D/Beast/Beast_Temp/ZombieScream_Montage.ZombieScream_Montage"
        (:OnCompleted
          (CallFunction|ChangeWalkSpeed "Normal"))))
    (:else)))

(fn ConstructionScript
  (bind _mesh (Variables|Character|GetMesh))
  (bind _mesh_2 (Variables|Character|GetMesh))
  (bind _clawglow_dummy (Variables|Default|GetClawGlow_Dummy))
  (Transformation|AttachComponentToComponent (Variables|Default|GetRighHandCollision) _mesh_2 "RightHand" "KeepRelative" "KeepRelative" "KeepRelative" true)
  (Transformation|AttachComponentToComponent (Variables|Default|GetPlayerCapturedConstrain) _mesh_2 "RightHand" "KeepRelative" "KeepRelative" "KeepRelative" true)
  (Transformation|AttachComponentToComponent _clawglow_dummy _mesh "RightHand" "KeepRelative" "KeepRelative" "KeepRelative" true)
  (Rendering|SetVisibility _clawglow_dummy false false)
  (Transformation|AttachComponentToComponent (Variables|Default|GetCube) _mesh "RightHand" "KeepRelative" "KeepRelative" "KeepRelative" false))