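; Game mode Blueprint that runs the beast threat and beacon completion flow for a level.
; On BeginPlay it fades out a level transition widget.
; After the start sequence, a non-negative TimeToBeast delays an EQS query (also triggerable via SpawnBeast) that places the beast AI and adds its state and location widgets.
; Beacon completion expires the beast and, after a delay, briefly shows a totem-completed widget.
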(event Custom|QueryLocactionFinished
  (params (QueryInstance :type Env%20Query%20Instance%20Blueprint%20Wrapper%20Object%20Reference) (QueryStatus :type EEnvQueryStatus%20Enum :default "Processing"))
  ;[0.9427 1 0 1 58] SpawnBeast TODO: Fix the C++ implementation
  (if (Utilities|Enum|Equal(Enum) QueryStatus "Success")
    (bind _resultlocations (AI|EQS|GetQueryResultsasLocations QueryInstance))
    (bind _returnvalue (Game|SpawnActorfromClass (Variables|Default|GetBeastAI_Class) (Math|Transform|MakeTransform (Utilities|Array|Get(acopy) _resultlocations) "0, 0, 0" "1,1,1") "AdjustIfPossibleButAlwaysSpawn" 0 0))
    (bind _output_get (Variables|Default|SetBeastAI _returnvalue))
    (bind _returnvalue_2 (UserInterface|CreateWidget "/Game/UIX/PlayerHUDs/WBP_BeastState.WBP_BeastState_C"))
    (UserInterface|Viewport|AddtoViewport _returnvalue_2 0)
    (bind _returnvalue_3 (UserInterface|CreateWidget "/Game/Blueprints/Misc/WBP_BeastLocation.WBP_BeastLocation_C" 0 _output_get))
    (UserInterface|Viewport|AddtoViewport _returnvalue_3 0)
    (Development|PrintString "Beast Spawned" true true "(R=0.384994,G=1.000000,B=0.000000,A=1.000000)")
    (else
      (Development|PrintString "Problem Runnignquery" true true "(R=1.000000,G=0.486477,B=0.000000,A=1.000000)"))))

(event EventBeginPlay
  (bind _returnvalue (UserInterface|CreateWidget "/Game/UIX/MainMenu/WBP_LevelTransition.WBP_LevelTransition_C"))
  (UserInterface|Viewport|AddtoViewport _returnvalue 10)
  (Default|FadeOutSequence _returnvalue))

(event EventTick
  (params (DeltaSeconds :type Float%20%28single-precision%29)))

(event EventStartSequence
  (bind _timetobeast (Variables|Default|GetTimeToBeast))
  (|CallParentFunction)
  (if (not (< _timetobeast 0.0))
    ;[0.9427 1 0 1 58] SpawnBeast TODO: Fix the C++ implementation
    (Utilities|FlowControl|Delay _timetobeast)
    (bind _returnvalue (AI|EQS|RunEQSQuery "/Game/Blueprints/BeastAI/Query_FindBeastSpawn.Query_FindBeastSpawn" self "RandomBest5Pct" "/Script/AIModule.EnvQueryInstanceBlueprintWrapper"))
    (EventDispatchers|BindEventtoOnQueryFinishedEvent _returnvalue (delegate Custom|QueryLocactionFinished))))

(event EventTottemCompleted
  (|CallParentFunction))

(event EventBeaconCompleted
  (|CallParentFunction)
  (Utilities|FlowControl|Sequence
    (:then_0
      (bind _beastai (Variables|Default|GetBeastAI)
        (:then
          (Actor|SetLifeSpan _beastai 1.0)
          (Development|PrintString "Beast killed"))
        (:else)))
    (:then_1
      (Utilities|FlowControl|Delay 3.0)
      (bind _returnvalue (UserInterface|CreateWidget "/Game/UIX/WBP_TottemCompleted.WBP_TottemCompleted_C"))
      (UserInterface|Viewport|AddtoViewport _returnvalue 0)
      (Utilities|FlowControl|Delay 3.0)
      (Widget|RemovefromParent _returnvalue))))

(event EventSpawnBeast
  ;[0.9427 1 0 1 58] SpawnBeast TODO: Fix the C++ implementation
  (bind _returnvalue (AI|EQS|RunEQSQuery "/Game/Blueprints/BeastAI/Query_FindBeastSpawn.Query_FindBeastSpawn" self "RandomBest5Pct" "/Script/AIModule.EnvQueryInstanceBlueprintWrapper"))
  (EventDispatchers|BindEventtoOnQueryFinishedEvent _returnvalue (delegate Custom|QueryLocactionFinished)))

(fn ConstructionScript)