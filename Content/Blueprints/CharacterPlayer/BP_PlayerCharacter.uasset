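; Player character Blueprint for a torch-and-fog game, linking the C++ base to HUD, torch and level manager.
; Tick feeds position and torch intensity into a Material Parameter Collection for fog-of-war; beacon completion switches the radius to a timeline.
; Torch burnout activates the beast and HUD chase.
; It also handles scripted intro and exit walks, puzzle input toggling, totem fragments, capsule resizing, and random unbalance for C++ movement.
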(event Custom|FolowMouse
  (if (Variables|Puzzle|GetbWithPuzzlePart)
    _))

(event Custom|DisappearFog
  ;[1 1 1] Desapear FOG
  (Variables|Default|SetbBeaconCompleted true)
  (bind _radiusdelta (Timeline|FogDissapeared PlayFromStart)
    (:Update
      (Rendering|Material|SetScalarParameterValue "/Game/Material/MC_Fog_Parametros.MC_Fog_Parametros" "RadiusExponential" _radiusdelta :!class /Script/Engine.KismetMaterialLibrary))))

(event Custom|BeaconActivated_Event
  ;[1 1 1] BeginPlay
  (CallFunction|DisappearFog))

(event Custom|Add%20HUD
  ;[1 1 1] Add  Gameplay HUD
  (bind _returnvalue (UserInterface|CreateWidget "/Game/UIX/PlayerHUDs/WBP_HUD.WBP_HUD_C" (Game|GetPlayerController 0)))
  (bind _output_get (Variables|Default|SetHUD_Jugador _returnvalue))
  (UserInterface|Viewport|AddtoViewport _output_get 0)
  (Variables|/Game/UIX/PlayerHUDs/WBP_HUD.WBP_HUD_C|SetStamine _output_get (Variables|Default|GetStamine))
  (Variables|/Script/LittleLights.Base_HUD_Widget|SetDeltaStamine _output_get 0.0))

(event Custom|MovePlayerTo
  (params (Location :type Vector) (Speed :type Float%20%28single-precision%29) (NewParam :type Boolean))
  (bind _returnvalue (Transformation|GetActorLocation))
  (bind _charactermovement (Variables|Character|GetCharacterMovement))
  (bind _returnvalue_2 (Math|Vector|Distance(Vector) _returnvalue Location))
  (bind _returnvalue_3 (/ _returnvalue_2 Speed))
  ;[1 1 1] Called by LevelMaster to make the player to move to a place in the first seconds, like an intro
  (Input|DisableInput (Game|GetPlayerController 0))
  (Variables|Default|SetMaxWalkSpeed_Save (Variables|/Script/Engine.CharacterMovementComponent|GetMaxWalkSpeed _charactermovement))
  (Variables|/Script/Engine.CharacterMovementComponent|SetMaxWalkSpeed _charactermovement Speed)
  (AI|Navigation|SimpleMovetoLocation (Game|GetPlayerController 0) Location)
  (bind _levelmanager (Variables|Default|GetLevelManager)
    (:then
      (switch Utilities|FlowControl|Switch|SwitchonEGameState (Variables|/Script/LittleLights.Level_Manager_Base|GetCurrentGameState _levelmanager)
        (:GameInit
          (Utilities|FlowControl|Delay _returnvalue_3)
          (Development|PrintString "Player Moved Atomatically")
          (Variables|/Script/Engine.CharacterMovementComponent|SetMaxWalkSpeed (Variables|Character|GetCharacterMovement) (Variables|Default|GetMaxWalkSpeed_Save))
          (bind _asbp_level_manager_base (Utilities|Casting|CastToBP_LevelManagerBase (Variables|Default|GetLevelManager)))
          (Default|PlayerEndedAutoMovment _asbp_level_manager_base))
        (:LevelCompleted
          (Utilities|FlowControl|Delay (/ _returnvalue_3 2.0))
          (Development|PrintString "Player moving to exit" true true "(R=0.000000,G=0.660000,B=1.000000,A=1.000000)" 1.0)
          (bind _asbp_level_manager_base_2 (Utilities|Casting|CastToBP_LevelManagerBase (Variables|Default|GetLevelManager)))
          (Default|ChangetoNextLevel _asbp_level_manager_base_2))))
    (:else)))

(event Custom|BeastChasing
  (params (DistanceRatio :type Float%20%28single-precision%29))
  (bind _hud_jugador (Variables|Default|GetHUD_Jugador))
  (Variables|Default|SetDistanceRatio DistanceRatio)
  (Utilities|IsValid _hud_jugador
    (:Is%20Valid
      (Variables|/Game/UIX/PlayerHUDs/WBP_HUD.WBP_HUD_C|SetDeltaDistanceBeast _hud_jugador DistanceRatio))))

(event Custom|PossessView
  ;[1 1 1] Posses View
  (Game|Player|SetViewTargetwithBlend (Game|GetPlayerController 0) self 2.0 "VTBlend_Linear" 0.0 false))

(event Custom|Unbalance
  ;[1 1 1] Unbalance Mechanic:
  ; The rest is implemented in C++ between the moveent and the Tick
  (if (Variables|Default|GetbBalancing)
    (Variables|Default|SetUnbalanceVelocity (Math|Random|RandomFloatinRange -0.01 0.01))))

(event Custom|StartUnbalnce
  ;[1 1 1] Unbalance Mechanic:
  ; The rest is implemented in C++ between the moveent and the Tick
  (Utilities|Time|SetTimerbyFunctionName 0 "Unbalance" 1.0 true))

(event EventBeginPlay
  ;[1 1 1] BeginPlay
  (Utilities|FlowControl|Sequence
    (:then_0
      (bind (_bvalid _levelmanager) (CallFunction|GetLevelManager))
      (if _bvalid
        (Variables|Default|SetLevelManager _levelmanager)
        (CallFunction|AddHUD))
      (Variables|Default|SetSpringArmRef 0))
    (:then_2
      (bind _torch (Variables|Default|GetTorch)
        (:then
          (if (Variables|Default|GetbStartTorchOn)
            (Class|Torch|TurnonOrb _torch)))
        (:else)))))

(event Collision|EventActorBeginOverlap
  (params (OtherActor :type Actor%20Object%20Reference)))

(event EventTick
  (params (DeltaSeconds :type Float%20%28single-precision%29))
  (Utilities|FlowControl|Sequence
    (:then_0
      ;[1 1 1] FIX:FogWar Update posicion de jugador
      (Rendering|Material|SetVectorParameterValue "/Game/Material/MC_Fog_Parametros.MC_Fog_Parametros" "Pos" (Math|Conversions|ToLinearColor(Vector) (+ (Transformation|GetActorLocation) (Variables|Default|GetOffsetFogWar))) :!class /Script/Engine.KismetMaterialLibrary))
    (:then_2
      (CallFunction|UpdateFogRadius))
    (:then_3
      (bind _fog (Variables|Default|GetFog)
        (:then
          (Transformation|SetActorLocation _fog (Transformation|GetActorLocation) false false)
          (Transformation|SetWorldRotation (Variables|/Script/Engine.Actor|GetRootComponent _fog) (Variables|Default|GetFillLightRot) false false))
        (:else)))))

(event EventEndGameEvent
  ;[1 1 1] FinNivel o Juego
  (Development|PrintString "Mensaje a jugador:Fin Juego"))

(event EventStartGameEvent
  ;[1 1 1] Game Started Signal
  (Utilities|FlowControl|Sequence
    (:then_1
      (bind _torch (Variables|Default|GetTorch)
        (:then
          (Class|Torch|StartDecay _torch 3e+01 true))
        (:else)))))

(event EventPlayerFall
  ;[1 1 1] Unbalance Mechanic:
  ; The rest is implemented in C++ between the moveent and the Tick
  (Animation|Montage|PlayMontage (Variables|Character|GetMesh) "/Game/Assets3D/Lucas/Animations/FallMontage.FallMontage"
    (:OnCompleted
      (Variables|Default|SetbCanMove true))))

(event EventTorchOff
  ;[1 1 1] Called from Torch when light is down
  ;;[0 1 0] TorchOff (c++ delcared)
  (bind _asbp_level_manager_base (Utilities|Casting|CastToBP_LevelManagerBase (Variables|Default|GetLevelManager)))
  (Default|ActivateBeast _asbp_level_manager_base)
  (Default|ChaseStarted (Variables|Default|GetHUD_Jugador)))

(event Input|ActionEvents|InputActionPuzzleDebug
  (params (Key :type Key%20Structure :default "None"))
  (:Pressed
    (Variables|Puzzle|SetbPuzzleSolving (not (Variables|Puzzle|GetbPuzzleSolving)))
    (CallFunction|ToggleInput (not (Variables|Default|GetbCanMove)))
    (Variables|Default|SetbCanMove (not (Variables|Default|GetbCanMove)))))

(event Input|KeyboardEvents|Escape
  (params (Key :type Key%20Structure :default "None"))
  ;[0.4334 1 0.4037] Input
  (:Pressed
    (Game|QuitGame 0 "Quit" false)))

(event Input|MouseEvents|LeftMouseButton
  (params (Key :type Key%20Structure :default "None"))
  (:Pressed
    (Development|PrintString (Utilities|GetDisplayName (.hitactor (.HitResult (Game|Player|GetHitResultUnderCursorbyChannel (Game|GetPlayerController 0) "TraceTypeQuery1" false)))))
    (Variables|Puzzle|SetbWithPuzzlePart true)))

(fn ConstructionScript
  (Rendering|Material|SetVectorParameterValue "/Game/Material/MC_Fog_Parametros.MC_Fog_Parametros" "Pos" (Math|Conversions|ToLinearColor(Vector) (Transformation|GetActorLocation)) :!class /Script/Engine.KismetMaterialLibrary)
  (if (Variables|CameraSettings|GetOverrideSpringArm)
    _))

(fn ToggleInput
  (params (EnableGameInput :type Boolean))
  (bind _returnvalue (Game|GetPlayerController 0))
  (if EnableGameInput
    (Input|SetInputModeGameOnly _returnvalue)
    (Variables|/Script/Engine.PlayerController|SetbShowMouseCursor _returnvalue false)
    (else
      (Input|DisableInput _returnvalue 0)
      (Input|SetInputModeUIOnly _returnvalue 0 "DoNotLock")
      (Variables|/Script/Engine.PlayerController|SetbShowMouseCursor _returnvalue true))))

(fn UpdateFogRadius
  (bind _torch (Variables|Default|GetTorch))
  (if (not (Variables|Default|GetbBeaconCompleted))
    (Utilities|IsValid _torch
      (:Is%20Valid
        (Rendering|Material|SetScalarParameterValue "/Game/Material/MC_Fog_Parametros.MC_Fog_Parametros" "RadiusExponential" (Math|Float|Lerp (Variables|Default|GetMinFogVisibility) (Variables|Default|GetMaxFogVisibility) (Variables|/Script/LittleLights.Torch|GetDeltaIntensity _torch)) :!class /Script/Engine.KismetMaterialLibrary)))))

(fn AddTottemPiece
  (params (TotemPiece :type BP%20Tottem%20Fragment%20Object%20Reference))
  (Utilities|Array|AddUnique (Variables|Default|GetTottemFragments) TotemPiece))

(fn RestToottemPiece
  (params (Amount :type Integer))
  (Variables|Default|SetFragmentsAmount (- (Variables|Default|GetFragmentsAmount) Amount)))

(fn ChangeCollisionSize
  (params (HeightType :type CapsuleHeight_Type%20Enum :default "NormalHeight"))
  (bind _capsulecomponent (Variables|Default|GetCapsuleComponent))
  (switch Utilities|FlowControl|Switch|SwitchonCapsuleHeight_Type HeightType
    (:NormalHeight
      (Components|Capsule|SetCapsuleHalfHeight _capsulecomponent (LocalVariables|GetNormal_Capsule_HeightSize) true))
    (:CrouchingHeight
      (Components|Capsule|SetCapsuleHalfHeight _capsulecomponent (LocalVariables|GetCrouching_Capsule_Height) true))
    (:JumpingOverHeight
      (Components|Capsule|SetCapsuleHalfHeight _capsulecomponent (LocalVariables|GetJumpingOver_Capsule_Height) true))))

(fn DeactivateCollision
  (params (deactivate :type Boolean))
  (bind _capsulecomponent (Variables|Default|GetCapsuleComponent))
  (if deactivate
    (Components|Activation|SetActive _capsulecomponent false false)
    (else
      (Components|Activation|SetActive _capsulecomponent true false))))