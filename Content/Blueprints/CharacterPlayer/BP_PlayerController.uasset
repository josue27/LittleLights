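; Player controller Blueprint that handles input mode, the game-over screen, level restarts and obstacle-error feedback.
; BeginPlay switches to game input, while GameOverHUD removes any HUD, shows WBP_GameOver and switches to UI input.
; RestartGame fades in a transition widget before reopening the current level, and ShowObstacleFade extends its parent with a camera shake at the player's camera.
; HUD creation, quit and gamepad/keyboard detection logic is left disconnected.
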(event Custom|AddHud
  ;[1 1 1] AddHud
)

(event Custom|GameOverHUD
  ;[1 1 1] GAME OVER UI DISPLAY
  (bind _hud_jugador (Variables|Default|GetHUD_Jugador)
    (:then
      (Widget|RemovefromParent _hud_jugador))
    (:else
      _))
  (bind _returnvalue (UserInterface|CreateWidget "/Game/UIX/PlayerHUDs/WBP_GameOver.WBP_GameOver_C" self))
  (UserInterface|Viewport|AddtoViewport _returnvalue 3)
  (CallFunction|ChangetoUIInput))

(event Custom|RestartGame
  ;[1 1 1] Restart Game
  (bind _returnvalue (UserInterface|CreateWidget "/Game/UIX/MainMenu/WBP_LevelTransition.WBP_LevelTransition_C"))
  (UserInterface|Viewport|AddtoViewport _returnvalue 100)
  (Default|FadeinSequence _returnvalue 1.0)
  (Utilities|FlowControl|Delay 1.0)
  (bind _returnvalue_2 (Game|GetCurrentLevelName true))
  (Game|OpenLevel(byName) (Utilities|String|StringToName _returnvalue_2)))

(event EventBeginPlay
  (Utilities|FlowControl|Sequence
    (:then_0
      (Input|EnableInput self)
      (Class|LLPlayerControllerBase|ChangetoGameInput))))

(event EventTick
  (params (DeltaSeconds :type Float%20%28single-precision%29)))

(event EventShowObstacleFade
  (|CallParentFunction)
  (bind _asbp_player_character (Utilities|Casting|CastToBP_PlayerCharacter (Game|Player|GetPlayerPawn 0)))
  (Camera|PlayWorldCameraShake "/Game/Blueprints/FX/BP_ObstacleError_CamShake.BP_ObstacleError_CamShake_C" (Transformation|GetWorldLocation (Variables|/Script/LittleLights.PlayerCharacter|GetCameraComp _asbp_player_character)) 0.0 1.5e+03 0.5))

(fn ConstructionScript)