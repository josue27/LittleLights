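; Player character variant for the first tutorial, adding fog of war and scripted orb and camera sequences to its parent.
; Each tick, a vertical trace's collision UV positions materials drawn into two fog render targets, and occlusion is recalculated.
; Tutorial events spawn or refill the orb without decay, and timelines drive spring arm length and lighting for zoom-out and simulated decay.
; The decay's end advances BP_Tutorial_A_01's dialogue.
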(event Custom|SpawnOrbTutorial
  (bind _toolscomponent (Variables|Default|GetToolsComponent))
  (Variables|/Script/LittleLights.LL_ToolsComponent|GetOrb _toolscomponent
    (:then
      _)
    (:else
      (Class|LLToolsComponent|SpawnOrb _toolscomponent)))
  (Class|LLToolsComponent|RefillOrb _toolscomponent 3e+01 false)
  (CallFunction|UpdateOrbDelta 1.0)
  (EventDispatchers|AssignOnOrbRemainingTimeChanged _toolscomponent (delegate Custom|CustomEvent)))

(event Custom|SetNewCameraView
  (bind _filllight (Variables|Default|GetFillLight))
  (Utilities|FlowControl|Delay 0.5)
  (Rendering|Components|Light|SetIntensity (Variables|Default|GetFillOrbPointLight) 3e+03)
  (bind _delta (Timeline|TimeFristZoomout PlayFromStart)
    (:Update
      ;[0.1 0.15 0.2] SpringArm
      (Variables|/Script/Engine.SpringArmComponent|SetTargetArmLength (Variables|Default|GetSpringArmComponent) (Math|Float|Lerp 3e+03 7.5e+03 _delta))
      ;[0.1 0.15 0.2] Light
      (Rendering|Lighting|SetOuterConeAngle _filllight (Math|Float|Lerp 0.0 4e+01 _delta))
      (Rendering|Lighting|SetInnerConeAngle _filllight (Math|Float|Lerp 0.0 35.0 _delta)))))

(event Custom|StartDecaySimulation
  (bind _filllight (Variables|Default|GetFillLight))
  (Utilities|FlowControl|Delay 0.5)
  (Utilities|FlowControl|Sequence
    (:then_0
      (bind _newtrack_0 (Timeline|OrbDecay PlayFromStart)
        (:Update
          (Rendering|Components|Light|SetIntensity (Variables|Default|GetFillOrbPointLight) (Math|Float|Lerp 0.0 3e+03 _newtrack_0))
          ;[0.1 0.15 0.2] SpringArm
          (Variables|/Script/Engine.SpringArmComponent|SetTargetArmLength (Variables|Default|GetSpringArmComponent) (Math|Float|Lerp 3e+03 7.5e+03 _newtrack_0))
          ;[0.1 0.15 0.2] Light
          (Rendering|Lighting|SetOuterConeAngle _filllight (Math|Float|Lerp 15.0 4e+01 _newtrack_0))
          (Rendering|Lighting|SetInnerConeAngle _filllight (Math|Float|Lerp 1e+01 35.0 _newtrack_0)))
        (:Finished
          (bind _returnvalue (Actor|GetActorOfClass "/Game/Blueprints/LevelManagers/BP_Tutorial_A_01.BP_Tutorial_A_01_C"))
          (Default|ShowNextDialogue _returnvalue true true false true))))))

(event Custom|CustomEvent
  (params (InstigatorActor :type Actor%20Object%20Reference) (RemainingDuration :type Float%20%28single-precision%29))
  (CallFunction|UpdateOrbDelta RemainingDuration))

(event Input|EnhancedActionEvents|EnhancedInputActionIA_Vault
  (params (ActionValue :type Boolean) (ElapsedSeconds :type Float%20%28double-precision%29) (TriggeredSeconds :type Float%20%28double-precision%29) (InputAction :type Input%20Action%20Object%20Reference :default "/Game/Blueprints/Input/IA_Vault.IA_Vault")))

(event EventBeginPlay
  (|CallParentFunction)
  (Utilities|Struct|SetmembersinPostProcessSettings (Variables|/Script/Engine.CameraComponent|GetPostProcessSettings (Variables|Default|GetCameraComp)) 0.5 0.0 2e+02)
  ;[0.1 0.15 0.2] Fog of War
  (bind _returnvalue (Rendering|Material|CreateDynamicMaterialInstance "/Game/FogOfWarSystem/MM_FogOfWar.MM_FogOfWar" "None" "None" :!class /Script/Engine.KismetMaterialLibrary))
  (Variables|Default|SetFogOfWarMaterial _returnvalue)
  (bind _returnvalue_2 (Rendering|Material|CreateDynamicMaterialInstance "/Game/FogOfWarSystem/MM_FogOfWarReveal.MM_FogOfWarReveal" "None" "None" :!class /Script/Engine.KismetMaterialLibrary))
  (Variables|Default|SetFogOfWarReveal _returnvalue_2)
  (Rendering|ClearRenderTarget2D "/Game/FogOfWarSystem/FogOfWarReveal_Render.FogOfWarReveal_Render")
  (Rendering|ClearRenderTarget2D "/Game/FogOfWarSystem/FogOfWar_Render.FogOfWar_Render")
  (Rendering|Material|SetScalarParameterValue (Variables|Default|GetFogOfWarReveal) "Size" (Math|Float|Lerp 0.0625 0.08 0.0) :!class /Script/Engine.MaterialInstanceDynamic)
  (Rendering|DrawMaterialtoRenderTarget "/Game/FogOfWarSystem/FogOfWarReveal_Render.FogOfWarReveal_Render" (Variables|Default|GetFogOfWarReveal))
  (Rendering|Material|SetScalarParameterValue "/Game/Maps/SandBox/SphereMaskTEst/MPC_ShadowFog.MPC_ShadowFog" "AlphaShadowNoise" (Math|Float|Lerp 1.0 0.5 0.0) :!class /Script/Engine.KismetMaterialLibrary))

(event Collision|EventActorBeginOverlap
  (params (OtherActor :type Actor%20Object%20Reference))
  (|CallParentFunction OtherActor) ; This node is disabled and will not be called.\nDrag off pins to build functionality.
)

(event EventTick
  (params (DeltaSeconds :type Float%20%28single-precision%29))
  (bind _returnvalue (Transformation|GetActorLocation))
  (bind _fogofwarmaterial (Variables|Default|GetFogOfWarMaterial))
  (|CallParentFunction DeltaSeconds)
  (Utilities|FlowControl|Sequence
    (:then_0
      ;[0.1 0.15 0.2] Fog of ware update
      (bind _outhit (Collision|LineTraceByChannel (+ _returnvalue "0.000000,0.000000,500.000000") (+ _returnvalue "0.000000,0.000000,-500.000000") "TraceTypeQuery4" true 0 "None"))
      (if (.ReturnValue (Class|GameplayStatics|FindCollisionUV _outhit))
        (Rendering|Material|SetVectorParameterValue _fogofwarmaterial "Location" (Utilities|Struct|MakeLinearColor (.X (Math|Vector2D|BreakVector2D (.UV (Class|GameplayStatics|FindCollisionUV _outhit)))) (.Y (Math|Vector2D|BreakVector2D (.UV (Class|GameplayStatics|FindCollisionUV _outhit)))) 0.0 1.0) :!class /Script/Engine.MaterialInstanceDynamic)
        (Rendering|DrawMaterialtoRenderTarget "/Game/FogOfWarSystem/FogOfWarReveal_Render.FogOfWarReveal_Render" (Variables|Default|GetFogOfWarReveal))
        (Rendering|DrawMaterialtoRenderTarget "/Game/FogOfWarSystem/FogOfWar_Render.FogOfWar_Render" _fogofwarmaterial)))
    (:then_2
      (CallFunction|OcclusionCalculation))))

(event EventAddHUD)

(fn ConstructionScript
  (|CallParentFunction))