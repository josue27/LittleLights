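; Tutorial B player character variant that gates torch lighting behind a one-time dialog at a fire pit.
; On BeginPlay, if it starts with light, it stops the torch from decaying.
; The first interact inside a fire pit shows a tutorial widget, switches to UI input and locks movement; later presses call LightUpTorch directly, without rechecking the pit.
; TorchOff only prints a debug message.
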(event EventBeginPlay
  (|CallParentFunction)
  (if (Variables|Default|GetbStartWithLight)
    (bind _torch (Variables|Default|GetTorch)
      (:then
        (Variables|/Script/LittleLights.Torch|SetbStartDecay _torch false))
      (:else
        (Development|PrintString "no torch")))))

(event Collision|EventActorBeginOverlap
  (params (OtherActor :type Actor%20Object%20Reference))
  (|CallParentFunction OtherActor) ; This node is disabled and will not be called.\nDrag off pins to build functionality.
)

(event EventTick
  (params (DeltaSeconds :type Float%20%28single-precision%29))
  (|CallParentFunction DeltaSeconds) ; This node is disabled and will not be called.\nDrag off pins to build functionality.
)

(event EventTorchOff
  (Development|PrintString "Torch off"))

(event Input|ActionEvents|InputActionInteractInput
  (params (Key :type Key%20Structure))
  (:Pressed
    (if (Variables|TutorialB|GetfirstActionPressed)
      (Class|PlayerCharacter|LightUpTorch 0.0)
      (elif (Variables|Default|GetbInFirePit)
        (bind _returnvalue (UserInterface|CreateWidget "/Game/UIX/Tutorial_B/WBP_Tutorial_B_Dialog9.WBP_Tutorial_B_Dialog9_C"))
        (UserInterface|Viewport|AddtoViewport _returnvalue 0)
        (CallFunction|ChangetoUIInput)
        (CallFunction|PlayerCanMove false)
        (Variables|TutorialB|SetfirstActionPressed true)))))

(fn ConstructionScript
  (|CallParentFunction))