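; BP_EndTutorial_Base is a trigger actor that ends the tutorial and loads the next level.
; When the player character overlaps its Box, it switches to UI input and moves the player to the Arrow's location at intro speed.
; After a delay it plays the WBP_LevelTransition fade-in, then opens the referenced Level.
; An older camera-detach and spline-timeline exit route remains as deprecated, disconnected logic.
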(event OnComponentBeginOverlap(Box)
  (params (OverlappedComponent :type Primitive%20Component%20Object%20Reference) (OtherActor :type Actor%20Object%20Reference) (OtherComp :type Primitive%20Component%20Object%20Reference) (OtherBodyIndex :type Integer) (bFromSweep :type Boolean) (SweepResult :type Hit%20Result%20Structure%20%28by%20ref%29))
  (bind _playercharachter (Variables|Default|GetPlayerCharachter))
  (if (== OtherActor _playercharachter)
    (CallFunction|ChangetoUIInput)
    (Default|MovePlayerto _playercharachter (Transformation|GetWorldLocation (Variables|Default|GetArrow)) (Variables|Default|GetIntroVelocityMovement))
    (Utilities|FlowControl|Delay 2.0)
    (bind _returnvalue (UserInterface|CreateWidget "/Game/UIX/MainMenu/WBP_LevelTransition.WBP_LevelTransition_C"))
    (UserInterface|Viewport|AddtoViewport _returnvalue 0)
    (Default|FadeinSequence _returnvalue)
    (Utilities|FlowControl|Delay 1.8)
    (Game|OpenLevel(byObjectReference) (Variables|Default|GetLevel))))

(event EventBeginPlay)

(event Collision|EventActorBeginOverlap
  (params (OtherActor :type Actor%20Object%20Reference)))

(event EventTick
  (params (DeltaSeconds :type Float%20%28single-precision%29)))

(fn ConstructionScript)